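; Player character Blueprint for Jacob, handling interaction, carrying and pushing objects, NPC conversations and alpaca companion commands.
; InteractRadius overlaps select an Interface_Interactable target; grab and push functions attach it, adjusting movement, and dropping traces down to place it.
; Once enabled, Stay traces beneath the player to send AICompanionController there with a decal, snapping to pressure switches.
; LightUp/LightDown toggle emissive material and emitter; older grab-and-throw logic is disconnected.
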(event OnComponentBeginOverlap(InteractRadius)
  (params (OverlappedComponent :type Primitive%20Component%20Object%20Reference) (OtherActor :type Actor%20Object%20Reference) (OtherComp :type Primitive%20Component%20Object%20Reference) (OtherBodyIndex :type Integer) (bFromSweep :type Boolean) (SweepResult :type Hit%20Result%20Structure%20%28by%20ref%29))
  (bind _returnvalue (Utilities|GetClass OtherActor))
  (bind _ispushingobject (Variables|Default|GetIsPushingObject))
  (bind _isholdingobject (Variables|Default|GetIsHoldingObject))
  (bind _returnvalue_2 (or _isholdingobject _ispushingobject))
  ;[1 1 1] Begin/End Overlap
  (if (or (or (or (or (or (and _returnvalue_2 (Utilities|ClassIsChildOf _returnvalue "/Game/Jacob/Grab/BP_AttachedObjectPickup.BP_AttachedObjectPickup_C")) (and _returnvalue_2 (Utilities|ClassIsChildOf _returnvalue "/Game/Jacob/Push/BP_PushAndDragObject.BP_PushAndDragObject_C"))) (and _returnvalue_2 (Utilities|ClassIsChildOf _returnvalue "/Game/Jacob/Puzzle/PuzzleBridge/BP_Lever_Bridge.BP_Lever_Bridge_C"))) (and _returnvalue_2 (Utilities|ClassIsChildOf _returnvalue "/Game/Marcus/Enemy/BP_Lamp_TEST.BP_Lamp_TEST_C"))) (and _returnvalue_2 (Utilities|ClassIsChildOf _returnvalue "/Game/AICompanion/AI_Alan.AI_Alan_C"))) (and _returnvalue_2 (Utilities|ClassIsChildOf _returnvalue "/Game/Jacob/Puzzle/PuzzleBig/BP_Lever_BigPuzzle.BP_Lever_BigPuzzle_C")))
    (Variables|Default|SetCanDropObject false)
    (else
      (Variables|Default|SetCanDropObject true)
      (CallFunction|SetInteractable OtherActor))))

(event OnComponentEndOverlap(InteractRadius)
  (params (OverlappedComponent :type Primitive%20Component%20Object%20Reference) (OtherActor :type Actor%20Object%20Reference) (OtherComp :type Primitive%20Component%20Object%20Reference) (OtherBodyIndex :type Integer))
  (Variables|Default|SetCanDropObject true)
  (CallFunction|DisableInteract OtherActor))

(event Input|EnhancedActionEvents|EnhancedInputActionIA_Interact
  (params (ActionValue :type Boolean) (ElapsedSeconds :type Float%20%28double-precision%29) (TriggeredSeconds :type Float%20%28double-precision%29) (InputAction :type Input%20Action%20Object%20Reference :default "/Game/ThirdPerson/Input/Actions/IA_Interact.IA_Interact"))
  ;[1 1 1] Inputs
  (:Started
    (CallFunction|InteractwithObject)
    (CallFunction|InteractwithGrabObject)))

(event Input|EnhancedActionEvents|EnhancedInputActionIA_Grab
  (params (ActionValue :type Boolean) (ElapsedSeconds :type Float%20%28double-precision%29) (TriggeredSeconds :type Float%20%28double-precision%29) (InputAction :type Input%20Action%20Object%20Reference :default "/Game/ThirdPerson/Input/Actions/IA_Grab.IA_Grab"))
  ;[1 1 1] Inputs
)

(event EventBeginPlay
  (bind _mesh (Variables|Character|GetMesh))
  (bind _returnvalue (Rendering|Material|CreateDynamicMaterialInstance _mesh 1 "/Game/Materials/Characters/Stella_Emissive.Stella_Emissive" "None" :!class /Script/Engine.PrimitiveComponent))
  (bind _output_get (Variables|Default|SetNewVar _returnvalue))
  (Rendering|Material|SetMaterial _mesh 1 _output_get)
  (Rendering|Material|SetScalarParameterValue _output_get "None" 0.0 :!class /Script/Engine.MaterialInstanceDynamic)
  (CallFunction|DisableTextforAlpacaJump)
  (Variables|Default|SetAlpacaIsInStay true)
  (Variables|Default|SetLastCameraRef self))

(event EventTick
  (params (DeltaSeconds :type Float%20%28single-precision%29))
  ;[1 1 1] Tick
  (|CallParentFunction DeltaSeconds)
  (if (Variables|Default|GetEnableCallStay)
    (Utilities|FlowControl|DoOnce false
      (:Completed
        (CallFunction|TextEnableCall)))))

(event EventConversationClosed
  ;[1 1 1] Conversation Closed
  (CallFunction|UnlockPlayerMovement))

(event Input|ActionEvents|InputActionStay
  (params (Key :type Key%20Structure))
  (bind _returnvalue (Transformation|GetActorLocation))
  (bind (_x _y _z) (Math|Vector|BreakVector _returnvalue))
  (:Pressed
    (if (Variables|Default|GetEnableCallStay)
      (CallFunction|TextEnableCall)
      ;[1 1 1] Stay-K
      (bind (_outhit _returnvalue_2) (Collision|LineTraceByChannel _returnvalue (Math|Vector|MakeVector _x _y (- _z 1e+03)) "TraceTypeQuery1" false (Utilities|Array|MakeArray self 0 0) "None"))
      (if _returnvalue_2
        (if (Utilities|ClassIsChildOf (Utilities|GetClass (.HitActor (Collision|BreakHitResult _outhit))) "/Game/Jacob/BP_PressureSwitch_Parent.BP_PressureSwitch_Parent_C")
          (bind _returnvalue_3 (Actor|GetActorOfClass "/Script/GruppOnion.AICompanionController"))
          (Class|AICompanionController|CalltoLocation _returnvalue_3 (Transformation|GetActorLocation (.HitActor (Collision|BreakHitResult _outhit))))
          (Rendering|Decal|SpawnDecalatLocation "/Game/AICompanion/M_CallToLocation.M_CallToLocation" "100.000000,100.000000,100.000000" (Transformation|GetActorLocation (.HitActor (Collision|BreakHitResult _outhit))) "-90.000000,0.000000,0.000000" 3.0)
          (else
            (bind _returnvalue_4 (Actor|GetActorOfClass "/Script/GruppOnion.AICompanionController"))
            (Class|AICompanionController|CalltoLocation _returnvalue_4 (.Location (Collision|BreakHitResult _outhit)))
            (Rendering|Decal|SpawnDecalatLocation "/Game/AICompanion/M_CallToLocation.M_CallToLocation" "100.000000,100.000000,100.000000" (.Location (Collision|BreakHitResult _outhit)) "-90.000000,0.000000,0.000000" 3.0))))
      (else
        (Development|PrintString "You have not found the alpaca yet")))))

(fn ConstructionScript
  (|CallParentFunction))

(fn InteractwithObject
  (bind _interactable (Variables|Default|GetInteractable))
  (Utilities|IsValid _interactable
    (:Is%20Valid
      (if (Utilities|ClassIsChildOf (Utilities|GetClass _interactable) "/Game/Marcus/NPC/NPCs/NPC_Base.NPC_Base_C")
        (CallFunction|LockPlayerMovement))
      (Class|InterfaceInteractable|Interact(Message) (Variables|Default|GetInteractable) self))))

(fn LockPlayerMovement
  (Input|SetInputModeUIOnly (Game|GetPlayerController 0) 0 "DoNotLock" false)
  (Variables|/Script/Engine.PlayerController|SetbShowMouseCursor (Game|GetPlayerController 0) true))

(fn UnlockPlayerMovement
  (Variables|/Script/Engine.PlayerController|SetbShowMouseCursor (Game|GetPlayerController 0) false)
  (Input|SetInputModeGameOnly (Game|GetPlayerController 0) false))

(fn DisableInteract
  (params (Other%20Actor :type Object%20Object%20Reference))
  (if (and (!= Other%20Actor self) (== Other%20Actor (Variables|Default|GetInteractable)))
    (Class|InterfaceInteractable|SetInteractableState(Message) (Variables|Default|GetInteractable) false)
    (Variables|Default|SetInteractable 0)))

(fn SetInteractable
  (params (OtherObject :type Actor%20Object%20Reference))
  (if (!= OtherObject self)
    (if (Utilities|DoesObjectImplementInterface OtherObject "/Script/GruppOnion.Interface_Interactable")
      (Utilities|IsValid (Variables|Default|GetInteractable)
        (:Is%20Valid
          (Class|InterfaceInteractable|SetInteractableState(Message) (Variables|Default|GetInteractable) false)
          (Variables|Default|SetInteractable 0))
        (:Is%20Not%20Valid
          _))
      (Variables|Default|SetInteractable OtherObject)
      (Class|InterfaceInteractable|SetInteractableState(Message) (Variables|Default|GetInteractable) true))))

(fn Detach
  (bind _grabbedobject (Variables|Default|GetGrabbedObject))
  (Transformation|DetachFromActor _grabbedobject "KeepWorld" "KeepWorld" "KeepWorld")
  (Class|BPIForce|ApplyForcewithDirection(Message) _grabbedobject "0.000000,0.000000,-5.000000" 5e+01)
  (Development|PrintString "detach"))

(fn LightDown
  (Rendering|Material|SetScalarParameterValue (Variables|Default|GetNewVar) "bHasLight" 0.0 :!class /Script/Engine.MaterialInstanceDynamic)
  (Variables|Default|SetHasLight false)
  (Default|CallLightStatus)
  (Components|Activation|Deactivate (Variables|Default|GetLightEmitter)))

(fn LightUp
  (Rendering|Material|SetScalarParameterValue (Variables|Default|GetNewVar) "bHasLight" 1.0 :!class /Script/Engine.MaterialInstanceDynamic)
  (Components|Activation|Activate (Variables|Default|GetLightEmitter) false)
  (Variables|Default|SetHasLight true)
  (Default|CallLightStatus))

(fn GrabObject
  (bind _charactermovement (Variables|Character|GetCharacterMovement))
  (bind _interactable (Variables|Default|GetInteractable))
  (bind _returnvalue (Utilities|GetClass _interactable))
  (Development|PrintString "Grabbing")
  (bind _interactable_2 (Variables|Default|GetInteractable)
    (:then
      (Variables|Default|SetIsHoldingObject true)
      (Transformation|AttachComponentToComponent _interactable_2 (Variables|Default|GetObjectToGrab) "None" "SnapToTarget" "SnapToTarget" "KeepWorld" true)
      (Collision|IgnoreActorwhenMoving (Variables|Default|GetCapsuleComponent) _interactable_2 true)
      (Components|Capsule|SetCapsuleSize (Variables|Default|GetCapsuleComponent) 9e+01 9e+01 true)
      (Utilities|IsValid _interactable
        (:Is%20Valid
          (if (or (Utilities|ClassIsChildOf _returnvalue "/Game/Jacob/Grab/BP_AttachedObjectPickup_Pillar.BP_AttachedObjectPickup_Pillar_C") (Utilities|ClassIsChildOf _returnvalue "/Game/Jacob/Grab/BP_AttachedObjectPickup_Stone.BP_AttachedObjectPickup_Stone_C"))
            (Variables|/Script/Engine.CharacterMovementComponent|SetMaxWalkSpeed _charactermovement 1.2e+02)
            (Variables|/Script/Engine.CharacterMovementComponent|SetRotationRate _charactermovement "0.000000,200.000000,0.000000")))))
    (:else)))

(fn DropObject
  (bind _objecttograb (Variables|Default|GetObjectToGrab))
  (bind _returnvalue (Transformation|GetWorldLocation _objecttograb))
  (bind (_x _y _z) (Math|Vector|BreakVector _returnvalue))
  (Transformation|DetachFromActor (Variables|Default|GetInteractable) "KeepWorld" "KeepWorld" "KeepWorld")
  (bind (_outhit _returnvalue_2) (Collision|LineTraceByChannel _returnvalue (Math|Vector|MakeVector _x _y (- _z 1e+03)) "TraceTypeQuery1" false (Utilities|Array|MakeArray (Variables|Default|GetInteractable) self 0) "None"))
  (if _returnvalue_2
    (if (Utilities|DoesObjectImplementInterface (.HitActor (Collision|BreakHitResult _outhit)) 0)
      (Transformation|SetActorLocationAndRotation (Variables|Default|GetInteractable) (- (.Origin (Collision|GetActorBounds (.HitActor (Collision|BreakHitResult _outhit)) false false)) "8.700000,8.700000,-10.000000") (Transformation|GetActorRotation (.HitActor (Collision|BreakHitResult _outhit))))
      (else
        (Transformation|SetActorLocation (Variables|Default|GetInteractable) (.Location (Collision|BreakHitResult _outhit)) false false)))
    (Variables|Default|SetIsHoldingObject false)
    (Components|Capsule|SetCapsuleSize (Variables|Default|GetCapsuleComponent) 32.571621 9e+01 true)
    (Variables|/Script/Engine.CharacterMovementComponent|SetMaxWalkSpeed (Variables|Character|GetCharacterMovement) 3.5e+02)
    (Variables|/Script/Engine.CharacterMovementComponent|SetRotationRate (Variables|Character|GetCharacterMovement) "0.000000,350.000000,0.000000")))

(fn InteractwithGrabObject
  (bind _interactable (Variables|Default|GetInteractable))
  (Utilities|IsValid _interactable
    (:Is%20Valid
      (if (Utilities|ClassIsChildOf (Utilities|GetClass _interactable) "/Game/Marcus/NPC/NPCs/NPC_Base.NPC_Base_C")
        (CallFunction|LockPlayerMovement)
        (else
          (Class|InterfaceInteractable|InteractGrab(Message) (Variables|Default|GetInteractable) self))))))

(fn GrabandPushObject
  (Development|PrintString "Grabbing")
  (bind _interactable (Variables|Default|GetInteractable)
    (:then
      (Variables|Default|SetIsHoldingObject true)
      (Transformation|AttachComponentToComponent _interactable (Variables|Default|GetObjectToPush) "None" "KeepWorld" "KeepWorld" "KeepWorld" true)
      (Collision|IgnoreActorwhenMoving (Variables|Default|GetCapsuleComponent) _interactable false)
      (Variables|/Script/Engine.CharacterMovementComponent|SetMaxWalkSpeed (Variables|Character|GetCharacterMovement) 9e+01)
      (Variables|/Script/Engine.CharacterMovementComponent|SetRotationRate (Variables|Character|GetCharacterMovement) "0, 0, 0"))
    (:else)))

(fn DropandPushObject
  (bind _charactermovement (Variables|Character|GetCharacterMovement))
  (bind _interactable (Variables|Default|GetInteractable))
  (bind _asbp_push_and_drag_object (Utilities|Casting|CastToBP_PushAndDragObject _interactable))
  (Collision|SetCollisionEnabled (Variables|/Game/Jacob/Push/BP_PushAndDragObject.BP_PushAndDragObject_C|GetCube _asbp_push_and_drag_object) "QueryAndPhysics")
  (Transformation|DetachFromActor _interactable "KeepWorld" "KeepWorld" "KeepWorld")
  (Variables|Default|SetIsHoldingObject false)
  (Variables|/Script/Engine.CharacterMovementComponent|SetMaxWalkSpeed _charactermovement 3.5e+02)
  (Variables|/Script/Engine.CharacterMovementComponent|SetRotationRate _charactermovement "0.000000,350.000000,0.000000")
  (Class|MovementComponent|SetPlaneConstraintNormal _charactermovement "0, 0, 0"))

(fn DisableTextforAlpacaJump
  (bind _asnew_hud (Utilities|Casting|CastToNewHUD (HUD|GetHUD (Game|GetPlayerController 0))))
  (bind _output_get (Variables|Default|SetAs%20New%20HUD _asnew_hud))
  (Default|AlpaccaJumpText (Variables|/Game/Jacob/UI/NewHUD.NewHUD_C|GetUIRef _output_get) false))

(fn TextEnableCall
  (bind _asnew_hud (Utilities|Casting|CastToNewHUD (HUD|GetHUD (Game|GetPlayerController 0))))
  (bind _output_get (Variables|Default|SetAs%20New%20HUD _asnew_hud))
  (Default|AlpacaCallText (Variables|/Game/Jacob/UI/NewHUD.NewHUD_C|GetUIRef _output_get) true))