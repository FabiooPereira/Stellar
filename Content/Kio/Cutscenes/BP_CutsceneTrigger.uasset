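; Trigger actor that starts the outro cutscene and leads into the end credits.
; On any actor overlap, it tells the player's third-person character to hide for the outro and plays a referenced level sequence, without checking which actor overlapped.
; A fixed delay, rather than a sequence-finished event, then calls GoToMain, which despite its name has the game mode play the end credits.
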(event Custom|Go%20To%20Main
  (Utilities|FlowControl|Delay 0.0)
  (bind _asbp_beyond_the_fluff_game_mode (Utilities|Casting|CastToBP_BeyondTheFluffGameMode (Game|GetGameMode)))
  (Default|PlayEndCredits _asbp_beyond_the_fluff_game_mode))

(event EventBeginPlay)

(event Collision|EventActorBeginOverlap
  (params (OtherActor :type Actor%20Object%20Reference))
  (bind _asbp_third_person_character (Utilities|Casting|CastToBP_ThirdPersonCharacter (Game|Player|GetPlayerPawn 0)))
  (Default|OutroHidePlayer _asbp_third_person_character)
  (Sequencer|Player|Play (Variables|/Script/LevelSequence.LevelSequenceActor|GetSequencePlayer (Variables|Default|GetLevel%20Sequence_0)) :!class /Script/MovieScene.MovieSceneSequencePlayer)
  (Utilities|FlowControl|Delay 12.5)
  (CallFunction|GotoMain))

(event EventTick
  (params (DeltaSeconds :type Float%20%28single-precision%29)))

(fn ConstructionScript)