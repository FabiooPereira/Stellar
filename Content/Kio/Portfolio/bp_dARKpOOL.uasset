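; Dark pool VFX showcase actor that takes the player's view and numpad input to spawn and despawn a Niagara pool with smoke.
; Timelines drive pool size, reinitializing it on every update, and ramp the smoke parameters.
; SwitchOnKey picks a size curve by CurrentKey, but Spawn always resets it to NumPadOne.
; DeSpawn switches to the third curve, fades smoke, then reverses the pool timeline after a delay.
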(event Custom|DeSpawn
  (Variables|Default|SetCurrentKey "NumPadThree")
  (CallFunction|KillSmoke)
  (Utilities|FlowControl|Delay 0.4)
  (CallFunction|DeSpawnPool))

(event Custom|KillSmoke
  (bind _smoke (Variables|Default|GetSmoke))
  (bind _smoke_2 (Variables|Default|GetSmoke))
  (Niagara|SetNiagaraVariable(Float) _smoke "User.StartWidth" -1.0)
  (Niagara|SetNiagaraVariable(Float) _smoke "User.KillParticle" 0.0)
  (bind _kill (Timeline|Timeline_KillSmoke PlayFromStart)
    (:Update
      (Niagara|SetNiagaraVariable(Float) _smoke_2 "User.Kill" _kill)
      (Niagara|SetNiagaraVariable(Float) _smoke_2 "User.KillParticle" _kill))))

(event Custom|Spawn
  (bind _smoke (Variables|Default|GetSmoke))
  (Variables|Default|SetCurrentKey "NumPadOne")
  (CallFunction|SpawnPool)
  (bind _time (Timeline|Timeline PlayFromStart)
    (:Update
      (if (== _time 1.0)
        (Utilities|FlowControl|DoOnce false :!label _label
          (:Completed
            (Components|Activation|Activate _smoke true)
            (Niagara|ReinitializeSystem _smoke)
            (CallFunction|StartSmoke)))))
    (:Finished
      (goto _label Reset))))

(event Custom|StartSmoke
  (bind _smoke (Variables|Default|GetSmoke))
  (bind _smoke_2 (Variables|Default|GetSmoke))
  (Niagara|SetNiagaraVariable(Float) _smoke "User.Kill" 0.0)
  (Niagara|SetNiagaraVariable(Float) _smoke "User.KillParticle" -1.0)
  (bind (_direction _kill _particlelifetime) (Timeline|Timeline_StartSmoke PlayFromStart)
    (:Update
      (Niagara|SetNiagaraVariable(Float) _smoke_2 "User.StartWidth" _kill)
      (Niagara|SetNiagaraVariable(Float) _smoke_2 "User.Kill" _particlelifetime))))

(event Custom|DeSpawnPool
  (bind (_direction _size _size2 _size3) (Timeline|Pool_Timeline ReverseFromEnd)
    (:Update
      (bind _output (CallFunction|SwitchonKey (Utilities|Array|MakeArray _size _size2 _size3)))
      (CallFunction|SetPoolSize _output))))

(event Custom|SpawnPool
  (bind (_direction _size _size2 _size3) (Timeline|Pool_Timeline Play)
    (:Update
      (bind _output (CallFunction|SwitchonKey (Utilities|Array|MakeArray _size _size2 _size3)))
      (CallFunction|SetPoolSize _output))))

(event EventBeginPlay
  (bind _returnvalue (Game|GetPlayerController 0))
  (bind _pool (Variables|Default|GetPool))
  (Input|EnableInput _returnvalue)
  (Effects|Components|ParticleSystem|SetFloatParameter _pool "User.size" 0.0)
  (Niagara|ReinitializeSystem _pool)
  (Game|Player|SetViewTargetwithBlend _returnvalue (Variables|Default|GetCamera) 0.0 "VTBlend_Linear" 0.0 false))

(event Input|KeyboardEvents|NumPadThree
  (params (Key :type Key%20Structure :default "None"))
  (:Pressed
    (Variables|Default|SetCurrentKey Key)
    (CallFunction|Spawn)))

(event Input|KeyboardEvents|NumPadZero
  (params (Key :type Key%20Structure :default "None"))
  (:Pressed
    (Variables|Default|SetCurrentKey "NumPadThree")
    (CallFunction|DeSpawn)))

(event Input|KeyboardEvents|NumPadTwo
  (params (Key :type Key%20Structure :default "None"))
  (:Pressed
    (Variables|Default|SetCurrentKey Key)
    (CallFunction|Spawn)))

(event Input|KeyboardEvents|NumPadOne
  (params (Key :type Key%20Structure :default "None"))
  (:Pressed
    (Variables|Default|SetCurrentKey Key)
    (CallFunction|Spawn)))

(fn ConstructionScript)

(fn SetPoolSize
  (params (Size :type Float%20%28single-precision%29))
  (bind _pool (Variables|Default|GetPool))
  (Effects|Components|ParticleSystem|SetFloatParameter _pool "User.size" Size)
  (Niagara|ReinitializeSystem _pool))

(fn SwitchonKey
  (params (Curves :type Array%20of%20Floats%20%28double-precision%29))
  (switch string (Utilities|String|ToString(Text) (Class|KismetInputLibrary|KeyGetDisplayName (Variables|Default|GetCurrentKey) true))
    (:Default
      (Development|PrintString "default"))
    (:num%201
      (return (Utilities|Array|Get(acopy) Curves)))
    (:num%202
      (return (Utilities|Array|Get(acopy) Curves 1)))
    (:num%203
      (return (Utilities|Array|Get(acopy) Curves 2)))))