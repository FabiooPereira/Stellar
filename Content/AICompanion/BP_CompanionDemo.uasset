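; BP_CompanionDemo is a demo interactable for the AI companion folder that stands in for a conversation partner.
; SetInteractableState stores whether interaction is allowed and swaps the static mesh material to show that state.
; Interact stores the instigator, waits briefly, then sends it a conversation-closed message without running any dialogue.
; BeginPlay prints the player character's name.
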(event EventTick
  (params (DeltaSeconds :type Float%20%28single-precision%29)))

(event EventBeginPlay
  (Development|PrintString (Utilities|GetDisplayName (Game|GetPlayerCharacter 0))))

(event EventSetInteractableState
  (params (bCanShowInteract? :type Boolean))
  (bind _output_get (Variables|Default|SetbCanInteract? bCanShowInteract?))
  (if _output_get
    (Rendering|Material|SetMaterial (Variables|Default|GetStaticMesh) 0 "/AnimationSharing/AnimSharingGreen.AnimSharingGreen")
    (else
      (Rendering|Material|SetMaterial (Variables|Default|GetStaticMesh) 0 "/DatasmithContent/Materials/FBXImporter/DeltaGenReference.DeltaGenReference"))))

(event EventInteract
  (params (Instigator :type Actor%20Object%20Reference))
  (bind _output_get (Variables|Default|SetInteractInstigator Instigator))
  (Utilities|FlowControl|Delay 2.0)
  (Class|BPIInteractable|ConversationClosed(Message) _output_get))

(fn ConstructionScript)