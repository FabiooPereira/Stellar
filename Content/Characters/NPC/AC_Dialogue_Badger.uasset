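; Dialogue component for the Badger NPC, overriding the parent Dialogue function to script a branching conversation.
; Tree 0 asks the player for help, with nested AddDialogue calls branching on the chosen option.
; Agreeing fully advances the tree index to 1, while backing out rolls back or clears dialogue progress before closing.
; Tree 1 plays a randomly picked line about being stuck, then resets progress and closes.
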(fn Dialogue
  (|CallParentFunction)
  (switch int (Variables|Default|GetDialogueTreeIndex)
    (:0
      (bind (_state _optionindex) (CallFunction|AddDialogue "Badger" "Hello There friend! Can you help me?" (Utilities|Array|MakeArray "Yes" "No") "/Engine/VREditor/Sounds/UI/Camera_Shutter.Camera_Shutter"))
      (switch Utilities|FlowControl|Switch|SwitchonEnum_DialogueState _state
        (:NewEnumerator0
          (switch int _optionindex
            (:0
              (bind (_state_2 _optionindex_2) (CallFunction|AddDialogue "Badger" "Oh how great! Let's get going friend!" (Utilities|Array|MakeArray "Lets go!" "On second thought...")))
              (switch Utilities|FlowControl|Switch|SwitchonEnum_DialogueState _state_2
                (:NewEnumerator0
                  (switch int _optionindex_2
                    (:0
                      (bind _state_3 (CallFunction|AddDialogue "Badger" "Awsome! But... I cant move (yet)" (Utilities|Array|MakeArray "Continue")))
                      (switch Utilities|FlowControl|Switch|SwitchonEnum_DialogueState _state_3
                        (:NewEnumerator0
                          (CallFunction|SetDialogueTreeIndex 1)
                          (CallFunction|CloseConversation))))
                    (:1
                      (bind _state_4 (CallFunction|AddDialogue "Badger" "What a bummer..." (Utilities|Array|MakeArray "Continue")))
                      (switch Utilities|FlowControl|Switch|SwitchonEnum_DialogueState _state_4
                        (:NewEnumerator0
                          (CallFunction|RemoveDialogueProgress 2)
                          (CallFunction|CloseConversation))))))))
            (:1
              (bind _state_5 (CallFunction|AddDialogue "Badger" "You break my heart!" (Utilities|Array|MakeArray "Continue") "/Engine/VREditor/Sounds/UI/Camera_Shutter.Camera_Shutter"))
              (switch Utilities|FlowControl|Switch|SwitchonEnum_DialogueState _state_5
                (:NewEnumerator0
                  (CallFunction|ClearDialogueProgress)
                  (CallFunction|CloseConversation))))))))
    (:1
      (bind _state_6 (CallFunction|AddDialogue "Badger" (Utilities|Select :Index (Math|Random|RandomIntegerinRange 0 1) :Option%200 "I'm still stuck here friend..." :Option%201 "Why can't I move!") (Utilities|Array|MakeArray "Continue")))
      (switch Utilities|FlowControl|Switch|SwitchonEnum_DialogueState _state_6
        (:NewEnumerator0
          (CallFunction|ClearDialogueProgress)
          (CallFunction|CloseConversation))))))