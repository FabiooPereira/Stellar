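; BP_LightSource_Base is a base Blueprint for an interactable crystal light source that the player can light up.
; SetInteractableState stores whether interaction is possible and swaps the Crystal material to show that state.
; Interact casts the instigator to BP_Player and, if the player has light, raises the Light intensity, without checking CanInteract.
; A RemoveLight call exists but is disconnected, so the player's light is not removed here.
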(event EventSetInteractableState
  (params (bCanShowInteract? :type Boolean))
  (bind _crystal (Variables|Default|GetCrystal))
  (bind _output_get (Variables|Default|SetbCanInteract? bCanShowInteract?))
  (if _output_get
    (Rendering|Material|SetMaterial _crystal 0 "/AnimationSharing/AnimSharingGreen.AnimSharingGreen")
    (else
      (Rendering|Material|SetMaterial _crystal 0 "/DatasmithContent/Materials/FBXImporter/DeltaGenReference.DeltaGenReference"))))

(event EventInteract
  (params (Instigator :type Actor%20Object%20Reference))
  (bind _asbp_player (Utilities|Casting|CastToBP_Player Instigator))
  (if (Variables|/Game/ThirdPerson/Blueprints/BP_Player.BP_Player_C|GetbHasLight? _asbp_player)
    (Rendering|Components|Light|SetIntensity (Variables|Default|GetLight) 1e+04)))

(fn ConstructionScript)