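; Interactable lamp that the player, BP_PlayerJacob, can light by giving up their carried light, or darken to take the light back.
; Interact checks the player's HasLight against the lamp's lit flag, swaps the Lampa mesh material and calls LightDown or LightUp on the player.
; A text prompt yaws toward the camera every tick and is shown or hidden through SetInteractableState.
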(event EventTick
  (params (DeltaSeconds :type Float%20%28single-precision%29))
  (Transformation|SetWorldRotation (Variables|Default|GetTextRender) (Math|Rotator|MakeRotator 0.0 0.0 (.yaw (Math|Rotator|FindLookatRotation (Transformation|GetSocketLocation (Variables|Default|GetTextRender) "None") (Transformation|GetActorLocation (Game|GetPlayerCameraManager 0))))) false false))

(event EventSetInteractableState
  (params (bCanShowInteract :type Boolean))
  (bind _textrender (Variables|Default|GetTextRender))
  (if bCanShowInteract
    (Rendering|SetVisibility _textrender true false)
    (else
      (Rendering|SetVisibility _textrender false false))))

(event EventConversationClosed)

(event EventInteract
  (params (Instigator :type Actor%20Object%20Reference))
  (bind _lampa (Variables|Default|GetLampa))
  (bind _asbp_player_jacob (Utilities|Casting|CastToBP_PlayerJacob Instigator))
  (Variables|Default|SetPlayer _asbp_player_jacob)
  (if (Variables|/Game/ThirdPerson/Blueprints/BP_PlayerJacob.BP_PlayerJacob_C|GetHasLight _asbp_player_jacob)
    (if (not (Variables|Default|GetLampIsLIt))
      (Rendering|Material|SetMaterial _lampa 0 "/DatasmithContent/Materials/Arealight.Arealight")
      (Default|LightDown (Variables|Default|GetPlayer))
      (Variables|Default|SetLampIsLIt true))
    (elif (Variables|Default|GetLampIsLIt)
      (Rendering|Material|SetMaterial _lampa 0 "/Engine/BasicShapes/BasicShapeMaterial.BasicShapeMaterial")
      (Default|LightUp (Variables|Default|GetPlayer))
      (Variables|Default|SetLampIsLIt false))))

(fn ConstructionScript)

(fn LitLamp)