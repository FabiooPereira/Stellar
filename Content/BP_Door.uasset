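; BP_Door is a door actor that opens when enough pressure switches are active at once.
; SwitchActivated and SwitchDeactivated adjust a running count and compare it to PressureSwitchesNeeded, playing or reversing the DoorActivation timeline.
; The timeline's DoorPosition track drives the Door component's relative yaw, so it swings open and back from wherever it currently is.
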(event Custom|SwitchActivated
  (Math|Integer|IncrementInt (Variables|Default|GetPressureSwitchesActive)
    (:%20%20
      (if (>= (Variables|Default|GetPressureSwitchesActive) (Variables|Default|GetPressureSwitchesNeeded))
        (bind _doorposition (Timeline|DoorActivation Play)
          (:Update
            (Transformation|SetRelativeRotation (Variables|Default|GetDoor) (Math|Rotator|MakeRotator 0.0 0.0 _doorposition) false false)))
        (else
          (Timeline|DoorActivation Reverse))))))

(event Custom|SwitchDeactivated
  (Math|Integer|DecrementInt (Variables|Default|GetPressureSwitchesActive)
    (:%20%20
      (if (>= (Variables|Default|GetPressureSwitchesActive) (Variables|Default|GetPressureSwitchesNeeded))
        (bind _doorposition (Timeline|DoorActivation Play)
          (:Update
            (Transformation|SetRelativeRotation (Variables|Default|GetDoor) (Math|Rotator|MakeRotator 0.0 0.0 _doorposition) false false)))
        (else
          (Timeline|DoorActivation Reverse))))))

(event EventBeginPlay)

(event Collision|EventActorBeginOverlap
  (params (OtherActor :type Actor%20Object%20Reference)))

(event EventTick
  (params (DeltaSeconds :type Float%20%28single-precision%29)))

(fn ConstructionScript)