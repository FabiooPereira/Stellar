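; Fixed-position camera that rotates to follow the player and becomes the active view while the player overlaps it.
; Each tick it lerps toward the look-at rotation; any axis straying past its limit from the initial rotation becomes that signed limit, not an offset from the start.
; Overlap begin and end set a flag, rechecked after a delay before switching view target and character active camera between this and BP_TracingCamera.
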(event EventBeginPlay
  (Variables|Default|SetPlayerCharacter (Game|GetPlayerCharacter 0))
  (Variables|Default|SetInitialRotation (Transformation|GetWorldRotation (Variables|CameraActor|GetCameraComponent))))

(event Collision|EventActorBeginOverlap
  (params (OtherActor :type Actor%20Object%20Reference))
  ;[1 1 1] StartOfCollision
  (if (== OtherActor (Variables|Default|GetPlayerCharacter))
    (Variables|Default|SetCameraSwitch true)
    (Utilities|FlowControl|Delay 2.0)
    (if (Variables|Default|GetCameraSwitch)
      (Game|Player|SetViewTargetwithBlend (Game|GetPlayerController 0) self 0.0 "VTBlend_EaseIn" 2.0 false)
      (bind _asgrupp_onion_character (Utilities|Casting|CastToGruppOnionCharacter (Variables|Default|GetPlayerCharacter)))
      (Class|GruppOnionCharacter|SetActiveCamera _asgrupp_onion_character (Variables|CameraActor|GetCameraComponent)))))

(event EventTick
  (params (DeltaSeconds :type Float%20%28single-precision%29))
  (bind _finalrotation (CallFunction|UpdateRotationtoMove (Variables|Default|GetInitialRotation) (Math|Rotator|FindLookatRotation (Transformation|GetWorldLocation (Variables|CameraActor|GetCameraComponent)) (Transformation|GetActorLocation (Variables|Default|GetPlayerCharacter))) (Variables|Default|GetXLimitRotation%28Roll%29) (Variables|Default|GetYLimitRotation%28Pitch%29) (Variables|Default|GetZLimitRotation%28Yaw%29)))
  (Transformation|SetWorldRotation (Variables|CameraActor|GetCameraComponent) (Math|Rotator|Lerp(Rotator) (Transformation|GetSocketRotation (Variables|CameraActor|GetCameraComponent) "None") _finalrotation (* DeltaSeconds (Variables|Default|GetLerpForce))) false false))

(event Collision|EventActorEndOverlap
  (params (OtherActor :type Actor%20Object%20Reference))
  ;[1 1 1] EndOfCollision
  (if (== OtherActor (Variables|Default|GetPlayerCharacter))
    (Variables|Default|SetCameraSwitch false)
    (Utilities|FlowControl|Delay 2.0)
    (if (not (Variables|Default|GetCameraSwitch))
      (bind _returnvalue (Actor|GetActorOfClass "/Game/BP_TracingCamera.BP_TracingCamera_C"))
      (Game|Player|SetViewTargetwithBlend (Game|GetPlayerController 0) _returnvalue 0.0 "VTBlend_EaseOut" 2.0 false)
      (bind _asgrupp_onion_character (Utilities|Casting|CastToGruppOnionCharacter (Variables|Default|GetPlayerCharacter)))
      (bind _returnvalue_2 (Actor|GetActorOfClass "/Game/BP_TracingCamera.BP_TracingCamera_C"))
      (Class|GruppOnionCharacter|SetActiveCamera _asgrupp_onion_character (Variables|/Script/Engine.CameraActor|GetCameraComponent _returnvalue_2)))))

(fn ConstructionScript)

(fn UpdateRotationtoMove
  (params (InitialRotation :type Rotator) (TargetRotation :type Rotator) (LimitX%28Roll%29 :type Float%20%28double-precision%29) (LimitY%28Pitch%29 :type Float%20%28double-precision%29) (LimitZ%28Yaw%29 :type Float%20%28double-precision%29))
  (bind _returnvalue (Math|Rotator|Delta(Rotator) InitialRotation TargetRotation))
  (bind _finalrotation (CallFunction|UpdateRotation (.roll TargetRotation) LimitX%28Roll%29 (.roll _returnvalue)))
  (bind _finalrotation_2 (CallFunction|UpdateRotation (.pitch TargetRotation) LimitY%28Pitch%29 (.pitch _returnvalue)))
  (bind _finalrotation_3 (CallFunction|UpdateRotation (.yaw TargetRotation) LimitZ%28Yaw%29 (.yaw _returnvalue)))
  (return (Math|Rotator|MakeRotator _finalrotation _finalrotation_2 _finalrotation_3)))

(fn UpdateRotation
  (params (LookToplayerRotation :type Float%20%28double-precision%29) (Limit :type Float%20%28double-precision%29) (DeltaRotation :type Float%20%28double-precision%29))
  (LocalVariables|SetInitialRotaionValue LookToplayerRotation)
  (if (> (Math|Float|Absolute(Float) DeltaRotation) Limit)
    (LocalVariables|SetFinalRotationvalue (* (Math|Float|Sign(Float) (LocalVariables|GetInitialRotaionValue)) Limit))
    (else
      (LocalVariables|SetFinalRotationvalue (LocalVariables|GetInitialRotaionValue))))
  (return (LocalVariables|GetFinalRotationvalue)))