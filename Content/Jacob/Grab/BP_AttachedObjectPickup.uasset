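; Grabbable cube that BP_PlayerJacob can pick up and drop, and that detects pressure switches.
; Interaction state toggles the HUD grab prompt and custom-depth highlight, while InteractGrab calls the player's grab or drop, driving Niagara and dust effects.
; Box overlaps with BP_PressureSwitch_Parent set IsTriggeringSwitch and swap the cube material; that flag also keeps the highlight on.
; Physics force and reset events are labelled inactive; the placement check is marked to be moved.
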(event OnComponentBeginOverlap(Box)
  (params (OverlappedComponent :type Primitive%20Component%20Object%20Reference) (OtherActor :type Actor%20Object%20Reference) (OtherComp :type Primitive%20Component%20Object%20Reference) (OtherBodyIndex :type Integer) (bFromSweep :type Boolean) (SweepResult :type Hit%20Result%20Structure%20%28by%20ref%29))
  ;[1 1 1] Check Object Placement(Should be moved)
  (bind _asbp_pressure_switch_parent (Utilities|Casting|CastToBP_PressureSwitch_Parent OtherActor))
  (if (Collision|IsOverlappingActor (Variables|Default|GetBox) _asbp_pressure_switch_parent :!class /Script/Engine.PrimitiveComponent)
    (Variables|Default|SetIsTriggeringSwitch true)
    (Rendering|Material|SetMaterial (Variables|Default|GetCube) 0 "/Game/StarterContent/Blueprints/Assets/M_LightStage_Arrows.M_LightStage_Arrows")
    (else
      (Variables|Default|SetIsTriggeringSwitch false)
      (Rendering|Material|SetMaterial (Variables|Default|GetCube) 0 "/Game/Elsa/Materials/Pillar_Alter_Crystal_Stones/M_Pillar_Alter_Crystal_Stones.M_Pillar_Alter_Crystal_Stones"))))

(event OnComponentEndOverlap(Box)
  (params (OverlappedComponent :type Primitive%20Component%20Object%20Reference) (OtherActor :type Actor%20Object%20Reference) (OtherComp :type Primitive%20Component%20Object%20Reference) (OtherBodyIndex :type Integer))
  ;[1 1 1] Check Object Placement(Should be moved)
  (bind _asbp_pressure_switch_parent (Utilities|Casting|CastToBP_PressureSwitch_Parent OtherActor))
  (if (Collision|IsOverlappingActor (Variables|Default|GetBox) _asbp_pressure_switch_parent :!class /Script/Engine.PrimitiveComponent)
    (Variables|Default|SetIsTriggeringSwitch true)
    (Rendering|Material|SetMaterial (Variables|Default|GetCube) 0 "/Game/StarterContent/Blueprints/Assets/M_LightStage_Arrows.M_LightStage_Arrows")
    (else
      (Variables|Default|SetIsTriggeringSwitch false)
      (Rendering|Material|SetMaterial (Variables|Default|GetCube) 0 "/Game/Elsa/Materials/Pillar_Alter_Crystal_Stones/M_Pillar_Alter_Crystal_Stones.M_Pillar_Alter_Crystal_Stones"))))

(event EventBeginPlay)

(event Collision|EventActorBeginOverlap
  (params (OtherActor :type Actor%20Object%20Reference)))

(event EventInteractGrab
  (params (Instigator :type Actor%20Object%20Reference))
  ;[1 1 1] Grab/Drop
  (bind _asbp_player_jacob (Utilities|Casting|CastToBP_PlayerJacob Instigator))
  (if (Variables|/Game/ThirdPerson/Blueprints/BP_PlayerJacob.BP_PlayerJacob_C|GetIsHoldingObject _asbp_player_jacob)
    (if (Variables|/Game/ThirdPerson/Blueprints/BP_PlayerJacob.BP_PlayerJacob_C|GetCanDropObject _asbp_player_jacob)
      (Default|DropObject _asbp_player_jacob)
      (CallFunction|TextEnable)
      (Components|Activation|Deactivate (Variables|Default|GetNiagara))
      (Niagara|ReinitializeSystem (Variables|Default|GetDust)))
    (elif (Variables|Default|GetbCanInteract?)
      (Default|GrabObject _asbp_player_jacob)
      (CallFunction|TextDisable)
      (Components|Activation|Activate (Variables|Default|GetNiagara) false))))

(event EventTick
  (params (DeltaSeconds :type Float%20%28single-precision%29)))

(event EventResetForce
  (bind _cube (Variables|Default|GetCube))
  ;[1 1 1] Reset Force(Inactive)
  (if (Physics|IsSimulatingPhysics _cube "None")
    (Physics|SetSimulatePhysics _cube false)
    (Transformation|SetActorLocation (Transformation|GetWorldLocation _cube) false false)
    (Transformation|AttachComponentToComponent (Variables|Default|GetCube) (Variables|Default|GetDefaultSceneRoot) "None" "KeepWorld" "KeepWorld" "KeepWorld" true)))

(event EventApplyForcewithDirection
  (params (DirectionVector :type Vector :default "0, 0, 0") (Power :type Float%20%28double-precision%29))
  ;[1 1 1] Apply Force With Direction(Inactive)
  (Physics|SetSimulatePhysics (Variables|Default|GetCube) true))

(event EventSetInteractableState
  (params (bCanShowInteract :type Boolean))
  ;[1 1 1] Interact(Start/End Overlap)
  (bind _asbp_player_jacob (Utilities|Casting|CastToBP_PlayerJacob (Game|GetPlayerCharacter 0)))
  (if (not (or (Variables|/Game/ThirdPerson/Blueprints/BP_PlayerJacob.BP_PlayerJacob_C|GetIsHoldingObject _asbp_player_jacob) (Variables|/Game/ThirdPerson/Blueprints/BP_PlayerJacob.BP_PlayerJacob_C|GetIsPushingObject _asbp_player_jacob)))
    (bind _output_get (Variables|Default|SetbCanInteract? bCanShowInteract))
    (if _output_get
      (CallFunction|TextEnable)
      (Rendering|SetRenderCustomDepth (Variables|Default|GetCube) true)
      (else
        (CallFunction|TextDisable)
        (if (not (Variables|Default|GetIsTriggeringSwitch))
          (Rendering|SetRenderCustomDepth (Variables|Default|GetCube) false))))))

(fn ConstructionScript)

(fn TextDisable
  (bind _as_new_hud (Variables|Default|GetAs%20New%20HUD)
    (:then
      (Default|SetTextInputPlayer (Variables|/Game/Jacob/UI/NewHUD.NewHUD_C|GetUIRef _as_new_hud) "" "" false))
    (:else)))

(fn TextEnable
  (bind _asnew_hud (Utilities|Casting|CastToNewHUD (HUD|GetHUD (Game|GetPlayerController 0))))
  (bind _output_get (Variables|Default|SetAs%20New%20HUD _asnew_hud))
  (Default|SetTextInputPlayer (Variables|/Game/Jacob/UI/NewHUD.NewHUD_C|GetUIRef _output_get) "GRAB: B" "GRAB: E" true))