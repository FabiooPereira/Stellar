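; Attached-object pickup for the Crystal Cave that only responds to interactable-state changes while its referenced Lamp is lit.
; When lit, SetInteractableState stores CanInteract, toggles the button prompt and switches custom depth rendering on the Cube.
; Custom depth stays on when interaction ends if IsTriggeringSwitch is set.
; Tick calls ChangeTextOnInput every frame with gamepad and keyboard labels for the prompt.
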(event EventBeginPlay
  (|CallParentFunction))

(event Collision|EventActorBeginOverlap
  (params (OtherActor :type Actor%20Object%20Reference))
  (|CallParentFunction OtherActor) ; This node is disabled and will not be called.\nDrag off pins to build functionality.
)

(event EventTick
  (params (DeltaSeconds :type Float%20%28single-precision%29))
  (|CallParentFunction DeltaSeconds)
  (CallFunction|ChangeTextonInput "B" "E"))

(event EventSetInteractableState
  (params (bCanShowInteract :type Boolean))
  ;[1 1 1] Interact(Start/End Overlap)
  (if (Variables|/Game/ThirdPerson/Blueprints/BP_Lamp.BP_Lamp_C|GetLampIsLIt (Variables|Default|GetLamp))
    (bind _output_get (Variables|Default|SetbCanInteract? bCanShowInteract))
    (if _output_get
      (Rendering|SetVisibility (Variables|Default|GetInteractButtonText) true false)
      (Rendering|SetRenderCustomDepth (Variables|Default|GetCube) true)
      (else
        (Rendering|SetVisibility (Variables|Default|GetInteractButtonText) false false)
        (if (not (Variables|Default|GetIsTriggeringSwitch))
          (Rendering|SetRenderCustomDepth (Variables|Default|GetCube) false))))
    (elif (Variables|Default|GetIsTriggeringSwitch)
      _)))

(fn ConstructionScript
  (|CallParentFunction))