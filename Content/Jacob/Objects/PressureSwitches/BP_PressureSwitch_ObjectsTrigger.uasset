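; Pressure switch that activates its linked BridgesToActivate when the Jacob player or a crystal pickup overlaps its box.
; Overlap macros keep a count capped at two, so leaving while two are counted does not release the switch.
; A DoOnce gates activation, which messages the bridges and lights the plate material.
; The final exit sends the deactivate message, restores the normal material and resets the gate.
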(event OnComponentBeginOverlap(Box)
  (params (OverlappedComponent :type Primitive%20Component%20Object%20Reference) (OtherActor :type Actor%20Object%20Reference) (OtherComp :type Primitive%20Component%20Object%20Reference) (OtherBodyIndex :type Integer) (bFromSweep :type Boolean) (SweepResult :type Hit%20Result%20Structure%20%28by%20ref%29))
  (bind _returnvalue (Utilities|GetClass OtherActor))
  ;[1 1 1] Switch Trigger
  (if (or (Utilities|ClassIsChildOf _returnvalue "/Game/ThirdPerson/Blueprints/BP_PlayerJacob.BP_PlayerJacob_C") (Utilities|ClassIsChildOf _returnvalue "/Game/Jacob/Grab/BP_AttachedObjectPickup_Crystal.BP_AttachedObjectPickup_Crystal_C"))
    (|CanBeginOverlap_2)
    (Utilities|FlowControl|DoOnce false
      (:Completed
        (Class|BPIEventTrigger|ObjectActivated(Message) (Variables|Default|GetBridgesToActivate))
        (Rendering|Material|SetMaterial (Variables|Default|GetSwitch) 0 "/Game/Linnea/Textures/PressurePlates/M_PressurePlateLight.M_PressurePlateLight")))))

(event OnComponentEndOverlap(Box)
  (params (OverlappedComponent :type Primitive%20Component%20Object%20Reference) (OtherActor :type Actor%20Object%20Reference) (OtherComp :type Primitive%20Component%20Object%20Reference) (OtherBodyIndex :type Integer))
  (bind _returnvalue (Utilities|GetClass OtherActor))
  (bind _switch (Variables|Default|GetSwitch))
  (bind _bridgestoactivate (Variables|Default|GetBridgesToActivate))
  ;[1 1 1] Switch Trigger
  (if (or (Utilities|ClassIsChildOf _returnvalue "/Game/ThirdPerson/Blueprints/BP_PlayerJacob.BP_PlayerJacob_C") (Utilities|ClassIsChildOf _returnvalue "/Game/Jacob/Grab/BP_AttachedObjectPickup_Crystal.BP_AttachedObjectPickup_Crystal_C"))
    (|CanEndOverlap_2)
    (Class|BPIEventTrigger|ObjectDeactivated(Message) _bridgestoactivate)
    (Rendering|Material|SetMaterial _switch 0 "/Game/Linnea/Textures/PressurePlates/M_PressurePlateNormal.M_PressurePlateNormal")
    (Utilities|FlowControl|DoOnce false) ; enters at Reset
  ))

(event EventBeginPlay)

(event Collision|EventActorBeginOverlap
  (params (OtherActor :type Actor%20Object%20Reference)))

(event EventTick
  (params (DeltaSeconds :type Float%20%28single-precision%29)))

(fn ConstructionScript)