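; Pressure switch that responds to fox trigger objects (BP_ObjectToTrigger_Fox) entering or leaving its overlap box.
; Begin and end overlap check the other actor's class, then send activated or deactivated messages to the linked ObjectToActivate.
; The same events set the emissive strength on the fox's material, lighting it while it overlaps the switch and switching the glow off when it leaves.
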(event OnComponentBeginOverlap(OverlapBox)
  (params (OverlappedComponent :type Primitive%20Component%20Object%20Reference) (OtherActor :type Actor%20Object%20Reference) (OtherComp :type Primitive%20Component%20Object%20Reference) (OtherBodyIndex :type Integer) (bFromSweep :type Boolean) (SweepResult :type Hit%20Result%20Structure%20%28by%20ref%29))
  ;[1 1 1] Switch Trigger
  (if (Utilities|ClassIsChildOf (Utilities|GetClass OtherActor) "/Game/Jacob/Objects/Other/BP_ObjectToTrigger_Fox.BP_ObjectToTrigger_Fox_C")
    (Class|BPIEventTrigger|ObjectActivated(Message) (Variables|Default|GetObjectToActivate))
    (bind _asbp_cube (Utilities|Casting|CastToBP_ObjectToTrigger_Fox OtherActor))
    (Rendering|Material|SetScalarParameterValue (Variables|/Game/Jacob/Objects/Other/BP_ObjectToTrigger_Fox.BP_ObjectToTrigger_Fox_C|GetFoxMaterial _asbp_cube) "Emissive Strength" 1e+01 :!class /Script/Engine.MaterialInstanceDynamic)))

(event OnComponentEndOverlap(OverlapBox)
  (params (OverlappedComponent :type Primitive%20Component%20Object%20Reference) (OtherActor :type Actor%20Object%20Reference) (OtherComp :type Primitive%20Component%20Object%20Reference) (OtherBodyIndex :type Integer))
  ;[1 1 1] Switch Trigger
  (if (Utilities|ClassIsChildOf (Utilities|GetClass OtherActor) "/Game/Jacob/Objects/Other/BP_ObjectToTrigger_Fox.BP_ObjectToTrigger_Fox_C")
    (Class|BPIEventTrigger|ObjectDeactivated(Message) (Variables|Default|GetObjectToActivate))
    (bind _asbp_cube (Utilities|Casting|CastToBP_ObjectToTrigger_Fox OtherActor))
    (Rendering|Material|SetScalarParameterValue (Variables|/Game/Jacob/Objects/Other/BP_ObjectToTrigger_Fox.BP_ObjectToTrigger_Fox_C|GetFoxMaterial _asbp_cube) "Emissive Strength" 0.0 :!class /Script/Engine.MaterialInstanceDynamic)))

(event EventBeginPlay
  (|CallParentFunction))

(event Collision|EventActorBeginOverlap
  (params (OtherActor :type Actor%20Object%20Reference)))

(event EventTick
  (params (DeltaSeconds :type Float%20%28single-precision%29))
  (|CallParentFunction DeltaSeconds) ; This node is disabled and will not be called.\nDrag off pins to build functionality.
)

(fn ConstructionScript
  (|CallParentFunction))