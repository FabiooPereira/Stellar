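; Pressure switch trigger that responds to AI_Alan or the mounted player entering and leaving its box.
; On entry it messages its linked bridges to activate and swaps the base to an emissive material, guarded by a DoOnce.
; An overlap counter capped at two holds the switch on when one of two occupants leaves.
; Otherwise, exit deactivates the bridges, restores the basic material and resets the DoOnce.
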(event OnComponentBeginOverlap(Box)
  (params (OverlappedComponent :type Primitive%20Component%20Object%20Reference) (OtherActor :type Actor%20Object%20Reference) (OtherComp :type Primitive%20Component%20Object%20Reference) (OtherBodyIndex :type Integer) (bFromSweep :type Boolean) (SweepResult :type Hit%20Result%20Structure%20%28by%20ref%29))
  (bind _returnvalue (Utilities|GetClass OtherActor))
  ;[1 1 1] Switch Trigger
  (if (or (Utilities|ClassIsChildOf _returnvalue "/Game/AICompanion/AI_Alan.AI_Alan_C") (Utilities|ClassIsChildOf _returnvalue "/Game/ThirdPerson/Blueprints/BP_Player_Mounted.BP_Player_Mounted_C"))
    (|CanBeginOverlap_2)
    (Utilities|FlowControl|DoOnce false
      (:Completed
        (Class|BPIEventTrigger|ObjectActivated(Message) (Variables|Default|GetBridgesToActivate))
        (Rendering|Material|SetMaterial (Variables|Default|GetBase) 0 "/Engine/EngineMaterials/EmissiveMeshMaterial.EmissiveMeshMaterial")))))

(event OnComponentEndOverlap(Box)
  (params (OverlappedComponent :type Primitive%20Component%20Object%20Reference) (OtherActor :type Actor%20Object%20Reference) (OtherComp :type Primitive%20Component%20Object%20Reference) (OtherBodyIndex :type Integer))
  (bind _returnvalue (Utilities|GetClass OtherActor))
  (bind _base (Variables|Default|GetBase))
  (bind _bridgestoactivate (Variables|Default|GetBridgesToActivate))
  ;[1 1 1] Switch Trigger
  (if (or (Utilities|ClassIsChildOf _returnvalue "/Game/AICompanion/AI_Alan.AI_Alan_C") (Utilities|ClassIsChildOf _returnvalue "/Game/ThirdPerson/Blueprints/BP_Player_Mounted.BP_Player_Mounted_C"))
    (|CanEndOverlap_2)
    (Class|BPIEventTrigger|ObjectDeactivated(Message) _bridgestoactivate)
    (Rendering|Material|SetMaterial _base 0 "/Engine/BasicShapes/BasicShapeMaterial.BasicShapeMaterial")
    (Utilities|FlowControl|DoOnce false) ; enters at Reset
  ))

(event EventBeginPlay)

(event Collision|EventActorBeginOverlap
  (params (OtherActor :type Actor%20Object%20Reference)))

(event EventTick
  (params (DeltaSeconds :type Float%20%28single-precision%29)))

(fn ConstructionScript)