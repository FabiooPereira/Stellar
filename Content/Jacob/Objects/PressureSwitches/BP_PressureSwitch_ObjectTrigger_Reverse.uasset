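; Reversed pressure switch that activates a linked wall object when the player (Jacob) or a crystal pickup leaves its overlap box.
; End overlap passes a class check and a DoOnce, then CanEndOverlap decrements and prints the overlap count, continuing to activation unless the count was two.
; Begin overlap is empty, and leftover logic for snapping grabbed objects onto the switch is unconnected and marked buggy.
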(event OnComponentBeginOverlap(OverlapBox)
  (params (OverlappedComponent :type Primitive%20Component%20Object%20Reference) (OtherActor :type Actor%20Object%20Reference) (OtherComp :type Primitive%20Component%20Object%20Reference) (OtherBodyIndex :type Integer) (bFromSweep :type Boolean) (SweepResult :type Hit%20Result%20Structure%20%28by%20ref%29))
  ;[1 1 1] Switch Trigger
)

(event OnComponentEndOverlap(OverlapBox)
  (params (OverlappedComponent :type Primitive%20Component%20Object%20Reference) (OtherActor :type Actor%20Object%20Reference) (OtherComp :type Primitive%20Component%20Object%20Reference) (OtherBodyIndex :type Integer))
  (bind _returnvalue (Utilities|GetClass OtherActor))
  ;[1 1 1] Switch Trigger
  (if (or (Utilities|ClassIsChildOf _returnvalue "/Game/ThirdPerson/Blueprints/BP_PlayerJacob.BP_PlayerJacob_C") (Utilities|ClassIsChildOf _returnvalue "/Game/Jacob/Grab/BP_AttachedObjectPickup_Crystal.BP_AttachedObjectPickup_Crystal_C"))
    (Utilities|FlowControl|DoOnce false
      (:Completed
        (|CanEndOverlap)
        (Default|ObjectActivated (Variables|Default|GetWallToActivate))))))

(event EventBeginPlay
  (|CallParentFunction) ; This node is disabled and will not be called.\nDrag off pins to build functionality.
)

(event Collision|EventActorBeginOverlap
  (params (OtherActor :type Actor%20Object%20Reference)))

(event EventTick
  (params (DeltaSeconds :type Float%20%28single-precision%29))
  (|CallParentFunction DeltaSeconds) ; This node is disabled and will not be called.\nDrag off pins to build functionality.
)

(fn ConstructionScript
  (|CallParentFunction))