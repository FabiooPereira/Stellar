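; A triggered door that swings open on a yaw timeline, with sound, once enough linked triggers are active.
; Activation and deactivation events adjust a counter and share one threshold check, reversing the door below it unless PlayOnce is set.
; Until the first opening finishes, it freezes player movement, switches to UI-only input and blends the view to the door.
; It then restores player view, input and speed.
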(event EventBeginPlay)

(event Collision|EventActorBeginOverlap
  (params (OtherActor :type Actor%20Object%20Reference)))

(event EventTick
  (params (DeltaSeconds :type Float%20%28single-precision%29)))

(event EventObjectDeactivated
  ;[1 1 1] Door Activation/Deactivation
  (Math|Integer|DecrementInt (Variables|Default|GetTriggersActive)
    (:%20%20
      (if (>= (Variables|Default|GetTriggersActive) (Variables|Default|GetTriggersNeeded))
        (if (Variables|Default|GetbPlayOnce)
          (Utilities|FlowControl|DoOnce false
            (:Completed
              _)))
        (if (Variables|Default|GetPlayed)
          _
          (else
            (CallFunction|FocusStart)))
        (CallFunction|PlaySound)
        (bind _doorposition (Timeline|DoorActivation Play)
          (:Update
            (Transformation|SetRelativeRotation (Variables|Default|GetDoor) (Math|Rotator|MakeRotator 0.0 0.0 _doorposition) false false))
          (:Finished
            (if (not (Variables|Default|GetPlayed))
              (CallFunction|FocusEnd)
              (Variables|Default|SetPlayed true))))
        (elif (not (Variables|Default|GetbPlayOnce))
          (CallFunction|PlaySound)
          (Timeline|DoorActivation Reverse))))))

(event EventObjectActivated
  ;[1 1 1] Door Activation/Deactivation
  (Math|Integer|IncrementInt (Variables|Default|GetTriggersActive)
    (:%20%20
      (if (>= (Variables|Default|GetTriggersActive) (Variables|Default|GetTriggersNeeded))
        (if (Variables|Default|GetbPlayOnce)
          (Utilities|FlowControl|DoOnce false
            (:Completed
              _)))
        (if (Variables|Default|GetPlayed)
          _
          (else
            (CallFunction|FocusStart)))
        (CallFunction|PlaySound)
        (bind _doorposition (Timeline|DoorActivation Play)
          (:Update
            (Transformation|SetRelativeRotation (Variables|Default|GetDoor) (Math|Rotator|MakeRotator 0.0 0.0 _doorposition) false false))
          (:Finished
            (if (not (Variables|Default|GetPlayed))
              (CallFunction|FocusEnd)
              (Variables|Default|SetPlayed true))))
        (elif (not (Variables|Default|GetbPlayOnce))
          (CallFunction|PlaySound)
          (Timeline|DoorActivation Reverse))))))

(event EventFocusEnd
  ;[1 1 1] Sets this local camera view as the player player controller view
  (Game|Player|SetViewTargetwithBlend (Game|GetPlayerController 0) (Game|GetPlayerCharacter 0) 2.0 "VTBlend_EaseInOut" 2.0 true)
  (Input|SetInputModeGameOnly (Game|GetPlayerController 0) true)
  (bind _asbp_third_person_character (Utilities|Casting|CastToBP_ThirdPersonCharacter (Game|GetPlayerCharacter 0)))
  (Variables|/Script/Engine.CharacterMovementComponent|SetMinAnalogWalkSpeed (Variables|/Script/Engine.Character|GetCharacterMovement _asbp_third_person_character) 9e+01)
  (Variables|/Script/Engine.CharacterMovementComponent|SetMaxWalkSpeed (Variables|/Script/Engine.Character|GetCharacterMovement _asbp_third_person_character) 3.5e+02))

(event EventFocusStart
  ;[1 1 1] Sets this players local camera view as the player player controller view
  (bind _asbp_third_person_character (Utilities|Casting|CastToBP_ThirdPersonCharacter (Game|GetPlayerCharacter 0)))
  (Variables|/Script/Engine.CharacterMovementComponent|SetMinAnalogWalkSpeed (Variables|/Script/Engine.Character|GetCharacterMovement _asbp_third_person_character) 0.0)
  (Variables|/Script/Engine.CharacterMovementComponent|SetMaxWalkSpeed (Variables|/Script/Engine.Character|GetCharacterMovement _asbp_third_person_character) 0.0)
  (Input|SetInputModeUIOnly (Game|GetPlayerController 0) 0 "DoNotLock" true)
  (Game|Player|SetViewTargetwithBlend (Game|GetPlayerController 0) self 2.0 "VTBlend_EaseInOut" 2.0 true))

(fn ConstructionScript)

(fn PlaySound
  (Audio|PlaySoundatLocation "/Game/Kio/Import/SFX_Bridge.SFX_Bridge" (Transformation|GetWorldLocation (Variables|Default|GetDoor)) "0, 0, 0" 0.2 0.4 0.0 0 0 0 0))