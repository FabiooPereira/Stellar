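; Puzzle clue actor with three boxes that slide and light up while something overlaps its trigger area.
; Overlap begin and end set a reverse flag and call MoveCubes, which plays or reverses three timelines, each started from the previous one's update.
; The timelines drive each box's relative Y position.
; When each finishes, it switches the emissive strength on that box's dynamic fox statue material on or off.
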(event OnComponentBeginOverlap(OverlapArea)
  (params (OverlappedComponent :type Primitive%20Component%20Object%20Reference) (OtherActor :type Actor%20Object%20Reference) (OtherComp :type Primitive%20Component%20Object%20Reference) (OtherBodyIndex :type Integer) (bFromSweep :type Boolean) (SweepResult :type Hit%20Result%20Structure%20%28by%20ref%29))
  ;[1 1 1] Overlap Begin/End
  (Variables|Default|SetShouldReverse false)
  (CallFunction|MoveCubes))

(event OnComponentEndOverlap(OverlapArea)
  (params (OverlappedComponent :type Primitive%20Component%20Object%20Reference) (OtherActor :type Actor%20Object%20Reference) (OtherComp :type Primitive%20Component%20Object%20Reference) (OtherBodyIndex :type Integer))
  ;[1 1 1] Overlap Begin/End
  (Variables|Default|SetShouldReverse true)
  (CallFunction|MoveCubes))

(event Custom|MoveCubes
  ;[1 1 1] Move Cubes
  (if (Variables|Default|GetShouldReverse)
    (bind _newtrack_0 (Timeline|Timeline Reverse)
      (:Update
        (Transformation|SetRelativeLocation (Variables|Default|GetBox1) (Math|Vector|MakeVector -3e+01 _newtrack_0 -49.0) false false)
        (if (Variables|Default|GetShouldReverse)
          (bind _newtrack_0_2 (Timeline|Timeline_1 Reverse)
            (:Update
              (Transformation|SetRelativeLocation (Variables|Default|GetBox2) (Math|Vector|MakeVector 0.0 _newtrack_0_2 -49.0) false false)
              (if (Variables|Default|GetShouldReverse)
                (bind _newtrack_0_3 (Timeline|Timeline_0 Reverse)
                  (:Update
                    (Transformation|SetRelativeLocation (Variables|Default|GetBox3) (Math|Vector|MakeVector 3e+01 _newtrack_0_3 -49.0) false false))
                  (:Finished
                    (if (Variables|Default|GetShouldReverse)
                      (Rendering|Material|SetScalarParameterValue (Variables|Default|GetFoxMaterial3) "Emissive Strength" 0.0 :!class /Script/Engine.MaterialInstanceDynamic)
                      (else
                        (Rendering|Material|SetScalarParameterValue (Variables|Default|GetFoxMaterial3) "Emissive Strength" 1e+01 :!class /Script/Engine.MaterialInstanceDynamic)))))
                (else
                  (Timeline|Timeline_0 Play))))
            (:Finished
              (if (Variables|Default|GetShouldReverse)
                (Rendering|Material|SetScalarParameterValue (Variables|Default|GetFoxMaterial2) "Emissive Strength" 0.0 :!class /Script/Engine.MaterialInstanceDynamic)
                (else
                  (Rendering|Material|SetScalarParameterValue (Variables|Default|GetFoxMaterial2) "Emissive Strength" 1e+01 :!class /Script/Engine.MaterialInstanceDynamic)))))
          (else
            (Timeline|Timeline_1 Play))))
      (:Finished
        (if (Variables|Default|GetShouldReverse)
          (Rendering|Material|SetScalarParameterValue (Variables|Default|GetFoxMaterial1) "Emissive Strength" 0.0 :!class /Script/Engine.MaterialInstanceDynamic)
          (else
            (Rendering|Material|SetScalarParameterValue (Variables|Default|GetFoxMaterial1) "Emissive Strength" 1e+01 :!class /Script/Engine.MaterialInstanceDynamic)))))
    (else
      (Timeline|Timeline Play))))

(event EventBeginPlay
  (bind _returnvalue (Rendering|Material|CreateDynamicMaterialInstance (Variables|Default|GetBox1) 0 "/Game/Elsa/Materials/FoxStatue/MI_FoxStatue.MI_FoxStatue" "None" :!class /Script/Engine.PrimitiveComponent))
  (bind _output_get (Variables|Default|SetFoxMaterial1 _returnvalue))
  (Rendering|Material|SetMaterial (Variables|Default|GetBox1) 0 _output_get)
  (bind _returnvalue_2 (Rendering|Material|CreateDynamicMaterialInstance (Variables|Default|GetBox2) 0 "/Game/Elsa/Materials/FoxStatue/MI_FoxStatue.MI_FoxStatue" "None" :!class /Script/Engine.PrimitiveComponent))
  (bind _output_get_2 (Variables|Default|SetFoxMaterial2 _returnvalue_2))
  (Rendering|Material|SetMaterial (Variables|Default|GetBox2) 0 _output_get_2)
  (bind _returnvalue_3 (Rendering|Material|CreateDynamicMaterialInstance (Variables|Default|GetBox3) 0 "/Game/Elsa/Materials/FoxStatue/MI_FoxStatue.MI_FoxStatue" "None" :!class /Script/Engine.PrimitiveComponent))
  (bind _output_get_3 (Variables|Default|SetFoxMaterial3 _returnvalue_3))
  (Rendering|Material|SetMaterial (Variables|Default|GetBox3) 0 _output_get_3))

(event Collision|EventActorBeginOverlap
  (params (OtherActor :type Actor%20Object%20Reference)))

(event EventTick
  (params (DeltaSeconds :type Float%20%28single-precision%29)))

(fn ConstructionScript)