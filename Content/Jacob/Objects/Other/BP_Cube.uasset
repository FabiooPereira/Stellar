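; BP_Cube is a fox-statue block that slides between button positions when activated, presumably by a lever.
; BeginPlay places it just above the current button and applies a dynamic fox material.
; ObjectActivated plays a stone-sliding sound and, unless the linked lamp is lit, steps the index back and forth through the Buttons array.
; Once activated, Tick continuously eases the cube toward the target using a delta-time-scaled lerp.
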(event EventBeginPlay
  ;[1 1 1] Set Location For Box
  (bind _targetlocation (CallFunction|SetTargetLocation))
  (Transformation|SetActorLocation _targetlocation false false)
  (bind _returnvalue (Rendering|Material|CreateDynamicMaterialInstance (Variables|Components|GetCube) 0 "/Game/Elsa/Materials/FoxStatue/MI_FoxStatue.MI_FoxStatue" "None" :!class /Script/Engine.PrimitiveComponent))
  (bind _output_get (Variables|Default|SetFoxMaterial _returnvalue))
  (Rendering|Material|SetMaterial (Variables|Components|GetCube) 0 _output_get))

(event EventObjectActivated
  ;[1 1 1] Box Transition Activation
  (Audio|PlaySound2D "/Game/Tove/Sound/SFX/Game_SFX/Sliding_Stone.Sliding_Stone" 1.0 1.0 0.0 0 0)
  (Variables|Default|SetLeverActivated true)
  (if (not (Variables|/Game/Marcus/Enemy/BP_Lamp_TEST.BP_Lamp_TEST_C|GetLampIsLIt (Variables|Default|GetLamp)))
    (|NextDirectionCalc)))

(event EventTick
  (params (DeltaSeconds :type Float%20%28single-precision%29))
  ;[1 1 1] Smooth Transition Between Locations
  (if (Variables|Default|GetLeverActivated)
    (Transformation|SetActorLocation (Math|Vector|Lerp(Vector) (Transformation|GetActorLocation) (Variables|Default|GetTargetLocation) (* DeltaSeconds 5.0)) false false)))

(fn ConstructionScript)

(fn SetTargetLocation
  (bind _buttons (Variables|Default|GetButtons))
  (bind _currentindex (Variables|Default|GetCurrentIndex))
  (bind _output (Utilities|Array|Get(acopy) _buttons _currentindex))
  (bind _returnvalue (Transformation|GetActorLocation _output))
  (bind _output_get (Variables|Default|SetTargetLocation (Math|Vector|MakeVector (.x _returnvalue) (.y _returnvalue) (+ (.z _returnvalue) 1e+01))))
  (return _output_get))