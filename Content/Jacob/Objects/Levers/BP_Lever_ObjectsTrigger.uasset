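; Interactable lever that activates a linked object through ObjectActivatedMessage and rotates its handle with a timeline.
; When in range, it shows prompt text and a custom-depth highlight.
; With UsingLamp, it needs a lit lamp, testing only the array's last element after an empty loop; otherwise it is single-use unless IsBigPuzzle allows repeat pulls.
; Tick also sends the message once when SwitchActivated is set.
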(event EventBeginPlay)

(event EventTick
  (params (DeltaSeconds :type Float%20%28single-precision%29))
  (if (Variables|Default|GetSwitchActivated)
    (Utilities|FlowControl|DoOnce false
      (:Completed
        (Class|BPIEventTrigger|ObjectActivated(Message) (Variables|Default|GetObjectToActivate))))))

(event EventSetInteractableState
  (params (bCanShowInteract :type Boolean))
  ;[1 1 1] Set Interactable State
  (if (Variables|Default|GetUsingLamp)
    (for _array_element (Variables|Default|GetLamp)
      _)
    (if (Variables|/Game/Marcus/Enemy/BP_Lamp_TEST.BP_Lamp_TEST_C|GetLampIsLIt _array_element)
      (if (not (Variables|Default|GetLeverIsPressed)) :!label _label
        (bind _output_get (Variables|Default|SetbCanInteract? bCanShowInteract :!label _label_2))
        (if _output_get
          (CallFunction|TextEnable)
          (Rendering|SetRenderCustomDepth (Variables|Default|GetLever) true)
          (else
            (CallFunction|TextDisable)
            (Rendering|SetRenderCustomDepth (Variables|Default|GetLever) false)))))
    (elif (Variables|Default|GetIsBigPuzzle)
      (goto _label_2)
      (else
        (goto _label)))))

(event EventInteract
  (params (Instigator :type Actor%20Object%20Reference))
  ;[1 1 1] Lever Trigger
  (if (Variables|Default|GetUsingLamp)
    (for _array_element (Variables|Default|GetLamp)
      _)
    (if (Variables|/Game/Marcus/Enemy/BP_Lamp_TEST.BP_Lamp_TEST_C|GetLampIsLIt _array_element)
      (if (not (Variables|Default|GetLeverIsPressed)) :!label _label
        (Utilities|FlowControl|DoOnce false
          (:Completed
            (Variables|Default|SetLeverIsPressed true)
            (Class|BPIEventTrigger|ObjectActivated(Message) (Variables|Default|GetObjectToActivate) :!label _label_2)
            (bind _switchposition (Timeline|Timeline Play)
              (:Update
                (Transformation|SetRelativeRotation (Variables|Default|GetLever) (Math|Rotator|MakeRotator 0.0 _switchposition 0.0) false false)
                (if (not (Variables|Default|GetIsBigPuzzle))
                  (CallFunction|TextDisable)
                  (Rendering|SetRenderCustomDepth (Variables|Default|GetLever) false))))))))
    (elif (Variables|Default|GetIsBigPuzzle)
      (goto _label_2)
      (else
        (goto _label)))))

(fn ConstructionScript)