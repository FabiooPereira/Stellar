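; BP_Lever_DELETE1 is an interactable lever that sends an activation message to BoxesToActivate.
; Setting its interactable state toggles prompt text and the custom-depth highlight.
; Interact fires through a DoOnce, hides the highlight and plays a timeline pitching the lever, then re-arms and restores the highlight if still interactable.
; A GetForceResponsiveObject function capsule-traces ahead for WorldDynamic actors but is not called here.
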(event EventBeginPlay)

(event EventTick
  (params (DeltaSeconds :type Float%20%28single-precision%29)))

(event EventSetInteractableState
  (params (bCanShowInteract :type Boolean))
  ;[1 1 1] Set Interactable State
  (bind _output_get (Variables|Default|SetbCanInteract? bCanShowInteract))
  (if _output_get
    (CallFunction|TextEnable)
    (Rendering|SetRenderCustomDepth (Variables|Default|GetLever) true)
    (else
      (CallFunction|TextDisable)
      (Rendering|SetRenderCustomDepth (Variables|Default|GetLever) false))))

(event EventInteract
  (params (Instigator :type Actor%20Object%20Reference))
  ;[1 1 1] Switch Trigger
  (Utilities|FlowControl|DoOnce false :!label _label
    (:Completed
      (Class|BPIEventTrigger|ObjectActivated(Message) (Variables|Default|GetBoxesToActivate))
      (Rendering|SetRenderCustomDepth (Variables|Default|GetLever) false)
      (bind _switchposition (Timeline|Timeline PlayFromStart)
        (:Update
          (Transformation|SetRelativeRotation (Variables|Default|GetLever) (Math|Rotator|MakeRotator 0.0 _switchposition 0.0) false false))
        (:Finished
          (if (Variables|Default|GetbCanInteract?)
            (Rendering|SetRenderCustomDepth (Variables|Default|GetLever) true)
            (goto _label Reset)
            (else
              (goto _label Reset))))))))

(fn ConstructionScript)