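; BP_TextGenerator is a world-space text actor that can show different prompts for gamepad or keyboard input.
; ChangeTextOnInput reads the player character's IsController flag to choose which string its TextRender displays.
; Tick calls it every frame with both strings empty.
; SetTextRotation yaws the text toward the player camera, but nothing in this Blueprint calls it.
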(event EventBeginPlay)

(event Collision|EventActorBeginOverlap
  (params (OtherActor :type Actor%20Object%20Reference)))

(event EventTick
  (params (DeltaSeconds :type Float%20%28single-precision%29))
  (CallFunction|ChangeTextonInput))

(event EventChangeTextonInput
  (params (GamepadText :type Text) (KeyboardText :type Text))
  (bind _asbp_third_person_character (Utilities|Casting|CastToBP_ThirdPersonCharacter (Game|GetPlayerCharacter 0)))
  (if (Variables|/Game/ThirdPerson/Blueprints/BP_ThirdPersonCharacter.BP_ThirdPersonCharacter_C|GetisController _asbp_third_person_character)
    (Rendering|Components|TextRender|SetText (Variables|Default|GetTextRender) GamepadText)
    (else
      (Rendering|Components|TextRender|SetText (Variables|Default|GetTextRender) KeyboardText))))

(fn ConstructionScript)

(fn SetTextRotation
  (Transformation|SetWorldRotation (Variables|Default|GetTextRender) (Math|Rotator|MakeRotator 0.0 0.0 (.yaw (Math|Rotator|FindLookatRotation (Transformation|GetWorldLocation (Variables|Default|GetTextRender)) (Transformation|GetActorLocation (Game|GetPlayerCameraManager 0))))) false false))