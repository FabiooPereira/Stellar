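; Pushable and draggable object actor for BP_PlayerJacob, highlighted through custom depth on its cube mesh.
; An overlap volume sets the player's pushing flag on entry, unless already holding an object, and clears it on exit.
; InteractGrab uses that flag to call the player's grab or drop function, gated by CanInteract or CanDropObject.
; Interactable state and grab/drop also toggle the HUD's drag text.
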(event OnComponentBeginOverlap(OverlapCollision)
  (params (OverlappedComponent :type Primitive%20Component%20Object%20Reference) (OtherActor :type Actor%20Object%20Reference) (OtherComp :type Primitive%20Component%20Object%20Reference) (OtherBodyIndex :type Integer) (bFromSweep :type Boolean) (SweepResult :type Hit%20Result%20Structure%20%28by%20ref%29))
  (bind _asbp_player_jacob (Utilities|Casting|CastToBP_PlayerJacob OtherActor))
  (if (not (Variables|/Game/ThirdPerson/Blueprints/BP_PlayerJacob.BP_PlayerJacob_C|GetIsHoldingObject _asbp_player_jacob))
    (Variables|/Game/ThirdPerson/Blueprints/BP_PlayerJacob.BP_PlayerJacob_C|SetIsPushingObject _asbp_player_jacob true)
    (Rendering|SetRenderCustomDepth (Variables|Default|GetCube) true)))

(event OnComponentEndOverlap(OverlapCollision)
  (params (OverlappedComponent :type Primitive%20Component%20Object%20Reference) (OtherActor :type Actor%20Object%20Reference) (OtherComp :type Primitive%20Component%20Object%20Reference) (OtherBodyIndex :type Integer))
  (bind _asbp_player_jacob (Utilities|Casting|CastToBP_PlayerJacob OtherActor))
  (Variables|/Game/ThirdPerson/Blueprints/BP_PlayerJacob.BP_PlayerJacob_C|SetIsPushingObject _asbp_player_jacob false)
  (Rendering|SetRenderCustomDepth (Variables|Default|GetCube) false))

(event EventInteractGrab
  (params (Instigator :type Actor%20Object%20Reference))
  (bind _asbp_player_jacob (Utilities|Casting|CastToBP_PlayerJacob Instigator))
  (if (Variables|/Game/ThirdPerson/Blueprints/BP_PlayerJacob.BP_PlayerJacob_C|GetIsPushingObject _asbp_player_jacob)
    (if (Variables|Default|GetbCanInteract?)
      (Variables|/Game/ThirdPerson/Blueprints/BP_PlayerJacob.BP_PlayerJacob_C|SetIsPushingObject _asbp_player_jacob false)
      (Default|GrabandPushObject _asbp_player_jacob)
      (CallFunction|TextEnable))
    (elif (Variables|/Game/ThirdPerson/Blueprints/BP_PlayerJacob.BP_PlayerJacob_C|GetCanDropObject _asbp_player_jacob)
      (Variables|/Game/ThirdPerson/Blueprints/BP_PlayerJacob.BP_PlayerJacob_C|SetIsPushingObject _asbp_player_jacob true)
      (Default|DropandPushObject _asbp_player_jacob)
      (CallFunction|TextDisable))))

(event EventSetInteractableState
  (params (bCanShowInteract :type Boolean))
  (bind _cube (Variables|Default|GetCube))
  (bind _output_get (Variables|Default|SetbCanInteract? bCanShowInteract))
  (if _output_get
    (CallFunction|TextEnable)
    (Rendering|SetRenderCustomDepth _cube true)
    (else
      (CallFunction|TextDisable)
      (Rendering|SetRenderCustomDepth _cube false))))

(event EventTick
  (params (DeltaSeconds :type Float%20%28single-precision%29)))

(fn ConstructionScript)

(fn TextDisable
  (bind _as_new_hud (Variables|Default|GetAs%20New%20HUD)
    (:then
      (Default|DragText (Variables|/Game/Jacob/NewHUD.NewHUD_C|GetUIRef _as_new_hud) false))
    (:else)))

(fn TextEnable
  (bind _asnew_hud (Utilities|Casting|CastToNewHUD (HUD|GetHUD (Game|GetPlayerController 0))))
  (bind _output_get (Variables|Default|SetAs%20New%20HUD _asnew_hud))
  (Default|DragText (Variables|/Game/Jacob/NewHUD.NewHUD_C|GetUIRef _output_get) true))