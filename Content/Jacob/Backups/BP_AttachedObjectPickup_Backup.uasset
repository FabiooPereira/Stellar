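; Backup of a pickup actor whose cube tracks held and interactable states and toggles between static and physics-simulated.
; ApplyForcewithDirection only turns on cube physics, applying no force.
; ResetForce stops simulation, moves the actor to the cube's world location and reattaches the cube to the root, since simulating detaches it.
; Overlap events are empty, and both interactable states set the same glowing material.
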(event OnComponentBeginOverlap(Box)
  (params (OverlappedComponent :type Primitive%20Component%20Object%20Reference) (OtherActor :type Actor%20Object%20Reference) (OtherComp :type Primitive%20Component%20Object%20Reference) (OtherBodyIndex :type Integer) (bFromSweep :type Boolean) (SweepResult :type Hit%20Result%20Structure%20%28by%20ref%29))
  ;[1 1 1] Begin Overlap
)

(event OnComponentEndOverlap(Cube)
  (params (OverlappedComponent :type Primitive%20Component%20Object%20Reference) (OtherActor :type Actor%20Object%20Reference) (OtherComp :type Primitive%20Component%20Object%20Reference) (OtherBodyIndex :type Integer))
  ;[1 1 1] End Overlap
)

(event Custom|ChangeHoldingStatusOnObject_1
  (params (IsHolding :type Boolean))
  ;[1 1 1] Status Change
  (Variables|Default|SetObjectPickedUp IsHolding))

(event EventBeginPlay
  (Physics|SetSimulatePhysics (Variables|Default|GetCube) false))

(event Collision|EventActorBeginOverlap
  (params (OtherActor :type Actor%20Object%20Reference)))

(event EventTick
  (params (DeltaSeconds :type Float%20%28single-precision%29)))

(event EventSetInteractableState
  (params (bCanShowInteract? :type Boolean))
  (bind _cube (Variables|Default|GetCube))
  ;[1 1 1] Interactable State
  (bind _output_get (Variables|Default|SetbCanInteract? bCanShowInteract?))
  (if _output_get
    (Rendering|Material|SetMaterial _cube 0 "/Game/Kio/Extra/MI_GlowingCube.MI_GlowingCube")
    (else
      (Rendering|Material|SetMaterial _cube 0 "/Game/Kio/Extra/MI_GlowingCube.MI_GlowingCube"))))

(event EventResetForce
  (bind _cube (Variables|Default|GetCube))
  ;[1 1 1] Reset Force
  (if (Physics|IsSimulatingPhysics _cube "None")
    (Physics|SetSimulatePhysics _cube false)
    (Transformation|SetActorLocation (Transformation|GetWorldLocation _cube) false false)
    (Transformation|AttachComponentToComponent (Variables|Default|GetCube) (Variables|Default|GetDefaultSceneRoot) "None" "KeepWorld" "KeepWorld" "KeepWorld" true)))

(event EventApplyForcewithDirection
  (params (DirectionVector :type Vector :default "0, 0, 0") (Power :type Float%20%28double-precision%29))
  ;[1 1 1] Apply Force With Direction
  (Physics|SetSimulatePhysics (Variables|Default|GetCube) true))

(fn ConstructionScript)