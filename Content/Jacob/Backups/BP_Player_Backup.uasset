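; Player character Blueprint handling interaction, companion stay and call commands, gliding and object carrying.
; An overlap sphere tracks one BPI_Interactable; using an NPC switches input to UI-only until the conversation closes.
; Gliding starts after a ground trace misses, lowering gravity and raising air control until release or landing.
; Pickups attach to a hold component and drop onto a downward trace hit; older force-based grab-and-throw logic remains unconnected.
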(event OnComponentBeginOverlap(InteractRadius)
  (params (OverlappedComponent :type Primitive%20Component%20Object%20Reference) (OtherActor :type Actor%20Object%20Reference) (OtherComp :type Primitive%20Component%20Object%20Reference) (OtherBodyIndex :type Integer) (bFromSweep :type Boolean) (SweepResult :type Hit%20Result%20Structure%20%28by%20ref%29))
  (CallFunction|SetInteractable OtherActor))

(event OnComponentEndOverlap(InteractRadius)
  (params (OverlappedComponent :type Primitive%20Component%20Object%20Reference) (OtherActor :type Actor%20Object%20Reference) (OtherComp :type Primitive%20Component%20Object%20Reference) (OtherBodyIndex :type Integer))
  (CallFunction|DisableInteract OtherActor))

(event Input|EnhancedActionEvents|EnhancedInputActionIA_Interact
  (params (ActionValue :type Boolean) (ElapsedSeconds :type Float%20%28double-precision%29) (TriggeredSeconds :type Float%20%28double-precision%29) (InputAction :type Input%20Action%20Object%20Reference :default "/Game/ThirdPerson/Input/Actions/IA_Interact.IA_Interact"))
  (:Started
    (CallFunction|InteractwithObject)))

(event EventBeginPlay)

(event Collision|EventActorBeginOverlap
  (params (OtherActor :type Actor%20Object%20Reference))
  (|CallParentFunction OtherActor) ; This node is disabled and will not be called.\nDrag off pins to build functionality.
)

(event EventTick
  (params (DeltaSeconds :type Float%20%28single-precision%29))
  (|CallParentFunction DeltaSeconds))

(event EventConversationClosed
  (CallFunction|UnlockPlayerMovement))

(event EventOnLanded
  (params (Hit :type Hit%20Result%20Structure%20%28by%20ref%29))
  (bind _charactermovement (Variables|Character|GetCharacterMovement))
  ;[1 1 1] Gliding
  (Variables|Default|SetHasLanded true)
  (Rendering|SetVisibility (Variables|Default|GetHangGlider) false false)
  (Variables|/Script/Engine.CharacterMovementComponent|SetGravityScale _charactermovement 1.75)
  (Variables|/Script/Engine.CharacterMovementComponent|SetAirControl _charactermovement 0.35))

(event EventDropObject
  (bind _objecttograb (Variables|Default|GetObjectToGrab))
  (bind _returnvalue (Transformation|GetWorldLocation _objecttograb))
  (bind (_x _y _z) (Math|Vector|BreakVector _returnvalue))
  ;[1 1 1] Grab function - Drop
  (Class|BPIInteractable|SetInteractableState(Message) (Variables|Default|GetInteractable) true)
  (Transformation|DetachFromActor (Variables|Default|GetPickedUpActor) "KeepWorld" "KeepWorld" "KeepWorld")
  (bind (_outhit _returnvalue_2) (Collision|LineTraceByChannel _returnvalue (Math|Vector|MakeVector _x _y (- _z 1e+03)) "TraceTypeQuery1" false (Utilities|Array|MakeArray (Variables|Default|GetPickedUpActor) self) "None"))
  (if _returnvalue_2
    (Transformation|SetActorLocation (Variables|Default|GetPickedUpActor) (.Location (Collision|BreakHitResult _outhit)) false false)
    (Variables|Default|SetIsHoldingObject false)
    (Class|BPIObjectAttachment|ChangeHoldingStatusonObject(Message) (Variables|Default|GetPickedUpActor) false)
    (Variables|Default|SetPickedUpActor 0)))

(event EventPickupObject
  (bind _pickedupactor (Variables|Default|GetPickedUpActor))
  ;[1 1 1] Grab function - Pickup
  (Class|BPIInteractable|SetInteractableState(Message) (Variables|Default|GetInteractable) false)
  (Variables|Default|GetPickedUpActor
    (:then
      (Variables|Default|SetIsHoldingObject true)
      (Variables|Default|SetCanPickupObject false)
      (Class|BPIObjectAttachment|ChangeHoldingStatusonObject(Message) _pickedupactor true)
      (Transformation|AttachComponentToComponent _pickedupactor (Variables|Default|GetObjectToGrab) "None" "SnapToTarget" "SnapToTarget" "KeepWorld" true))
    (:else)))

(event EventOverlapStatusChange
  (params (OverlapType :type E_OverlapStatusChange%20Enum :default "NewEnumerator0") (PickupActor :type Actor%20Object%20Reference))
  ;[1 1 1] Grab Overlap
  (switch Utilities|FlowControl|Switch|SwitchonE_OverlapStatusChange OverlapType
    (:NewEnumerator0
      (if (not (Variables|Default|GetIsHoldingObject))
        (Variables|Default|SetPickedUpActor (Utilities|Select :Index OverlapType :NewEnumerator0 PickupActor :NewEnumerator1 0) :!label _label)
        (Variables|Default|SetCanPickupObject (Utilities|Select :Index OverlapType :NewEnumerator0 true :NewEnumerator1 false))))
    (:NewEnumerator1
      (if (not (Variables|Default|GetIsHoldingObject))
        (goto _label)))))

(event Input|ActionEvents|InputActionStay
  (params (Key :type Key%20Structure))
  (:Pressed
    (Class|GruppOnionCharacter|StayCompanion)))

(event Input|ActionEvents|InputActionCall
  (params (Key :type Key%20Structure))
  (:Pressed
    (Class|GruppOnionCharacter|CallCompanion)))

(event Input|ActionEvents|InputActionGlide
  (params (Key :type Key%20Structure))
  (bind _returnvalue (Transformation|GetActorLocation))
  (bind _charactermovement (Variables|Character|GetCharacterMovement))
  (bind _charactermovement_2 (Variables|Character|GetCharacterMovement))
  ;[1 1 1] Gliding
  (:Pressed
    (if (Variables|Default|GetHasLanded)
      (bind _returnvalue_2 (Collision|LineTraceByChannel _returnvalue (+ _returnvalue (* (Transformation|GetActorUpVector) -1e+02)) "TraceTypeQuery1" false 0 "None"))
      (if (not _returnvalue_2)
        (Rendering|SetVisibility (Variables|Default|GetHangGlider) true false)
        (Variables|/Script/Engine.CharacterMovementComponent|SetGravityScale _charactermovement_2 0.15)
        (Variables|/Script/Engine.CharacterMovementComponent|SetAirControl _charactermovement_2 0.9)
        (Character|LaunchCharacter "0.000000,0.000000,10.000000" false true)
        (Variables|Default|SetHasLanded false))))
  (:Released
    (Rendering|SetVisibility (Variables|Default|GetHangGlider) false false)
    (Variables|/Script/Engine.CharacterMovementComponent|SetGravityScale _charactermovement 1.75)
    (Variables|/Script/Engine.CharacterMovementComponent|SetAirControl _charactermovement 0.35)))

(event Input|ActionEvents|InputActionGrab
  (params (Key :type Key%20Structure))
  ;[1 1 1] Grab Input
  (:Pressed
    (if (Variables|Default|GetIsHoldingObject)
      (CallFunction|DropObject)
      (elif (Variables|Default|GetCanPickupObject)
        (CallFunction|PickupObject)))))

(fn ConstructionScript
  (|CallParentFunction))

(fn InteractwithObject
  (bind _interactable (Variables|Default|GetInteractable))
  (Utilities|IsValid _interactable
    (:Is%20Valid
      (if (Utilities|ClassIsChildOf (Utilities|GetClass _interactable) "/Game/Marcus/NPC/NPCs/NPC_Base.NPC_Base_C")
        (CallFunction|LockPlayerMovement))
      (Class|BPIInteractable|Interact(Message) (Variables|Default|GetInteractable) self))))

(fn LockPlayerMovement
  (Input|SetInputModeUIOnly (Game|GetPlayerController 0) 0 "DoNotLock" false)
  (Variables|/Script/Engine.PlayerController|SetbShowMouseCursor (Game|GetPlayerController 0) true))

(fn UnlockPlayerMovement
  (Variables|/Script/Engine.PlayerController|SetbShowMouseCursor (Game|GetPlayerController 0) false)
  (Input|SetInputModeGameOnly (Game|GetPlayerController 0) false))

(fn DisableInteract
  (params (Other%20Actor :type Object%20Object%20Reference))
  (if (and (!= Other%20Actor self) (== Other%20Actor (Variables|Default|GetInteractable)))
    (Class|BPIInteractable|SetInteractableState(Message) (Variables|Default|GetInteractable) false)
    (Variables|Default|SetInteractable 0)))

(fn SetInteractable
  (params (OtherObject :type Actor%20Object%20Reference))
  (if (!= OtherObject self)
    (if (Utilities|DoesObjectImplementInterface OtherObject "/Game/Marcus/BPI_Interactable.BPI_Interactable_C")
      (Utilities|IsValid (Variables|Default|GetInteractable)
        (:Is%20Valid
          (Class|BPIInteractable|SetInteractableState(Message) (Variables|Default|GetInteractable) false)
          (Variables|Default|SetInteractable 0))
        (:Is%20Not%20Valid
          _))
      (Variables|Default|SetInteractable OtherObject)
      (Class|BPIInteractable|SetInteractableState(Message) (Variables|Default|GetInteractable) true))))

(fn Detach
  (bind _grabbedobject (Variables|Default|GetGrabbedObject))
  (Transformation|DetachFromActor _grabbedobject "KeepWorld" "KeepWorld" "KeepWorld")
  (Class|BPIForce|ApplyForcewithDirection(Message) _grabbedobject "0.000000,0.000000,-5.000000" 5e+01)
  (Development|PrintString "detach"))