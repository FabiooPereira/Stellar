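; A pickup cube that characters can attach and hold, with an interact prompt that yaws toward the camera each tick.
; Box overlaps toggle the prompt, message the character through BPI_CharacterAttachmentInteraction and swap the cube's material; exit notifications are skipped while held or flagged as on a pressure switch.
; Force events toggle cube physics; resetting moves the actor to the simulated cube and reattaches it to the root.
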(event OnComponentBeginOverlap(Box)
  (params (OverlappedComponent :type Primitive%20Component%20Object%20Reference) (OtherActor :type Actor%20Object%20Reference) (OtherComp :type Primitive%20Component%20Object%20Reference) (OtherBodyIndex :type Integer) (bFromSweep :type Boolean) (SweepResult :type Hit%20Result%20Structure%20%28by%20ref%29))
  ;[1 1 1] Begin Overlap
  (Rendering|SetVisibility (Variables|Default|GetInteractButtonText) true false)
  (if (Utilities|DoesObjectImplementInterface OtherActor "/Game/BPI_CharacterAttachmentInteraction.BPI_CharacterAttachmentInteraction_C")
    (Class|BPICharacterAttachmentInteraction|OverlapStatusChange(Message) OtherActor "NewEnumerator0" self)
    (Rendering|Material|SetMaterial (Variables|Default|GetCube) 0 "/Game/StarterContent/Blueprints/Assets/M_LightStage_Arrows.M_LightStage_Arrows")
    (elif (Utilities|DoesObjectImplementInterface OtherActor "/Game/BPI_IsPressureSwitch.BPI_IsPressureSwitch_C")
      (Variables|Default|SetIsTriggeringSwitch true)
      (else
        (Variables|Default|SetIsTriggeringSwitch false)))))

(event OnComponentEndOverlap(Box)
  (params (OverlappedComponent :type Primitive%20Component%20Object%20Reference) (OtherActor :type Actor%20Object%20Reference) (OtherComp :type Primitive%20Component%20Object%20Reference) (OtherBodyIndex :type Integer))
  ;[1 1 1] End Overlap
  (Rendering|SetVisibility (Variables|Default|GetInteractButtonText) false false)
  (if (and (Utilities|DoesObjectImplementInterface OtherActor "/Game/BPI_CharacterAttachmentInteraction.BPI_CharacterAttachmentInteraction_C") (not (Variables|Default|GetObjectPickedUp)))
    (if (not (Variables|Default|GetIsTriggeringSwitch))
      (Class|BPICharacterAttachmentInteraction|OverlapStatusChange(Message) OtherActor "NewEnumerator1")
      (Rendering|Material|SetMaterial (Variables|Default|GetCube) 0 "/Game/Materials/M_Red.M_Red"))))

(event EventBeginPlay)

(event Collision|EventActorBeginOverlap
  (params (OtherActor :type Actor%20Object%20Reference)))

(event EventTick
  (params (DeltaSeconds :type Float%20%28single-precision%29))
  (CallFunction|SetTextRotation))

(event EventChangeHoldingStatusonObject
  (params (IsHolding :type Boolean))
  ;[1 1 1] Status Change
  (Variables|Default|SetObjectPickedUp IsHolding))

(event EventSetInteractableState
  (params (bCanShowInteract? :type Boolean))
  ;[1 1 1] Interactable State
  (bind _output_get (Variables|Default|SetbCanInteract? bCanShowInteract?))
  (if _output_get
    _))

(event EventResetForce
  (bind _cube (Variables|Default|GetCube))
  ;[1 1 1] Reset Force
  (if (Physics|IsSimulatingPhysics _cube "None")
    (Physics|SetSimulatePhysics _cube false)
    (Transformation|SetActorLocation (Transformation|GetWorldLocation _cube) false false)
    (Transformation|AttachComponentToComponent (Variables|Default|GetCube) (Variables|Default|GetDefaultSceneRoot) "None" "KeepWorld" "KeepWorld" "KeepWorld" true)))

(event EventApplyForcewithDirection
  (params (DirectionVector :type Vector :default "0, 0, 0") (Power :type Float%20%28double-precision%29))
  ;[1 1 1] Apply Force With Direction
  (Physics|SetSimulatePhysics (Variables|Default|GetCube) true))

(fn ConstructionScript)

(fn SetTextRotation
  (Transformation|SetWorldRotation (Variables|Default|GetInteractButtonText) (Math|Rotator|MakeRotator 0.0 0.0 (.yaw (Math|Rotator|FindLookatRotation (Transformation|GetWorldLocation (Variables|Default|GetInteractButtonText)) (Transformation|GetActorLocation (Game|GetPlayerCameraManager 0))))) false false))