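; A physics-driven actor that can be pushed by directed force and toggled as interactable, apparently a backup copy of a force-responsive object.
; Its static mesh simulates physics from BeginPlay, and applying force adds a velocity-change impulse along a given direction scaled by power.
; Resetting force stops simulation, moves the actor to the mesh's location and reattaches the mesh to the root.
; Setting interactable state stores a flag and swaps the mesh material.
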(event EventBeginPlay
  (Physics|SetSimulatePhysics (Variables|Default|GetStaticMesh) true))

(event Collision|EventActorBeginOverlap
  (params (OtherActor :type Actor%20Object%20Reference)))

(event EventTick
  (params (DeltaSeconds :type Float%20%28single-precision%29)))

(event EventResetForce
  (bind _staticmesh (Variables|Default|GetStaticMesh))
  ;[1 1 1] Reset Force
  (if (Physics|IsSimulatingPhysics _staticmesh "None")
    (Physics|SetSimulatePhysics _staticmesh false)
    (Transformation|SetActorLocation (Transformation|GetWorldLocation _staticmesh) false false)
    (Transformation|AttachComponentToComponent (Variables|Default|GetStaticMesh) (Variables|Default|GetDefaultSceneRoot) "None" "KeepWorld" "KeepWorld" "KeepWorld" true)))

(event EventApplyForcewithDirection
  (params (DirectionVector :type Vector :default "0, 0, 0") (Power :type Float%20%28double-precision%29))
  (bind _staticmesh (Variables|Default|GetStaticMesh))
  ;[1 1 1] Apply Force With Direction
  (Physics|SetSimulatePhysics _staticmesh true)
  (Physics|AddImpulse _staticmesh (* DirectionVector Power) "None" true))

(event EventSetInteractableState
  (params (bCanShowInteract? :type Boolean))
  (bind _staticmesh (Variables|Default|GetStaticMesh))
  ;[1 1 1] Interactable State
  (bind _output_get (Variables|Default|SetbCanInteract? bCanShowInteract?))
  (if _output_get
    (Rendering|Material|SetMaterial _staticmesh 0 "/Engine/MapTemplates/Materials/BasicAsset01.BasicAsset01")
    (else
      (Rendering|Material|SetMaterial _staticmesh 0 "/Game/StarterContent/Materials/M_Basic_Wall.M_Basic_Wall"))))

(fn ConstructionScript)