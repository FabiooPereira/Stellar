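; BP_Lever_Parent is a base Blueprint for levers that supplies shared helpers for showing and hiding a pull prompt on the HUD.
; TextEnable casts the first player's HUD to NewHUD, caches it, and shows gamepad and keyboard pull hints through its UI reference.
; TextDisable clears and hides that prompt if the cached HUD is valid.
; ComponentIsChild checks whether a component's parent actor is this lever; the event graph holds no logic.
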(event EventBeginPlay)

(event EventTick
  (params (DeltaSeconds :type Float%20%28single-precision%29)))

(fn ConstructionScript)

(fn ComponentIsChild
  (params (Component :type Actor%20Object%20Reference%20%28by%20ref%29))
  (return (== (Actor|GetParentActor Component) self)))

(fn TextDisable
  (bind _as_new_hud (Variables|Default|GetAs%20New%20HUD)
    (:then
      (Default|SetTextInput (Variables|/Game/Jacob/UI/NewHUD.NewHUD_C|GetUIRef _as_new_hud) "" "" false))
    (:else)))

(fn TextEnable
  (bind _asnew_hud (Utilities|Casting|CastToNewHUD (HUD|GetHUD (Game|GetPlayerController 0))))
  (bind _output_get (Variables|Default|SetAs%20New%20HUD _asnew_hud))
  (Default|SetTextInput (Variables|/Game/Jacob/UI/NewHUD.NewHUD_C|GetUIRef _output_get) "PULL: B" "PULL: E" true))