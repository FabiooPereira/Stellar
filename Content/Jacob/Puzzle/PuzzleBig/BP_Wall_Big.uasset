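; BP_Wall_Big is a puzzle wall that moves vertically when enough pressure switches are active.
; Activation and deactivation events adjust an active switch count and compare it to the required number.
; Meeting the threshold turns on the linked PuzzleLight and plays a timeline that drives the wall's relative Z location.
; Falling below it turns the light off and reverses the timeline, but only if that light is valid.
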(event Custom|SwitchActivatedWall_Big
  ;[1 1 1] Door Activation/Deactivation
  (Math|Integer|IncrementInt (Variables|Default|GetPressureSwitchesActive)
    (:%20%20
      (if (>= (Variables|Default|GetPressureSwitchesActive) (Variables|Default|GetPressureSwitchesNeeded))
        (bind _output_get (Variables|Default|SetPuzzleLight (Variables|Default|GetPuzzleLight)))
        (Default|TurnonLight _output_get)
        (bind _doorposition (Timeline|WallActivation_Big Play)
          (:Update
            (Transformation|SetRelativeLocation (Variables|Default|GetWall) (Math|Vector|MakeVector 0.0 0.0 _doorposition) false false)))
        (else
          (bind _puzzlelight (Variables|Default|GetPuzzleLight)
            (:then
              (Default|TurnOffLight _puzzlelight)
              (Timeline|WallActivation_Big Reverse))
            (:else)))))))

(event Custom|SwitchDeactivatedWall_Big
  ;[1 1 1] Door Activation/Deactivation
  (Math|Integer|DecrementInt (Variables|Default|GetPressureSwitchesActive)
    (:%20%20
      (if (>= (Variables|Default|GetPressureSwitchesActive) (Variables|Default|GetPressureSwitchesNeeded))
        (bind _output_get (Variables|Default|SetPuzzleLight (Variables|Default|GetPuzzleLight)))
        (Default|TurnonLight _output_get)
        (bind _doorposition (Timeline|WallActivation_Big Play)
          (:Update
            (Transformation|SetRelativeLocation (Variables|Default|GetWall) (Math|Vector|MakeVector 0.0 0.0 _doorposition) false false)))
        (else
          (bind _puzzlelight (Variables|Default|GetPuzzleLight)
            (:then
              (Default|TurnOffLight _puzzlelight)
              (Timeline|WallActivation_Big Reverse))
            (:else)))))))

(event EventBeginPlay)

(event Collision|EventActorBeginOverlap
  (params (OtherActor :type Actor%20Object%20Reference)))

(event EventTick
  (params (DeltaSeconds :type Float%20%28single-precision%29)))

(fn ConstructionScript)