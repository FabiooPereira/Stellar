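; BP_Box_Big2 is a puzzle box that steps between button positions each time its lever activation event fires.
; NextDirectionCalc advances the index along the Buttons array, reversing at either end, and sets a target hovering above that position.
; BeginPlay snaps the box to its starting position, then Tick eases it toward the target with a delta-time lerp.
; The pressure switch count has no effect on movement, and the door timeline is unconnected.
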(event Custom|LeverActivatedBox_Big
  ;[1 1 1] Door Activation/Deactivation
  (|NextDirectionCalc))

(event Custom|LeverDeactivatedBox_Big
  ;[1 1 1] Door Activation/Deactivation
  (Math|Integer|DecrementInt (Variables|Default|GetPressureSwitchesActive)
    (:%20%20
      (if (>= (Variables|Default|GetPressureSwitchesActive) (Variables|Default|GetPressureSwitchesNeeded))
        _))))

(event EventBeginPlay
  (bind _buttons (Variables|Default|GetButtons))
  (bind _currentindex (Variables|Default|GetCurrentIndex))
  (bind _output (Utilities|Array|Get(acopy) _buttons _currentindex))
  (bind _output_get (Variables|Default|SetTargetLocation (Math|Vector|MakeVector (.x _output) (.y _output) (+ (.z _output) 55.0))))
  (Transformation|SetActorLocation _output_get false false))

(event EventTick
  (params (DeltaSeconds :type Float%20%28single-precision%29))
  (Transformation|SetActorLocation (Math|Vector|Lerp(Vector) (Transformation|GetActorLocation) (Variables|Default|GetTargetLocation) (* DeltaSeconds 5.0)) false false))

(fn ConstructionScript)