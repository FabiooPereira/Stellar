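; BP_Box_Big3 is a big puzzle box that snaps above an entry in its Buttons array on BeginPlay and responds to lever events.
; Lever activations increment a switch count; reaching the required number plays a timeline sliding the Cube along relative X, otherwise the timeline reverses.
; Lever deactivation only decrements the count, leaving the timeline untouched.
; Logic for stepping the box through successive Buttons is disconnected and never runs.
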(event Custom|LeverActivatedBox_Big
  ;[1 1 1] Door Activation/Deactivation
  (Math|Integer|IncrementInt (Variables|Default|GetPressureSwitchesActive)
    (:%20%20
      (if (>= (Variables|Default|GetPressureSwitchesActive) (Variables|Default|GetPressureSwitchesNeeded))
        (bind _doorposition (Timeline|BoxActivation_Big Play)
          (:Update
            (Transformation|SetRelativeLocation (Variables|Default|GetCube) (Math|Vector|MakeVector _doorposition 0.0 0.0) false false)))
        (else
          (Timeline|BoxActivation_Big Reverse))))))

(event Custom|LeverDeactivatedBox_Big
  ;[1 1 1] Door Activation/Deactivation
  (Math|Integer|DecrementInt (Variables|Default|GetPressureSwitchesActive)
    (:%20%20
      (if (>= (Variables|Default|GetPressureSwitchesActive) (Variables|Default|GetPressureSwitchesNeeded))
        _))))

(event EventBeginPlay
  (bind _buttons (Variables|Default|GetButtons))
  (bind _currentindex (Variables|Default|GetCurrentIndex))
  (bind _output (Utilities|Array|Get(acopy) _buttons _currentindex))
  (Transformation|SetActorLocation (Math|Vector|MakeVector (.x _output) (.y _output) (+ (.z _output) 55.0)) false false))

(event Collision|EventActorBeginOverlap
  (params (OtherActor :type Actor%20Object%20Reference)))

(event EventTick
  (params (DeltaSeconds :type Float%20%28single-precision%29)))

(fn ConstructionScript)