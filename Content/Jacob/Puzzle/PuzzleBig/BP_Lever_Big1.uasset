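; Interactable lever for the big puzzle that triggers its linked big box.
; SetInteractableState toggles the prompt text and swaps the lever material, while Tick yaws that text toward the player camera.
; Interact turns the lever red, calls LeverActivatedBoxBig on BoxToActivate and plays a Timeline rotating the lever, with a DoOnce blocking retriggers until it finishes.
; An unused, buggy branch snaps a traced force-responsive object onto the lever.
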(event EventBeginPlay)

(event EventTick
  (params (DeltaSeconds :type Float%20%28single-precision%29))
  (CallFunction|SetTextRotation))

(event EventSetInteractableState
  (params (bCanShowInteract :type Boolean))
  (bind _lever (Variables|Default|GetLever))
  (bind _output_get (Variables|Default|SetbCanInteract? bCanShowInteract))
  (if _output_get
    (Rendering|SetVisibility (Variables|Default|GetInteractButtonText) true false)
    (Rendering|Material|SetMaterial _lever 0 "/Game/StarterContent/Blueprints/Assets/M_LightStage_Arrows.M_LightStage_Arrows")
    (else
      (Rendering|SetVisibility (Variables|Default|GetInteractButtonText) false false)
      (Rendering|Material|SetMaterial _lever 0 "/Game/Materials/M_Red.M_Red"))))

(event EventInteract
  (params (Instigator :type Actor%20Object%20Reference))
  ;[1 1 1] Switch Trigger
  (Utilities|FlowControl|DoOnce false :!label _label
    (:Completed
      (Rendering|Material|SetMaterial (Variables|Default|GetLever) 0 "/Game/Materials/M_Red.M_Red")
      (Default|LeverActivatedBoxBig (Variables|Default|GetBoxToActivate))
      (bind _switchposition (Timeline|Timeline PlayFromStart)
        (:Update
          (Transformation|SetRelativeRotation (Variables|Default|GetLever) (Math|Rotator|MakeRotator _switchposition 0.0 0.0) false false))
        (:Finished
          (goto _label Reset))))))

(fn ConstructionScript)

(fn ComponentIsChild
  (params (Component :type Actor%20Object%20Reference%20%28by%20ref%29))
  (return (== (Actor|GetParentActor Component) self)))

(fn SetTextRotation
  (Transformation|SetWorldRotation (Variables|Default|GetInteractButtonText) (Math|Rotator|MakeRotator 0.0 0.0 (.yaw (Math|Rotator|FindLookatRotation (Transformation|GetSocketLocation (Variables|Default|GetInteractButtonText) "None") (Transformation|GetActorLocation (Game|GetPlayerCameraManager 0))))) false false))