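; Pressure switch for the big wall puzzle that responds to cube actors (BP_Cube or its children) resting in its trigger.
; When a cube begins overlapping the OverlapBox, it turns on its Light and sends an activated message to the referenced WallToActivate.
; When a cube ends overlap, it turns the Light off and sends the deactivated message, with no count of overlapping cubes.
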(event OnComponentBeginOverlap(OverlapBox)
  (params (OverlappedComponent :type Primitive%20Component%20Object%20Reference) (OtherActor :type Actor%20Object%20Reference) (OtherComp :type Primitive%20Component%20Object%20Reference) (OtherBodyIndex :type Integer) (bFromSweep :type Boolean) (SweepResult :type Hit%20Result%20Structure%20%28by%20ref%29))
  ;[1 1 1] Switch Trigger
  (if (Utilities|ClassIsChildOf (Utilities|GetClass OtherActor) "/Game/Jacob/Puzzle/PuzzleBig/BP_Cube.BP_Cube_C")
    (Default|TurnonLight (Variables|Default|GetLight))
    (Class|BPIEventTrigger|ObjectActivated(Message) (Variables|Default|GetWallToActivate))))

(event OnComponentEndOverlap(OverlapBox)
  (params (OverlappedComponent :type Primitive%20Component%20Object%20Reference) (OtherActor :type Actor%20Object%20Reference) (OtherComp :type Primitive%20Component%20Object%20Reference) (OtherBodyIndex :type Integer))
  ;[1 1 1] Switch Trigger
  (if (Utilities|ClassIsChildOf (Utilities|GetClass OtherActor) "/Game/Jacob/Puzzle/PuzzleBig/BP_Cube.BP_Cube_C")
    (Default|TurnOffLight (Variables|Default|GetLight))
    (Class|BPIEventTrigger|ObjectDeactivated(Message) (Variables|Default|GetWallToActivate))))

(event EventBeginPlay
  (|CallParentFunction))

(event Collision|EventActorBeginOverlap
  (params (OtherActor :type Actor%20Object%20Reference)))

(event EventTick
  (params (DeltaSeconds :type Float%20%28single-precision%29))
  (|CallParentFunction DeltaSeconds) ; This node is disabled and will not be called.\nDrag off pins to build functionality.
)

(fn ConstructionScript
  (|CallParentFunction))