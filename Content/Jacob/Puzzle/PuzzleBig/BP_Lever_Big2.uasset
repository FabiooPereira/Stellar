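; BP_Lever_Big2 is a one-shot puzzle lever that notifies its linked BoxToActivate through LeverActivatedBoxBig when interacted with.
; Until activated, SetInteractableState toggles the prompt text and lever material, while Tick yaws the prompt toward the player camera.
; Interact latches SwitchActivated and plays a Timeline that rotates the lever.
; A snap routine for force-responsive objects, found by capsule trace, is disconnected and marked buggy.
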(event EventBeginPlay)

(event EventTick
  (params (DeltaSeconds :type Float%20%28single-precision%29))
  (if (not (Variables|Default|GetSwitchActivated))
    (CallFunction|SetTextRotation)))

(event EventSetInteractableState
  (params (bCanShowInteract :type Boolean))
  (bind _lever (Variables|Default|GetLever))
  (if (not (Variables|Default|GetSwitchActivated))
    (bind _output_get (Variables|Default|SetbCanInteract? bCanShowInteract))
    (if _output_get
      (Rendering|SetVisibility (Variables|Default|GetInteractButtonText) true false)
      (Rendering|Material|SetMaterial _lever 0 "/Engine/EngineMaterials/DefaultLightFunctionMaterial.DefaultLightFunctionMaterial")
      (else
        (Rendering|SetVisibility (Variables|Default|GetInteractButtonText) false false)
        (Rendering|Material|SetMaterial _lever 0 "/Game/Materials/M_Red.M_Red")))))

(event EventInteract
  (params (Instigator :type Actor%20Object%20Reference))
  ;[1 1 1] Switch Trigger
  (Variables|Default|SetSwitchActivated true)
  (Default|LeverActivatedBoxBig (Variables|Default|GetBoxToActivate))
  (bind _switchposition (Timeline|Timeline Play)
    (:Update
      (Transformation|SetRelativeRotation (Variables|Default|GetLever) (Math|Rotator|MakeRotator _switchposition 0.0 0.0) false false))))

(fn ConstructionScript)

(fn ComponentIsChild
  (params (Component :type Actor%20Object%20Reference%20%28by%20ref%29))
  (return (== (Actor|GetParentActor Component) self)))

(fn SetTextRotation
  (Transformation|SetWorldRotation (Variables|Default|GetInteractButtonText) (Math|Rotator|MakeRotator 0.0 0.0 (.yaw (Math|Rotator|FindLookatRotation (Transformation|GetSocketLocation (Variables|Default|GetInteractButtonText) "None") (Transformation|GetActorLocation (Game|GetPlayerCameraManager 0))))) false false))