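; BP_Box_Big1 is a puzzle box that moves between an ordered array of button actors, hovering slightly above each one.
; It snaps to the current button on BeginPlay, then every Tick lerps toward its target location for a smooth glide.
; The LeverActivatedBox_Big event calls NextDirectionCalc, which steps the index and reverses at either end of the array, so the box ping-pongs along the buttons.
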(event Custom|LeverActivatedBox_Big
  ;[1 1 1] Box Transition Activation
  (|NextDirectionCalc))

(event EventBeginPlay
  (bind _buttons (Variables|Default|GetButtons))
  (bind _currentindex (Variables|Default|GetCurrentIndex))
  (bind _output (Utilities|Array|Get(acopy) _buttons _currentindex))
  (bind _returnvalue (Transformation|GetActorLocation _output))
  ;[1 1 1] Set Location For Box
  (bind _output_get (Variables|Default|SetTargetLocation (Math|Vector|MakeVector (.x _returnvalue) (.y _returnvalue) (+ (.z _returnvalue) 5e+01))))
  (Transformation|SetActorLocation _output_get false false))

(event EventTick
  (params (DeltaSeconds :type Float%20%28single-precision%29))
  ;[1 1 1] Smooth Transition Between Locations
  (Transformation|SetActorLocation (Math|Vector|Lerp(Vector) (Transformation|GetActorLocation) (Variables|Default|GetTargetLocation) (* DeltaSeconds 5.0)) false false))

(fn ConstructionScript)