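; Puzzle wall that moves vertically when its count of active triggers reaches the required number.
; ObjectActivated and ObjectDeactivated adjust the count, playing or reversing the door Timeline; Tick also fires activation once at the threshold.
; An optional camera focus blends the view to the wall with UI-only input.
; When the Timeline finishes, the view, game input and character walk speeds are set back for play.
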(event EventBeginPlay)

(event Collision|EventActorBeginOverlap
  (params (OtherActor :type Actor%20Object%20Reference)))

(event EventTick
  (params (DeltaSeconds :type Float%20%28single-precision%29))
  (if (>= (Variables|Default|GetTriggersActive) (Variables|Default|GetTriggersNeeded))
    (Utilities|FlowControl|DoOnce false
      (:Completed
        (CallFunction|ObjectActivated)))))

(event EventObjectDeactivated
  ;[1 1 1] Door Activation/Deactivation
  (Math|Integer|DecrementInt (Variables|Default|GetTriggersActive)
    (:%20%20
      (if (>= (Variables|Default|GetTriggersActive) (Variables|Default|GetTriggersNeeded))
        (if (Variables|Default|GetCameraActive)
          (Components|Activation|Activate (Variables|Default|GetCamera) false)
          (if (Variables|Default|GetPlayed)
            (bind _doorposition (Timeline|Timeline Play)
              (:Update
                (Transformation|SetRelativeLocation (Variables|Default|GetWall) (Math|Vector|MakeVector 0.0 0.0 _doorposition) false false))
              (:Finished
                (CallFunction|FocusEnd)
                (if (Variables|Default|GetDoorIsOpen)
                  (Variables|Default|SetPlayed true))))
            (else
              (CallFunction|FocusStart)
              (Timeline|Timeline Play)))
          (else
            (Components|Activation|Deactivate (Variables|Default|GetCamera))
            (Timeline|Timeline Play)))
        (else
          (Timeline|Timeline Reverse))))))

(event EventObjectActivated
  ;[1 1 1] Door Activation/Deactivation
  (Math|Integer|IncrementInt (Variables|Default|GetTriggersActive)
    (:%20%20
      (if (Variables|Default|GetShouldBeDelayed)
        (Utilities|FlowControl|Delay 0.3))
      (if (>= (Variables|Default|GetTriggersActive) (Variables|Default|GetTriggersNeeded))
        (if (Variables|Default|GetCameraActive)
          (Components|Activation|Activate (Variables|Default|GetCamera) false)
          (if (Variables|Default|GetPlayed)
            (bind _doorposition (Timeline|Timeline Play)
              (:Update
                (Transformation|SetRelativeLocation (Variables|Default|GetWall) (Math|Vector|MakeVector 0.0 0.0 _doorposition) false false))
              (:Finished
                (CallFunction|FocusEnd)
                (if (Variables|Default|GetDoorIsOpen)
                  (Variables|Default|SetPlayed true))))
            (else
              (CallFunction|FocusStart)
              (Timeline|Timeline Play)))
          (else
            (Components|Activation|Deactivate (Variables|Default|GetCamera))
            (Timeline|Timeline Play)))
        (else
          (Timeline|Timeline Reverse))))))

(event EventFocusStart
  (Utilities|FlowControl|DoOnce false
    (:Completed
      (Game|Player|SetViewTargetwithBlend (Game|GetPlayerController 0) self 2.0 "VTBlend_EaseInOut" 1.0 true)
      (Input|SetInputModeUIOnly (Game|GetPlayerController 0) 0 "DoNotLock" false))))

(event EventFocusEnd
  (Game|Player|SetViewTargetwithBlend (Game|GetPlayerController 0) (Game|GetPlayerCharacter 0) 2.0 "VTBlend_EaseInOut" 1.0 true)
  (Input|SetInputModeGameOnly (Game|GetPlayerController 0) false)
  (bind _asbp_third_person_character (Utilities|Casting|CastToBP_ThirdPersonCharacter (Game|GetPlayerCharacter 0)))
  (Variables|/Script/Engine.CharacterMovementComponent|SetMinAnalogWalkSpeed (Variables|/Script/Engine.Character|GetCharacterMovement _asbp_third_person_character) 9e+01)
  (Variables|/Script/Engine.CharacterMovementComponent|SetMaxWalkSpeed (Variables|/Script/Engine.Character|GetCharacterMovement _asbp_third_person_character) 3.5e+02))

(fn ConstructionScript)