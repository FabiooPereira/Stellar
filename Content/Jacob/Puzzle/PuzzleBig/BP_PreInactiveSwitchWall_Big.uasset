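; A large puzzle switch wall Blueprint, named as a pre-inactive variant, with an empty event graph and construction script.
; GetForceResponsiveObject capsule-traces a short distance along the actor's forward vector for WorldDynamic objects, returning the hit actor on True or exiting through False.
; ComponentIsChild reports whether a given component's parent actor is this wall.
; Neither helper is called within this Blueprint.
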(event EventBeginPlay)

(event EventTick
  (params (DeltaSeconds :type Float%20%28single-precision%29)))

(fn ConstructionScript)

(fn ComponentIsChild
  (params (Component :type Actor%20Object%20Reference%20%28by%20ref%29))
  (return (== (Actor|GetParentActor Component) self)))