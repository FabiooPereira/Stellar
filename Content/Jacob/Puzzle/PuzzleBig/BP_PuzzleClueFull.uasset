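; BP_PuzzleClueFull is a puzzle clue actor that moves three boxes vertically while something overlaps its OverlapArea.
; Begin and end overlap set ShouldReverse, then MoveCubes plays or reverses the timelines.
; Each timeline drives one box's Z, and the first two start the next from their Update, chaining Box1 to Box3.
; The Light's material switches when the first timeline finishes forward and resets when reversal begins.
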(event OnComponentBeginOverlap(OverlapArea)
  (params (OverlappedComponent :type Primitive%20Component%20Object%20Reference) (OtherActor :type Actor%20Object%20Reference) (OtherComp :type Primitive%20Component%20Object%20Reference) (OtherBodyIndex :type Integer) (bFromSweep :type Boolean) (SweepResult :type Hit%20Result%20Structure%20%28by%20ref%29))
  ;[1 1 1] Overlap Begin/End
  (Variables|Default|SetShouldReverse false)
  (CallFunction|MoveCubes))

(event OnComponentEndOverlap(OverlapArea)
  (params (OverlappedComponent :type Primitive%20Component%20Object%20Reference) (OtherActor :type Actor%20Object%20Reference) (OtherComp :type Primitive%20Component%20Object%20Reference) (OtherBodyIndex :type Integer))
  ;[1 1 1] Overlap Begin/End
  (Variables|Default|SetShouldReverse true)
  (CallFunction|MoveCubes))

(event Custom|MoveCubes
  ;[1 1 1] Move Cubes
  (if (Variables|Default|GetShouldReverse)
    (Rendering|Material|SetMaterial (Variables|Default|GetLight) 0 "/Engine/BasicShapes/BasicShapeMaterial.BasicShapeMaterial")
    (bind _newtrack_0 (Timeline|Timeline Reverse)
      (:Update
        (Transformation|SetRelativeLocation (Variables|Default|GetBox1) (Math|Vector|MakeVector -24.999999 13.59642 _newtrack_0) false false)
        (if (Variables|Default|GetShouldReverse)
          (bind _newtrack_0_2 (Timeline|Timeline_1 Reverse)
            (:Update
              (Transformation|SetRelativeLocation (Variables|Default|GetBox2) (Math|Vector|MakeVector 1e-06 13.59642 _newtrack_0_2) false false)
              (if (Variables|Default|GetShouldReverse)
                (bind _newtrack_0_3 (Timeline|Timeline_0 Reverse)
                  (:Update
                    (Transformation|SetRelativeLocation (Variables|Default|GetBox3) (Math|Vector|MakeVector 25.000001 13.59642 _newtrack_0_3) false false)))
                (else
                  (Timeline|Timeline_0 Play)))))
          (else
            (Timeline|Timeline_1 Play))))
      (:Finished
        (if (not (Variables|Default|GetShouldReverse))
          (Rendering|Material|SetMaterial (Variables|Default|GetLight) 0 "/Engine/EngineMaterials/DefaultLightFunctionMaterial.DefaultLightFunctionMaterial"))))
    (else
      (Timeline|Timeline Play))))

(event EventBeginPlay)

(event Collision|EventActorBeginOverlap
  (params (OtherActor :type Actor%20Object%20Reference)))

(event EventTick
  (params (DeltaSeconds :type Float%20%28single-precision%29)))

(fn ConstructionScript)