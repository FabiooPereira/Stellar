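; Puzzle bridge actor that rotates into or out of place according to how many pressure switches are active.
; Activate and deactivate events adjust a counter, then share a threshold check that plays or reverses the BridgeActivate timeline, which drives the bridge's roll.
; Each timeline update turns the blocking collider off after a short delay when ready, or back on otherwise.
; The bridge sound plays with random pitch only while the Lever's switch is not activated.
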(event EventBeginPlay)

(event Collision|EventActorBeginOverlap
  (params (OtherActor :type Actor%20Object%20Reference)))

(event EventTick
  (params (DeltaSeconds :type Float%20%28single-precision%29)))

(event EventObjectActivated
  ;[1 1 1] Stone Activation
  (Math|Integer|IncrementInt (Variables|Default|GetPressureSwitchesActive)
    (:%20%20
      (if (>= (Variables|Default|GetPressureSwitchesActive) (Variables|Default|GetPressureSwitchesNeeded))
        (Variables|Default|SetReadyToEnter true)
        (if (Variables|/Game/Jacob/BP_Lever_Parent.BP_Lever_Parent_C|GetSwitchActivated (Variables|Default|GetLever))
          (bind _rotation (Timeline|BridgeActivate Play)
            (:Update
              (Transformation|SetRelativeRotation (Variables|Default|GetBridge) (Math|Rotator|MakeRotator _rotation 0.0 0.0) false false)
              (if (Variables|Default|GetReadyToEnter)
                (Utilities|FlowControl|Delay 1.5)
                (Collision|SetCollisionEnabled (Variables|Default|GetCollider) "NoCollision")
                (else
                  (Collision|SetCollisionEnabled (Variables|Default|GetCollider) "QueryAndPhysics")))))
          (else
            (Audio|PlaySoundatLocation "/Game/Kio/Import/SFX_Bridge.SFX_Bridge" (Transformation|GetWorldLocation (Variables|Default|GetBridge)) "0, 0, 0" 0.2 (Math|Random|RandomFloat) 0.0 "/Game/Jacob/Sounds/MusicZoneAttenuation.MusicZoneAttenuation" 0 0 0)
            (Timeline|BridgeActivate Play)))
        (else
          (Variables|Default|SetReadyToEnter false)
          (if (Variables|/Game/Jacob/BP_Lever_Parent.BP_Lever_Parent_C|GetSwitchActivated (Variables|Default|GetLever))
            (Timeline|BridgeActivate Reverse)
            (else
              (Audio|PlaySoundatLocation "/Game/Kio/Import/SFX_Bridge.SFX_Bridge" (Transformation|GetWorldLocation (Variables|Default|GetBridge)) "0, 0, 0" 0.2 (Math|Random|RandomFloat) 0.0 "/Game/Jacob/Sounds/MusicZoneAttenuation.MusicZoneAttenuation" 0 0 0)
              (Timeline|BridgeActivate Reverse))))))))

(event EventObjectDeactivated
  ;[1 1 1] Stone Activation
  (Math|Integer|DecrementInt (Variables|Default|GetPressureSwitchesActive)
    (:%20%20
      (if (>= (Variables|Default|GetPressureSwitchesActive) (Variables|Default|GetPressureSwitchesNeeded))
        (Variables|Default|SetReadyToEnter true)
        (if (Variables|/Game/Jacob/BP_Lever_Parent.BP_Lever_Parent_C|GetSwitchActivated (Variables|Default|GetLever))
          (bind _rotation (Timeline|BridgeActivate Play)
            (:Update
              (Transformation|SetRelativeRotation (Variables|Default|GetBridge) (Math|Rotator|MakeRotator _rotation 0.0 0.0) false false)
              (if (Variables|Default|GetReadyToEnter)
                (Utilities|FlowControl|Delay 1.5)
                (Collision|SetCollisionEnabled (Variables|Default|GetCollider) "NoCollision")
                (else
                  (Collision|SetCollisionEnabled (Variables|Default|GetCollider) "QueryAndPhysics")))))
          (else
            (Audio|PlaySoundatLocation "/Game/Kio/Import/SFX_Bridge.SFX_Bridge" (Transformation|GetWorldLocation (Variables|Default|GetBridge)) "0, 0, 0" 0.2 (Math|Random|RandomFloat) 0.0 "/Game/Jacob/Sounds/MusicZoneAttenuation.MusicZoneAttenuation" 0 0 0)
            (Timeline|BridgeActivate Play)))
        (else
          (Variables|Default|SetReadyToEnter false)
          (if (Variables|/Game/Jacob/BP_Lever_Parent.BP_Lever_Parent_C|GetSwitchActivated (Variables|Default|GetLever))
            (Timeline|BridgeActivate Reverse)
            (else
              (Audio|PlaySoundatLocation "/Game/Kio/Import/SFX_Bridge.SFX_Bridge" (Transformation|GetWorldLocation (Variables|Default|GetBridge)) "0, 0, 0" 0.2 (Math|Random|RandomFloat) 0.0 "/Game/Jacob/Sounds/MusicZoneAttenuation.MusicZoneAttenuation" 0 0 0)
              (Timeline|BridgeActivate Reverse))))))))

(fn ConstructionScript)