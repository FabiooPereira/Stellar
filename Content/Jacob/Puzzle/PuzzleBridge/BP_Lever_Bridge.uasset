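; BP_Lever_Bridge is a one-shot interactable lever that activates a linked puzzle bridge.
; SetInteractableState toggles a text prompt and a custom depth highlight on the lever and base until the lever is used.
; Interact latches SwitchActivated, zeroes the bridge's TriggersNeeded, sends it ObjectActivatedMessage, and plays a timeline that pitches the lever while hiding the prompt and highlight.
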(event EventBeginPlay)

(event EventTick
  (params (DeltaSeconds :type Float%20%28single-precision%29))
  ;[1 1 1] Tick
  (if true
    _))

(event EventSetInteractableState
  (params (bCanShowInteract :type Boolean))
  ;[1 1 1] Interactable State
  (if (not (Variables|Default|GetSwitchActivated))
    (bind _output_get (Variables|Default|SetbCanInteract? bCanShowInteract))
    (if _output_get
      (CallFunction|TextEnable)
      (Rendering|SetRenderCustomDepth (Variables|Default|GetLever) true)
      (else
        (CallFunction|TextDisable)
        (Rendering|SetRenderCustomDepth (Variables|Default|GetLever) false)))))

(event EventInteract
  (params (Instigator :type Actor%20Object%20Reference))
  ;[1 1 1] Switch Trigger
  (if (not (Variables|Default|GetSwitchActivated))
    (Variables|Default|SetSwitchActivated true)
    (Variables|/Game/Jacob/BP_ObjectToTrigger_Parent.BP_ObjectToTrigger_Parent_C|SetTriggersNeeded (Variables|Default|GetBridgeToActivate) 0)
    (Class|BPIEventTrigger|ObjectActivated(Message) (Variables|Default|GetBridgeToActivate))
    (bind _switchposition (Timeline|Timeline_0 Play)
      (:Update
        (Transformation|SetRelativeRotation (Variables|Default|GetLever) (Math|Rotator|MakeRotator 0.0 _switchposition 0.0) false false)
        (CallFunction|TextDisable)
        (Rendering|SetRenderCustomDepth (Variables|Default|GetLever) false)))))

(fn ConstructionScript)