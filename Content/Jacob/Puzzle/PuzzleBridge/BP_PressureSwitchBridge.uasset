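; A pressure switch puzzle actor that activates a linked bridge while something overlaps its trigger.
; Overlaps are counted up to two; a DoOnce activates BridgeToActivate and makes the Base material emissive.
; Ending an overlap at any count other than two deactivates the bridge, restores the material and resets the DoOnce.
; An unused, buggy-labelled branch would snap a traced force-responsive object onto the switch, and counts are debug-printed.
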(event OnComponentBeginOverlap(OverlapBegin)
  (params (OverlappedComponent :type Primitive%20Component%20Object%20Reference) (OtherActor :type Actor%20Object%20Reference) (OtherComp :type Primitive%20Component%20Object%20Reference) (OtherBodyIndex :type Integer) (bFromSweep :type Boolean) (SweepResult :type Hit%20Result%20Structure%20%28by%20ref%29))
  (bind _overlapcount (Variables|Default|GetOverlapCount))
  ;[1 1 1] Switch Trigger
  (if (< (Variables|Default|GetOverlapCount) 2)
    (Math|Integer|IncrementInt _overlapcount
      (:%20%20
        (Development|PrintString (Utilities|String|ToString(Integer) _overlapcount))
        (Utilities|FlowControl|DoOnce false
          (:Completed
            (Default|SwitchActivatedBridge (Variables|Default|GetBridgeToActivate))
            (Rendering|Material|SetMaterial (Variables|Default|GetBase) 0 "/Engine/EngineMaterials/EmissiveMeshMaterial.EmissiveMeshMaterial")))))))

(event OnComponentEndOverlap(OverlapBegin)
  (params (OverlappedComponent :type Primitive%20Component%20Object%20Reference) (OtherActor :type Actor%20Object%20Reference) (OtherComp :type Primitive%20Component%20Object%20Reference) (OtherBodyIndex :type Integer))
  (bind _bridgetoactivate (Variables|Default|GetBridgeToActivate))
  (bind _overlapcount (Variables|Default|GetOverlapCount))
  (bind _base (Variables|Default|GetBase))
  (bind _overlapcount_2 (Variables|Default|GetOverlapCount))
  ;[1 1 1] Switch Trigger
  (if (== (Variables|Default|GetOverlapCount) 2)
    (Math|Integer|DecrementInt _overlapcount
      (:%20%20
        (Development|PrintString (Utilities|String|ToString(Integer) _overlapcount))))
    (else
      (Math|Integer|DecrementInt _overlapcount_2
        (:%20%20
          (Development|PrintString (Utilities|String|ToString(Integer) _overlapcount_2))
          (Default|SwitchDeactivatedBridge _bridgetoactivate)
          (Rendering|Material|SetMaterial _base 0 "/Engine/BasicShapes/BasicShapeMaterial.BasicShapeMaterial")
          (Utilities|FlowControl|DoOnce false) ; enters at Reset
        )))))

(event EventBeginPlay)

(event EventTick
  (params (DeltaSeconds :type Float%20%28single-precision%29)))

(fn ConstructionScript)

(fn ComponentIsChild
  (params (Component :type Actor%20Object%20Reference%20%28by%20ref%29))
  (return (== (Actor|GetParentActor Component) self)))