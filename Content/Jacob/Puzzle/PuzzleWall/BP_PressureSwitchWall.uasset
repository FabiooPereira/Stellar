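; BP_PressureSwitchWall is a puzzle pressure switch that drives a linked wall while something overlaps its trigger box.
; Begin overlap gives the base an emissive material and calls SwitchActivatedWall on WallToActivate; end overlap restores the basic material and calls SwitchDeactivatedWall.
; Overlaps are not filtered or counted.
; An unused, buggy-labelled snap routine would capsule-trace for a BP_ForceResponsiveObject, detach it and reposition it.
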(event OnComponentBeginOverlap(OverlapBox)
  (params (OverlappedComponent :type Primitive%20Component%20Object%20Reference) (OtherActor :type Actor%20Object%20Reference) (OtherComp :type Primitive%20Component%20Object%20Reference) (OtherBodyIndex :type Integer) (bFromSweep :type Boolean) (SweepResult :type Hit%20Result%20Structure%20%28by%20ref%29))
  ;[1 1 1] Switch Trigger
  (Rendering|Material|SetMaterial (Variables|Default|GetBase) 0 "/Engine/EngineMaterials/EmissiveMeshMaterial.EmissiveMeshMaterial")
  (Default|SwitchActivatedWall (Variables|Default|GetWallToActivate)))

(event OnComponentEndOverlap(OverlapBox)
  (params (OverlappedComponent :type Primitive%20Component%20Object%20Reference) (OtherActor :type Actor%20Object%20Reference) (OtherComp :type Primitive%20Component%20Object%20Reference) (OtherBodyIndex :type Integer))
  ;[1 1 1] Switch Trigger
  (Rendering|Material|SetMaterial (Variables|Default|GetBase) 0 "/Engine/BasicShapes/BasicShapeMaterial.BasicShapeMaterial")
  (Default|SwitchDeactivatedWall (Variables|Default|GetWallToActivate)))

(event EventBeginPlay)

(event EventTick
  (params (DeltaSeconds :type Float%20%28single-precision%29)))

(fn ConstructionScript)

(fn ComponentIsChild
  (params (Component :type Actor%20Object%20Reference%20%28by%20ref%29))
  (return (== (Actor|GetParentActor Component) self)))