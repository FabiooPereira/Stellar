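; Puzzle wall actor that moves vertically once enough linked triggers are active.
; ObjectActivated and ObjectDeactivated adjust an active-trigger count, then compare it with TriggersNeeded to play or reverse the WallActivation timeline driving the wall's relative Z.
; A bridge sound with random pitch plays on opening, and on reversing once DoorIsDown is set, a flag that is never cleared.
; Camera view-blend nodes are left unconnected.
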(event EventBeginPlay)

(event Collision|EventActorBeginOverlap
  (params (OtherActor :type Actor%20Object%20Reference)))

(event EventTick
  (params (DeltaSeconds :type Float%20%28single-precision%29)))

(event EventObjectDeactivated
  ;[1 1 1] Door Activation/Deactivation
  (Math|Integer|DecrementInt (Variables|Default|GetTriggersActive)
    (:%20%20
      (if (>= (Variables|Default|GetTriggersActive) (Variables|Default|GetTriggersNeeded))
        (Variables|Default|SetDoorIsDown true)
        (Audio|PlaySoundatLocation "/Game/Kio/Import/SFX_Bridge.SFX_Bridge" (Transformation|GetWorldLocation (Variables|Default|GetWall)) "0, 0, 0" 0.2 (Math|Random|RandomFloat) 0.0 "/Game/Jacob/Sounds/MusicZoneAttenuation.MusicZoneAttenuation" 0 0 0)
        (bind _doorposition (Timeline|WallActivation Play)
          (:Update
            (Transformation|SetRelativeLocation (Variables|Default|GetWall) (Math|Vector|MakeVector 0.0 0.0 _doorposition) false false)))
        (elif (Variables|Default|GetDoorIsDown)
          (Audio|PlaySoundatLocation "/Game/Kio/Import/SFX_Bridge.SFX_Bridge" (Transformation|GetWorldLocation (Variables|Default|GetWall)) "0, 0, 0" 0.2 (Math|Random|RandomFloat) 0.0 "/Game/Jacob/Sounds/MusicZoneAttenuation.MusicZoneAttenuation" 0 0 0)
          (Timeline|WallActivation Reverse)
          (else
            (Timeline|WallActivation Reverse)))))))

(event EventObjectActivated
  ;[1 1 1] Door Activation/Deactivation
  (Math|Integer|IncrementInt (Variables|Default|GetTriggersActive)
    (:%20%20
      (if (>= (Variables|Default|GetTriggersActive) (Variables|Default|GetTriggersNeeded))
        (Variables|Default|SetDoorIsDown true)
        (Audio|PlaySoundatLocation "/Game/Kio/Import/SFX_Bridge.SFX_Bridge" (Transformation|GetWorldLocation (Variables|Default|GetWall)) "0, 0, 0" 0.2 (Math|Random|RandomFloat) 0.0 "/Game/Jacob/Sounds/MusicZoneAttenuation.MusicZoneAttenuation" 0 0 0)
        (bind _doorposition (Timeline|WallActivation Play)
          (:Update
            (Transformation|SetRelativeLocation (Variables|Default|GetWall) (Math|Vector|MakeVector 0.0 0.0 _doorposition) false false)))
        (elif (Variables|Default|GetDoorIsDown)
          (Audio|PlaySoundatLocation "/Game/Kio/Import/SFX_Bridge.SFX_Bridge" (Transformation|GetWorldLocation (Variables|Default|GetWall)) "0, 0, 0" 0.2 (Math|Random|RandomFloat) 0.0 "/Game/Jacob/Sounds/MusicZoneAttenuation.MusicZoneAttenuation" 0 0 0)
          (Timeline|WallActivation Reverse)
          (else
            (Timeline|WallActivation Reverse)))))))

(fn ConstructionScript)