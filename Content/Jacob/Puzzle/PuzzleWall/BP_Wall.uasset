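; BP_Wall is a puzzle wall that moves vertically in response to pressure switches.
; Activation and deactivation events keep a count of active switches and compare it to the number needed.
; Meeting the threshold plays a timeline that sets the wall mesh's relative Z, while falling short reverses it.
; Camera blends to the wall and back to the player are present but unconnected, so they never run.
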(event Custom|SwitchActivatedWall
  ;[1 1 1] Door Activation/Deactivation
  (Math|Integer|IncrementInt (Variables|Default|GetPressureSwitchesActive)
    (:%20%20
      (if (>= (Variables|Default|GetPressureSwitchesActive) (Variables|Default|GetPressureSwitchesNeeded))
        (bind _doorposition (Timeline|WallActivation Play)
          (:Update
            (Transformation|SetRelativeLocation (Variables|Default|GetWall) (Math|Vector|MakeVector 0.0 0.0 _doorposition) false false)))
        (else
          (Timeline|WallActivation Reverse))))))

(event Custom|SwitchDeactivatedWall
  ;[1 1 1] Door Activation/Deactivation
  (Math|Integer|DecrementInt (Variables|Default|GetPressureSwitchesActive)
    (:%20%20
      (if (>= (Variables|Default|GetPressureSwitchesActive) (Variables|Default|GetPressureSwitchesNeeded))
        (bind _doorposition (Timeline|WallActivation Play)
          (:Update
            (Transformation|SetRelativeLocation (Variables|Default|GetWall) (Math|Vector|MakeVector 0.0 0.0 _doorposition) false false)))
        (else
          (Timeline|WallActivation Reverse))))))

(event EventBeginPlay)

(event Collision|EventActorBeginOverlap
  (params (OtherActor :type Actor%20Object%20Reference)))

(event EventTick
  (params (DeltaSeconds :type Float%20%28single-precision%29)))

(fn ConstructionScript)