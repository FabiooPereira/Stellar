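; A puzzle bridge that shuttles between two marker positions while enough pressure switches are active.
; ObjectActivated and ObjectDeactivated adjust a switch count that sets ReadyToEnter.
; While ready, Tick eases the bridge toward its target with VInterpTo, and a FlipFlop swaps the target between Location1 and Location2 whenever it gets close.
; The bridge halts in place when too few switches remain active; disconnected collision-toggle nodes never run.
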(event EventBeginPlay
  (Variables|Default|SetTargetLocation (Variables|/Script/Engine.SceneComponent|GetRelativeLocation (Variables|Default|GetLocation2))))

(event EventTick
  (params (DeltaSeconds :type Float%20%28single-precision%29))
  ;[1 1 1] Tick
  (CallFunction|SetLocationContinuous DeltaSeconds))

(event EventObjectActivated
  ;[1 1 1] Bridge Activation
  (Math|Integer|IncrementInt (Variables|Default|GetPressureSwitchesActive)
    (:%20%20
      (if (>= (Variables|Default|GetPressureSwitchesActive) (Variables|Default|GetPressureSwitchesNeeded))
        (Variables|Default|SetReadyToEnter true)
        (else
          (Variables|Default|SetReadyToEnter false))))))

(event EventObjectDeactivated
  ;[1 1 1] Bridge Activation
  (Math|Integer|DecrementInt (Variables|Default|GetPressureSwitchesActive)
    (:%20%20
      (if (>= (Variables|Default|GetPressureSwitchesActive) (Variables|Default|GetPressureSwitchesNeeded))
        (Variables|Default|SetReadyToEnter true)
        (else
          (Variables|Default|SetReadyToEnter false))))))

(fn ConstructionScript)

(fn SetLocationContinuous
  (params (DeltaTime :type Float%20%28single-precision%29))
  (if (Variables|Default|GetReadyToEnter)
    (Transformation|SetRelativeLocation (Variables|Default|GetBridge) (Math|Interpolation|VInterpTo (Variables|/Script/Engine.SceneComponent|GetRelativeLocation (Variables|Default|GetBridge)) (Variables|Default|GetTargetLocation) (* DeltaTime 4.0) 0.2) false false)
    (if (Utilities|Operators|EqualEqual (Variables|/Script/Engine.SceneComponent|GetRelativeLocation (Variables|Default|GetBridge)) (Variables|Default|GetTargetLocation) 1e+01)
      (Utilities|FlowControl|FlipFlop
        (:A
          (Variables|Default|SetTargetLocation (Variables|/Script/Engine.SceneComponent|GetRelativeLocation (Variables|Default|GetLocation1))))
        (:B
          (Variables|Default|SetTargetLocation (Variables|/Script/Engine.SceneComponent|GetRelativeLocation (Variables|Default|GetLocation2))))))))