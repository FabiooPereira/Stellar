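; Elevator for the rotating bridges puzzle that shuttles a platform between two marker locations once the player activates it.
; When the player character overlaps the trigger box, a one-second delay sets a flag that is never cleared.
; While the flag is set, Tick eases the platform toward the current target with VInterpTo.
; A FlipFlop swaps the target whenever the platform gets close, so it loops indefinitely.
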(event OnComponentBeginOverlap(Box)
  (params (OverlappedComponent :type Primitive%20Component%20Object%20Reference) (OtherActor :type Actor%20Object%20Reference) (OtherComp :type Primitive%20Component%20Object%20Reference) (OtherBodyIndex :type Integer) (bFromSweep :type Boolean) (SweepResult :type Hit%20Result%20Structure%20%28by%20ref%29))
  (if (== OtherActor (Game|GetPlayerCharacter 0))
    (Utilities|FlowControl|Delay 1.0)
    (Variables|Default|SetReady%20to%20Enter true)))

(event EventBeginPlay
  (Variables|Default|SetTarget%20Location (Variables|/Script/Engine.SceneComponent|GetRelativeLocation (Variables|Default|GetLocation2))))

(event EventTick
  (params (DeltaSeconds :type Float%20%28single-precision%29))
  (if (Variables|Default|GetReady%20to%20Enter)
    (Transformation|SetRelativeLocation (Variables|Default|GetElevator) (Math|Interpolation|VInterpTo (Variables|/Script/Engine.SceneComponent|GetRelativeLocation (Variables|Default|GetElevator)) (Variables|Default|GetTarget%20Location) (* DeltaSeconds 4.0) 0.2) false false)
    (if (Utilities|Operators|EqualEqual (Variables|/Script/Engine.SceneComponent|GetRelativeLocation (Variables|Default|GetElevator)) (Variables|Default|GetTarget%20Location) 1e+01)
      (Utilities|FlowControl|FlipFlop
        (:A
          (Variables|Default|SetTarget%20Location (Variables|/Script/Engine.SceneComponent|GetRelativeLocation (Variables|Default|GetLocation1))))
        (:B
          (Variables|Default|SetTarget%20Location (Variables|/Script/Engine.SceneComponent|GetRelativeLocation (Variables|Default|GetLocation2))))))))

(fn ConstructionScript)