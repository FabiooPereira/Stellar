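; Puzzle bridge actor that, despite its rotating-bridge name, raises or lowers along Z when triggered.
; ObjectActivated and ObjectDeactivated adjust an active pressure-switch count and set ReadyToEnter against the required count.
; Either event then toggles RotationValue to play or reverse the UpDown timeline, regardless of that threshold.
; Rotation timeline and collision-toggle nodes are left unconnected.
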(event EventBeginPlay)

(event Collision|EventActorBeginOverlap
  (params (OtherActor :type Actor%20Object%20Reference)))

(event EventTick
  (params (DeltaSeconds :type Float%20%28single-precision%29)))

(event EventObjectActivated
  ;[1 1 1] Bridge Activation
  (Math|Integer|IncrementInt (Variables|Default|GetPressureSwitchesActive)
    (:%20%20
      (if (>= (Variables|Default|GetPressureSwitchesActive) (Variables|Default|GetPressureSwitchesNeeded))
        (Variables|Default|SetReadyToEnter true)
        (else
          (Variables|Default|SetReadyToEnter false)))
      (if (== (Variables|Default|GetRotationValue) 0.0)
        (Variables|Default|SetRotationValue 9e+01)
        (bind _location_z (Timeline|Up/Down Play)
          (:Update
            (Transformation|SetRelativeLocation (Variables|Default|GetBridge) (Math|Vector|MakeVector 0.0 0.0 _location_z) false false)
            (if (Variables|Default|GetReadyToEnter)
              _)))
        (else
          (Variables|Default|SetRotationValue 0.0)
          (Timeline|Up/Down Reverse))))))

(event EventObjectDeactivated
  ;[1 1 1] Bridge Activation
  (Math|Integer|DecrementInt (Variables|Default|GetPressureSwitchesActive)
    (:%20%20
      (if (>= (Variables|Default|GetPressureSwitchesActive) (Variables|Default|GetPressureSwitchesNeeded))
        (Variables|Default|SetReadyToEnter true)
        (else
          (Variables|Default|SetReadyToEnter false)))
      (if (== (Variables|Default|GetRotationValue) 0.0)
        (Variables|Default|SetRotationValue 9e+01)
        (bind _location_z (Timeline|Up/Down Play)
          (:Update
            (Transformation|SetRelativeLocation (Variables|Default|GetBridge) (Math|Vector|MakeVector 0.0 0.0 _location_z) false false)
            (if (Variables|Default|GetReadyToEnter)
              _)))
        (else
          (Variables|Default|SetRotationValue 0.0)
          (Timeline|Up/Down Reverse))))))

(fn ConstructionScript)