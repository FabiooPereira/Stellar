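; Pressure switch for the rotating bridges puzzle that activates linked bridges while something stands on its trigger box.
; Begin overlap sends an activate message to each entry in BridgesToActivate and sets an emissive base material; end overlap sends deactivate and restores the basic material.
; Overlap-counting macros, capped at two and printing the count, work with a DoOnce so activation fires once and releases when the last counted overlap ends.
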(event OnComponentBeginOverlap(Box)
  (params (OverlappedComponent :type Primitive%20Component%20Object%20Reference) (OtherActor :type Actor%20Object%20Reference) (OtherComp :type Primitive%20Component%20Object%20Reference) (OtherBodyIndex :type Integer) (bFromSweep :type Boolean) (SweepResult :type Hit%20Result%20Structure%20%28by%20ref%29))
  ;[1 1 1] Switch Trigger
  (|CanBeginOverlap_2)
  (Utilities|FlowControl|DoOnce false
    (:Completed
      (for _array_element (Variables|Default|GetBridgesToActivate)
        (Class|BPIEventTrigger|ObjectActivated(Message) _array_element)
        (Rendering|Material|SetMaterial (Variables|Default|GetBase) 0 "/Engine/EngineMaterials/EmissiveMeshMaterial.EmissiveMeshMaterial")))))

(event OnComponentEndOverlap(Box)
  (params (OverlappedComponent :type Primitive%20Component%20Object%20Reference) (OtherActor :type Actor%20Object%20Reference) (OtherComp :type Primitive%20Component%20Object%20Reference) (OtherBodyIndex :type Integer))
  (bind _base (Variables|Default|GetBase))
  (bind _bridgestoactivate (Variables|Default|GetBridgesToActivate))
  ;[1 1 1] Switch Trigger
  (|CanEndOverlap_2)
  (for _array_element _bridgestoactivate
    (Class|BPIEventTrigger|ObjectDeactivated(Message) _array_element)
    (Rendering|Material|SetMaterial _base 0 "/Engine/BasicShapes/BasicShapeMaterial.BasicShapeMaterial")
    (Utilities|FlowControl|DoOnce false) ; enters at Reset
  ))

(event EventBeginPlay)

(event Collision|EventActorBeginOverlap
  (params (OtherActor :type Actor%20Object%20Reference)))

(event EventTick
  (params (DeltaSeconds :type Float%20%28single-precision%29)))

(fn ConstructionScript)