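; Puzzle bridge that slides between start and end points once enough triggers are active.
; Activation and deactivation events update a trigger count and toggle a blocking box collider, with IsReversed inverting the collision and a delay before it switches off.
; Tick eases the bridge with VInterpTo, either toward the point matching the trigger state or, in continuous mode, ping-ponging between both via FlipFlop while triggered.
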(event EventBeginPlay
  ;[1 1 1] Begin Play
  (Variables|Default|SetTargetLocation (Variables|/Script/Engine.SceneComponent|GetRelativeLocation (Variables|Default|GetEndLocation))))

(event EventTick
  (params (DeltaSeconds :type Float%20%28single-precision%29))
  ;[1 1 1] Tick
  (if (Variables|Default|GetIsContinuous)
    (|SetLocationContinuous DeltaSeconds)
    (else
      (|SetLocation DeltaSeconds))))

(event EventObjectActivated
  ;[1 1 1] Bridge Activation
  (Math|Integer|IncrementInt (Variables|Default|GetTriggersActive)
    (:%20%20
      (if (>= (Variables|Default|GetTriggersActive) (Variables|Default|GetTriggersNeeded))
        (Variables|Default|SetReadyToEnter true)
        (else
          (Variables|Default|SetReadyToEnter false)))
      (if (Variables|Default|GetReadyToEnter)
        (if (Variables|Default|GetIsReversed)
          (Collision|SetCollisionEnabled (Variables|Default|GetBoxCollider) "QueryAndPhysics")
          (else
            (Utilities|FlowControl|Delay 1.5)
            (Collision|SetCollisionEnabled (Variables|Default|GetBoxCollider) "NoCollision")))
        (elif (Variables|Default|GetIsReversed)
          (Utilities|FlowControl|Delay 1.5)
          (Collision|SetCollisionEnabled (Variables|Default|GetBoxCollider) "NoCollision")
          (else
            (Collision|SetCollisionEnabled (Variables|Default|GetBoxCollider) "QueryAndPhysics")))))))

(event EventObjectDeactivated
  ;[1 1 1] Bridge Activation
  (Math|Integer|DecrementInt (Variables|Default|GetTriggersActive)
    (:%20%20
      (if (>= (Variables|Default|GetTriggersActive) (Variables|Default|GetTriggersNeeded))
        (Variables|Default|SetReadyToEnter true)
        (else
          (Variables|Default|SetReadyToEnter false)))
      (if (Variables|Default|GetReadyToEnter)
        (if (Variables|Default|GetIsReversed)
          (Collision|SetCollisionEnabled (Variables|Default|GetBoxCollider) "QueryAndPhysics")
          (else
            (Utilities|FlowControl|Delay 1.5)
            (Collision|SetCollisionEnabled (Variables|Default|GetBoxCollider) "NoCollision")))
        (elif (Variables|Default|GetIsReversed)
          (Utilities|FlowControl|Delay 1.5)
          (Collision|SetCollisionEnabled (Variables|Default|GetBoxCollider) "NoCollision")
          (else
            (Collision|SetCollisionEnabled (Variables|Default|GetBoxCollider) "QueryAndPhysics")))))))

(fn ConstructionScript)