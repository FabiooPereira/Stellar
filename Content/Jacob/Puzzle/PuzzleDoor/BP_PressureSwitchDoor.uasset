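; Pressure switch for a puzzle door that activates its linked door and lights up its base material when something overlaps its box.
; An overlap counter capped at two and a DoOnce gate keep activation single, and deactivation is skipped when the count drops from two.
; Deactivation restores the basic material and resets the gate.
; An unused, buggy branch would snap a traced force-responsive object onto the switch.
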(event OnComponentBeginOverlap(OverlapBox)
  (params (OverlappedComponent :type Primitive%20Component%20Object%20Reference) (OtherActor :type Actor%20Object%20Reference) (OtherComp :type Primitive%20Component%20Object%20Reference) (OtherBodyIndex :type Integer) (bFromSweep :type Boolean) (SweepResult :type Hit%20Result%20Structure%20%28by%20ref%29))
  ;[1 1 1] Switch Trigger
  (|CanBeginOverlap)
  (Utilities|FlowControl|DoOnce false
    (:Completed
      (Rendering|Material|SetMaterial (Variables|Default|GetBase) 0 "/Engine/EngineMaterials/EmissiveMeshMaterial.EmissiveMeshMaterial")
      (Default|SwitchActivatedDoor (Variables|Default|GetDoorToActivate)))))

(event OnComponentEndOverlap(OverlapBox)
  (params (OverlappedComponent :type Primitive%20Component%20Object%20Reference) (OtherActor :type Actor%20Object%20Reference) (OtherComp :type Primitive%20Component%20Object%20Reference) (OtherBodyIndex :type Integer))
  (bind _doortoactivate (Variables|Default|GetDoorToActivate))
  (bind _base (Variables|Default|GetBase))
  ;[1 1 1] Switch Trigger
  (|CanEndOverlap)
  (Rendering|Material|SetMaterial _base 0 "/Engine/BasicShapes/BasicShapeMaterial.BasicShapeMaterial")
  (Default|SwitchDeactivatedDoor _doortoactivate)
  (Utilities|FlowControl|DoOnce false) ; enters at Reset
)

(event EventBeginPlay)

(event EventTick
  (params (DeltaSeconds :type Float%20%28single-precision%29)))

(fn ConstructionScript)

(fn ComponentIsChild
  (params (Component :type Actor%20Object%20Reference%20%28by%20ref%29))
  (return (== (Actor|GetParentActor Component) self)))