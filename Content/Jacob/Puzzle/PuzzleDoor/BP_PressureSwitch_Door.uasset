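; Pressure switch for a door puzzle that notifies its linked DoorToActivate when its overlap box is entered or cleared, swapping the base material to emissive and back.
; Gate graphs track up to two overlaps, printing the count, so one of two leaving keeps the switch active.
; A DoOnce limits activation to once until deactivation resets it.
; An unconnected, buggy snap-to-switch routine for force-responsive objects remains unused.
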(event OnComponentBeginOverlap(OverlapBox)
  (params (OverlappedComponent :type Primitive%20Component%20Object%20Reference) (OtherActor :type Actor%20Object%20Reference) (OtherComp :type Primitive%20Component%20Object%20Reference) (OtherBodyIndex :type Integer) (bFromSweep :type Boolean) (SweepResult :type Hit%20Result%20Structure%20%28by%20ref%29))
  ;[1 1 1] Switch Trigger
  (|CanBeginOverlap)
  (Utilities|FlowControl|DoOnce false
    (:Completed
      (Default|SwitchActivatedDoor (Variables|Default|GetDoorToActivate))
      (Rendering|Material|SetMaterial (Variables|Default|GetBase) 0 "/Engine/EngineMaterials/EmissiveMeshMaterial.EmissiveMeshMaterial"))))

(event OnComponentEndOverlap(OverlapBox)
  (params (OverlappedComponent :type Primitive%20Component%20Object%20Reference) (OtherActor :type Actor%20Object%20Reference) (OtherComp :type Primitive%20Component%20Object%20Reference) (OtherBodyIndex :type Integer))
  (bind _doortoactivate (Variables|Default|GetDoorToActivate))
  (bind _base (Variables|Default|GetBase))
  ;[1 1 1] Switch Trigger
  (|CanEndOverlap)
  (Default|SwitchDeactivatedDoor _doortoactivate)
  (Rendering|Material|SetMaterial _base 0 "/Engine/BasicShapes/BasicShapeMaterial.BasicShapeMaterial")
  (Utilities|FlowControl|DoOnce false) ; enters at Reset
)

(event EventBeginPlay
  (|CallParentFunction) ; This node is disabled and will not be called.\nDrag off pins to build functionality.
)

(event Collision|EventActorBeginOverlap
  (params (OtherActor :type Actor%20Object%20Reference)))

(event EventTick
  (params (DeltaSeconds :type Float%20%28single-precision%29))
  (|CallParentFunction DeltaSeconds) ; This node is disabled and will not be called.\nDrag off pins to build functionality.
)

(fn ConstructionScript
  (|CallParentFunction))