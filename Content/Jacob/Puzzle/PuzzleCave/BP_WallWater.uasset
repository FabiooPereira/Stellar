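; BP_WallWater is a puzzle actor for the water cave that moves a Cube once enough pressure switches are active.
; Switch activated and deactivated events adjust a counter and compare it against the required count, setting ReadyToEnter.
; The BridgeActivate timeline plays at the threshold and reverses below it, driving the Cube's relative Z location through a track named Rotation.
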(event Custom|SwitchActivatedWallWaterCave
  ;[1 1 1] Stone Activation
  (Math|Integer|IncrementInt (Variables|Default|GetPressureSwitchesActiveBridge)
    (:%20%20
      (if (>= (Variables|Default|GetPressureSwitchesActiveBridge) (Variables|Default|GetPressureSwitchesNeededBridge))
        (Variables|Default|SetReadyToEnter true)
        (bind _rotation (Timeline|BridgeActivate Play)
          (:Update
            (Transformation|SetRelativeLocation (Variables|Default|GetCube) (Math|Vector|MakeVector 0.0 0.0 _rotation) false false)))
        (else
          (Variables|Default|SetReadyToEnter false)
          (if (Variables|Default|GetReadyToEnter)
            (Timeline|BridgeActivate Play)
            (else
              (Timeline|BridgeActivate Reverse))))))))

(event Custom|SwitchDeactivatedWallWaterCave
  ;[1 1 1] Stone Activation
  (Math|Integer|DecrementInt (Variables|Default|GetPressureSwitchesActiveBridge)
    (:%20%20
      (if (>= (Variables|Default|GetPressureSwitchesActiveBridge) (Variables|Default|GetPressureSwitchesNeededBridge))
        (Variables|Default|SetReadyToEnter true)
        (bind _rotation (Timeline|BridgeActivate Play)
          (:Update
            (Transformation|SetRelativeLocation (Variables|Default|GetCube) (Math|Vector|MakeVector 0.0 0.0 _rotation) false false)))
        (else
          (Variables|Default|SetReadyToEnter false)
          (if (Variables|Default|GetReadyToEnter)
            (Timeline|BridgeActivate Play)
            (else
              (Timeline|BridgeActivate Reverse))))))))

(event EventBeginPlay)

(event Collision|EventActorBeginOverlap
  (params (OtherActor :type Actor%20Object%20Reference)))

(event EventTick
  (params (DeltaSeconds :type Float%20%28single-precision%29)))

(fn ConstructionScript)