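; BP_Lever_WallCave is a one-use puzzle lever that activates a linked cave wall, usable only while its linked lamp is lit.
; SetInteractableState toggles the prompt text and custom-depth highlight.
; Interact locks the lever, messages WallToActivate, then runs a timeline that rotates the lever and turns it red.
; A GetForceResponsiveObject helper capsule-traces ahead for WorldDynamic actors but is not called here.
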(event EventBeginPlay)

(event EventTick
  (params (DeltaSeconds :type Float%20%28single-precision%29)))

(event EventSetInteractableState
  (params (bCanShowInteract :type Boolean))
  ;[1 1 1] Set Interactable State
  (if (and (Variables|/Game/Marcus/Enemy/BP_Lamp_TEST.BP_Lamp_TEST_C|GetLampIsLIt (Variables|Default|GetLamp)) (Variables|Default|GetLeverIsNotPressed))
    (bind _output_get (Variables|Default|SetbCanInteract? bCanShowInteract))
    (if _output_get
      (CallFunction|TextEnable)
      (Rendering|SetRenderCustomDepth (Variables|Default|GetLever) true)
      (else
        (CallFunction|TextDisable)
        (Rendering|SetRenderCustomDepth (Variables|Default|GetLever) false)))))

(event EventInteract
  (params (Instigator :type Actor%20Object%20Reference))
  ;[1 1 1] Lever Trigger
  (if (and (Variables|/Game/Marcus/Enemy/BP_Lamp_TEST.BP_Lamp_TEST_C|GetLampIsLIt (Variables|Default|GetLamp)) (Variables|Default|GetLeverIsNotPressed))
    (Utilities|FlowControl|DoOnce false :!label _label
      (:Completed
        (Variables|Default|SetLeverIsNotPressed false)
        (Class|BPIEventTrigger|ObjectActivated(Message) (Variables|Default|GetWallToActivate))
        (bind _switchposition (Timeline|Timeline Play)
          (:Update
            (Rendering|Material|SetMaterial (Variables|Default|GetLever) 0 "/Game/Materials/M_Red.M_Red")
            (CallFunction|TextDisable)
            (Transformation|SetRelativeRotation (Variables|Default|GetLever) (Math|Rotator|MakeRotator _switchposition 0.0 0.0) false false))
          (:Finished
            (if (Variables|Default|GetbCanInteract?)
              (Rendering|SetRenderCustomDepth (Variables|Default|GetLever) false)
              (goto _label Reset)
              (else
                (goto _label Reset)))))))))

(fn ConstructionScript)