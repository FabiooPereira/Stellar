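; Cave puzzle pressure switch that activates a linked bridge and lights its base material while occupied, reverting both on release.
; An overlap counter capped at two, with a DoOnce, keeps the switch active until the last occupant leaves.
; A separate text volume detects BP_PlayerJacob and switches NewHUD alpaca prompts through paired DoOnce gates, picking the stay or call text from the AI companion controller's toggle on exit.
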(event OnComponentBeginOverlap(OverlapBox)
  (params (OverlappedComponent :type Primitive%20Component%20Object%20Reference) (OtherActor :type Actor%20Object%20Reference) (OtherComp :type Primitive%20Component%20Object%20Reference) (OtherBodyIndex :type Integer) (bFromSweep :type Boolean) (SweepResult :type Hit%20Result%20Structure%20%28by%20ref%29))
  ;[1 1 1] Switch Trigger
  (|CanBeginOverlap)
  (Utilities|FlowControl|DoOnce false
    (:Completed
      (Default|SwitchActivatedBridgeCave (Variables|Default|GetBridgeToActivate))
      (Rendering|Material|SetMaterial (Variables|Default|GetBase) 0 "/Engine/EngineMaterials/EmissiveMeshMaterial.EmissiveMeshMaterial"))))

(event OnComponentBeginOverlap(TextOverlap)
  (params (OverlappedComponent :type Primitive%20Component%20Object%20Reference) (OtherActor :type Actor%20Object%20Reference) (OtherComp :type Primitive%20Component%20Object%20Reference) (OtherBodyIndex :type Integer) (bFromSweep :type Boolean) (SweepResult :type Hit%20Result%20Structure%20%28by%20ref%29))
  (if (Utilities|ClassIsChildOf (Utilities|GetClass (stale OnComponentEndOverlap(TextOverlap) OtherActor)) "/Game/ThirdPerson/Blueprints/BP_PlayerJacob.BP_PlayerJacob_C")
    (Utilities|FlowControl|DoOnce false
      (:Completed
        (CallFunction|TextEnable)
        (Variables|Default|SetStandingOnPressurePlate true)
        (Utilities|FlowControl|DoOnce false) ; enters at Reset
      ))))

(event OnComponentEndOverlap(OverlapBox)
  (params (OverlappedComponent :type Primitive%20Component%20Object%20Reference) (OtherActor :type Actor%20Object%20Reference) (OtherComp :type Primitive%20Component%20Object%20Reference) (OtherBodyIndex :type Integer))
  (bind _base (Variables|Default|GetBase))
  (bind _bridgetoactivate (Variables|Default|GetBridgeToActivate))
  ;[1 1 1] Switch Trigger
  (|CanEndOverlap)
  (Default|SwitchDeactivatedBridgeCave _bridgetoactivate)
  (Rendering|Material|SetMaterial _base 0 "/Engine/BasicShapes/BasicShapeMaterial.BasicShapeMaterial")
  (Utilities|FlowControl|DoOnce false) ; enters at Reset
)

(event OnComponentEndOverlap(TextOverlap)
  (params (OverlappedComponent :type Primitive%20Component%20Object%20Reference) (OtherActor :type Actor%20Object%20Reference) (OtherComp :type Primitive%20Component%20Object%20Reference) (OtherBodyIndex :type Integer))
  (if (Utilities|ClassIsChildOf (Utilities|GetClass OtherActor) "/Game/ThirdPerson/Blueprints/BP_PlayerJacob.BP_PlayerJacob_C")
    (Utilities|FlowControl|DoOnce false
      (:Completed
        (CallFunction|TextDisableandEnableOtherText)
        (Variables|Default|SetStandingOnPressurePlate false)
        (Utilities|FlowControl|DoOnce false) ; enters at Reset
      ))))

(event EventBeginPlay
  (|CallParentFunction))

(event Collision|EventActorBeginOverlap
  (params (OtherActor :type Actor%20Object%20Reference)))

(event EventTick
  (params (DeltaSeconds :type Float%20%28single-precision%29))
  (|CallParentFunction DeltaSeconds))

(fn ConstructionScript
  (|CallParentFunction))

(fn TextEnable
  (bind _asnew_hud (Utilities|Casting|CastToNewHUD (HUD|GetHUD (Game|GetPlayerController 0))))
  (bind _output_get (Variables|Default|SetAs%20New%20HUD _asnew_hud))
  (Default|AlpacaCalltoButtonText (Variables|/Game/Jacob/NewHUD.NewHUD_C|GetUIRef _output_get) true))

(fn TextDisableandEnableOtherText
  (bind _returnvalue (Actor|GetActorOfClass "/Script/GruppOnion.AICompanionController"))
  (if (Variables|/Script/GruppOnion.AICompanionController|GetCallStayToogle _returnvalue)
    (bind _as_new_hud (Variables|Default|GetAs%20New%20HUD)
      (:then
        (Default|AlpacaStayText (Variables|/Game/Jacob/NewHUD.NewHUD_C|GetUIRef _as_new_hud) true))
      (:else))
    (else
      (bind _as_new_hud_2 (Variables|Default|GetAs%20New%20HUD)
        (:then
          (Default|AlpacaCallText (Variables|/Game/Jacob/NewHUD.NewHUD_C|GetUIRef _as_new_hud_2) true))
        (:else)))))