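; Pressure switch for the water cave puzzle that tracks pushable stones resting on it.
; Overlap box begin and end events accept only BP_PushAndDragObject_Stone actors and call the CanBeginOverlap and CanEndOverlap functions.
; These raise OverlapCount up to a cap of two or lower it, printing the count for debugging; no switch response is wired in this graph.
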(event OnComponentBeginOverlap(OverlapBox)
  (params (OverlappedComponent :type Primitive%20Component%20Object%20Reference) (OtherActor :type Actor%20Object%20Reference) (OtherComp :type Primitive%20Component%20Object%20Reference) (OtherBodyIndex :type Integer) (bFromSweep :type Boolean) (SweepResult :type Hit%20Result%20Structure%20%28by%20ref%29))
  ;[1 1 1] Switch Trigger
  (if (Utilities|ClassIsChildOf (Utilities|GetClass OtherActor) "/Game/Jacob/Push/BP_PushAndDragObject_Stone.BP_PushAndDragObject_Stone_C")
    (|CanBeginOverlap)))

(event OnComponentEndOverlap(OverlapBox)
  (params (OverlappedComponent :type Primitive%20Component%20Object%20Reference) (OtherActor :type Actor%20Object%20Reference) (OtherComp :type Primitive%20Component%20Object%20Reference) (OtherBodyIndex :type Integer))
  ;[1 1 1] Switch Trigger
  (if (Utilities|ClassIsChildOf (Utilities|GetClass OtherActor) "/Game/Jacob/Push/BP_PushAndDragObject_Stone.BP_PushAndDragObject_Stone_C")
    (|CanEndOverlap)))

(event EventBeginPlay
  (|CallParentFunction))

(event Collision|EventActorBeginOverlap
  (params (OtherActor :type Actor%20Object%20Reference)))

(event EventTick
  (params (DeltaSeconds :type Float%20%28single-precision%29))
  (|CallParentFunction DeltaSeconds))

(fn ConstructionScript
  (|CallParentFunction))