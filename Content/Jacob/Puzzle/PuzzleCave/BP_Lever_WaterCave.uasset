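; A water cave puzzle lever that, on interaction, toggles its linked water wall through SwitchActivatedWallWaterCave.
; While unpressed, SetInteractableState shows or hides the HUD lever prompt and swaps the lever material between arrows and red.
; Interact clears LeverIsNotPressed, freezing those updates, then a timeline rolls the lever with red material and prompt hidden.
; A DoOnce blocks re-triggering until the timeline finishes.
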(event EventBeginPlay)

(event EventTick
  (params (DeltaSeconds :type Float%20%28single-precision%29)))

(event EventSetInteractableState
  (params (bCanShowInteract :type Boolean))
  (bind _lever (Variables|Default|GetLever))
  ;[1 1 1] Set Interactable State
  (if (Variables|Default|GetLeverIsNotPressed)
    (bind _output_get (Variables|Default|SetbCanInteract? bCanShowInteract))
    (if _output_get
      (CallFunction|TextEnable)
      (Rendering|Material|SetMaterial _lever 0 "/Game/StarterContent/Blueprints/Assets/M_LightStage_Arrows.M_LightStage_Arrows")
      (else
        (CallFunction|TextDisable)
        (Rendering|Material|SetMaterial _lever 0 "/Game/Materials/M_Red.M_Red")))))

(event EventInteract
  (params (Instigator :type Actor%20Object%20Reference))
  ;[1 1 1] Lever Trigger
  (Utilities|FlowControl|DoOnce false :!label _label
    (:Completed
      (Variables|Default|SetLeverIsNotPressed false)
      (Default|SwitchActivatedWallWaterCave (Variables|Default|GetWallWaterToActivate))
      (bind _switchposition (Timeline|Timeline Play)
        (:Update
          (Rendering|Material|SetMaterial (Variables|Default|GetLever) 0 "/Game/Materials/M_Red.M_Red")
          (CallFunction|TextDisable)
          (Transformation|SetRelativeRotation (Variables|Default|GetLever) (Math|Rotator|MakeRotator _switchposition 0.0 0.0) false false))
        (:Finished
          (if (Variables|Default|GetbCanInteract?)
            (Rendering|Material|SetMaterial (Variables|Default|GetLever) 0 "/Game/Materials/M_Red.M_Red")
            (goto _label Reset)
            (else
              (goto _label Reset))))))))

(fn ConstructionScript)

(fn ComponentIsChild
  (params (Component :type Actor%20Object%20Reference%20%28by%20ref%29))
  (return (== (Actor|GetParentActor Component) self)))

(fn TextEnable
  (bind _asnew_hud (Utilities|Casting|CastToNewHUD (HUD|GetHUD (Game|GetPlayerController 0))))
  (bind _output_get (Variables|Default|SetAs%20New%20HUD _asnew_hud))
  (Default|LeverLock (Variables|/Game/Jacob/UI/NewHUD.NewHUD_C|GetUIRef _output_get) true))

(fn TextDisable
  (bind _as_new_hud (Variables|Default|GetAs%20New%20HUD)
    (:then
      (Default|LeverLock (Variables|/Game/Jacob/UI/NewHUD.NewHUD_C|GetUIRef _as_new_hud) false))
    (:else)))