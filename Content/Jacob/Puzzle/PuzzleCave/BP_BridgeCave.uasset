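; BP_BridgeCave is a cave puzzle bridge that rotates into place when enough pressure switches are active.
; Switch activation and deactivation events adjust a counter, then compare it to the required count to set ReadyToEnter.
; The BridgeActivate timeline plays or reverses to drive the bridge's roll.
; Its update disables the blocking collider after a short delay when ready, and re-enables it otherwise.
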(event Custom|SwitchActivatedBridgeCave
  ;[1 1 1] Bridge Activation
  (Math|Integer|IncrementInt (Variables|Default|GetPressureSwitchesActiveBridge)
    (:%20%20
      (if (>= (Variables|Default|GetPressureSwitchesActiveBridge) (Variables|Default|GetPressureSwitchesNeededBridge))
        (Variables|Default|SetReadyToEnter true)
        (bind _rotation (Timeline|BridgeActivate Play)
          (:Update
            (Transformation|SetRelativeRotation (Variables|Default|GetBridge) (Math|Rotator|MakeRotator _rotation 0.0 0.0) false false)
            (if (Variables|Default|GetReadyToEnter)
              (Utilities|FlowControl|Delay 1.5)
              (Collision|SetCollisionEnabled (Variables|Default|GetCollider) "NoCollision")
              (else
                (Collision|SetCollisionEnabled (Variables|Default|GetCollider) "QueryAndPhysics")))))
        (else
          (Variables|Default|SetReadyToEnter false)
          (if (Variables|Default|GetReadyToEnter)
            (Timeline|BridgeActivate Play)
            (else
              (Timeline|BridgeActivate Reverse))))))))

(event Custom|SwitchDeactivatedBridgeCave
  ;[1 1 1] Bridge Activation
  (Math|Integer|DecrementInt (Variables|Default|GetPressureSwitchesActiveBridge)
    (:%20%20
      (if (>= (Variables|Default|GetPressureSwitchesActiveBridge) (Variables|Default|GetPressureSwitchesNeededBridge))
        (Variables|Default|SetReadyToEnter true)
        (bind _rotation (Timeline|BridgeActivate Play)
          (:Update
            (Transformation|SetRelativeRotation (Variables|Default|GetBridge) (Math|Rotator|MakeRotator _rotation 0.0 0.0) false false)
            (if (Variables|Default|GetReadyToEnter)
              (Utilities|FlowControl|Delay 1.5)
              (Collision|SetCollisionEnabled (Variables|Default|GetCollider) "NoCollision")
              (else
                (Collision|SetCollisionEnabled (Variables|Default|GetCollider) "QueryAndPhysics")))))
        (else
          (Variables|Default|SetReadyToEnter false)
          (if (Variables|Default|GetReadyToEnter)
            (Timeline|BridgeActivate Play)
            (else
              (Timeline|BridgeActivate Reverse))))))))

(event EventBeginPlay)

(event Collision|EventActorBeginOverlap
  (params (OtherActor :type Actor%20Object%20Reference)))

(event EventTick
  (params (DeltaSeconds :type Float%20%28single-precision%29)))

(fn ConstructionScript)