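; Puzzle actor that counts active pressure switches and stops physics simulation on its Door component.
; Activation and deactivation events raise and lower the switch count.
; When an activation brings the count to the required number, a 12-second delay runs before physics is switched off.
; Deactivation never restores physics, as its threshold check leads to no action.
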(event Custom|RollingStoneActivatedDoorWithPhysics
  ;[1 1 1] Door Activation/Deactivation
  (Math|Integer|IncrementInt (Variables|Default|GetPressureSwitchesActive)
    (:%20%20
      (if (>= (Variables|Default|GetPressureSwitchesActive) (Variables|Default|GetPressureSwitchesNeeded))
        (Utilities|FlowControl|Delay 12.0)
        (Physics|SetSimulatePhysics (Variables|Default|GetDoor) false)))))

(event Custom|RollingStoneDeactivatedDoorWithPhysics
  ;[1 1 1] Door Activation/Deactivation
  (Math|Integer|DecrementInt (Variables|Default|GetPressureSwitchesActive)
    (:%20%20
      (if (>= (Variables|Default|GetPressureSwitchesActive) (Variables|Default|GetPressureSwitchesNeeded))
        _))))

(event EventBeginPlay)

(event Collision|EventActorBeginOverlap
  (params (OtherActor :type Actor%20Object%20Reference)))

(event EventTick
  (params (DeltaSeconds :type Float%20%28single-precision%29)))

(fn ConstructionScript)