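; BP_DoorWithPhysics is a puzzle door that is released into physics simulation once enough switch activations are received.
; Each LeverActivatedDoorWithPhysics call increments a counter and compares it to the required switch count.
; At or above that threshold, the Door component simulates physics for a fixed delay, then has simulation switched off again.
; The counter only increases, with no decrement or reset in this Blueprint.
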(event Custom|LeverActivatedDoorWithPhysics
  ;[1 1 1] Door Activation/Deactivation
  (Math|Integer|IncrementInt (Variables|Default|GetPressureSwitchesActive)
    (:%20%20
      (if (>= (Variables|Default|GetPressureSwitchesActive) (Variables|Default|GetPressureSwitchesNeeded))
        (Physics|SetSimulatePhysics (Variables|Default|GetDoor) true)
        (Utilities|FlowControl|Delay 7.0)
        (Physics|SetSimulatePhysics (Variables|Default|GetDoor) false)))))

(event EventBeginPlay)

(event Collision|EventActorBeginOverlap
  (params (OtherActor :type Actor%20Object%20Reference)))

(event EventTick
  (params (DeltaSeconds :type Float%20%28single-precision%29)))

(fn ConstructionScript)