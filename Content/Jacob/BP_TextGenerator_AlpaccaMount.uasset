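; BP_TextGenerator_AlpaccaMount is a trigger actor that signals the player's UI about the Alpacca Mount zone.
; When BP_PlayerJacob or any NPC_Base subclass enters its Box, it casts player 0's HUD to NewHUD and calls AlpaccaMountZone(true) on its UIRef, if valid.
; End overlap is empty, so this Blueprint never sends false on exit.
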(event OnComponentBeginOverlap(Box)
  (params (OverlappedComponent :type Primitive%20Component%20Object%20Reference) (OtherActor :type Actor%20Object%20Reference) (OtherComp :type Primitive%20Component%20Object%20Reference) (OtherBodyIndex :type Integer) (bFromSweep :type Boolean) (SweepResult :type Hit%20Result%20Structure%20%28by%20ref%29))
  (bind _returnvalue (Utilities|GetClass OtherActor))
  (if (or (Utilities|ClassIsChildOf _returnvalue "/Game/ThirdPerson/Blueprints/BP_PlayerJacob.BP_PlayerJacob_C") (Utilities|ClassIsChildOf _returnvalue "/Game/Marcus/NPC/NPCs/NPC_Base.NPC_Base_C"))
    (bind _asnew_hud (Utilities|Casting|CastToNewHUD (HUD|GetHUD (Game|GetPlayerController 0))))
    (bind _output_get (Variables|Default|SetAs%20New%20HUD _asnew_hud))
    (bind _uiref (Variables|/Game/Jacob/NewHUD.NewHUD_C|GetUIRef _output_get)
      (:then
        (Default|AlpaccaMountZone _uiref true))
      (:else))))

(event OnComponentEndOverlap(Box)
  (params (OverlappedComponent :type Primitive%20Component%20Object%20Reference) (OtherActor :type Actor%20Object%20Reference) (OtherComp :type Primitive%20Component%20Object%20Reference) (OtherBodyIndex :type Integer)))

(event EventBeginPlay
  (|CallParentFunction))

(event Collision|EventActorBeginOverlap
  (params (OtherActor :type Actor%20Object%20Reference))
  (|CallParentFunction OtherActor) ; This node is disabled and will not be called.\nDrag off pins to build functionality.
)

(event EventTick
  (params (DeltaSeconds :type Float%20%28single-precision%29))
  (|CallParentFunction 0.0))

(fn ConstructionScript
  (|CallParentFunction))