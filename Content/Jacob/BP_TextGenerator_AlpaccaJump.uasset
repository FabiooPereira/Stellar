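; BP_TextGenerator_AlpaccaJump is a trigger actor that toggles the alpaca jump text on the HUD.
; When a BP_Player_Mounted actor begins overlapping its Box, TextEnable casts player 0's HUD to NewHUD, stores it and turns the text on through UIRef.
; Any end overlap, regardless of actor class, calls TextDisable, which turns the text off if the stored HUD reference is valid.
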(event OnComponentBeginOverlap(Box)
  (params (OverlappedComponent :type Primitive%20Component%20Object%20Reference) (OtherActor :type Actor%20Object%20Reference) (OtherComp :type Primitive%20Component%20Object%20Reference) (OtherBodyIndex :type Integer) (bFromSweep :type Boolean) (SweepResult :type Hit%20Result%20Structure%20%28by%20ref%29))
  (if (Utilities|ClassIsChildOf (Utilities|GetClass OtherActor) "/Game/ThirdPerson/Blueprints/BP_Player_Mounted.BP_Player_Mounted_C")
    (CallFunction|TextEnable)))

(event OnComponentEndOverlap(Box)
  (params (OverlappedComponent :type Primitive%20Component%20Object%20Reference) (OtherActor :type Actor%20Object%20Reference) (OtherComp :type Primitive%20Component%20Object%20Reference) (OtherBodyIndex :type Integer))
  (CallFunction|TextDisable))

(event EventBeginPlay
  (|CallParentFunction))

(event Collision|EventActorBeginOverlap
  (params (OtherActor :type Actor%20Object%20Reference))
  (|CallParentFunction OtherActor) ; This node is disabled and will not be called.\nDrag off pins to build functionality.
)

(event EventTick
  (params (DeltaSeconds :type Float%20%28single-precision%29))
  (|CallParentFunction 0.0))

(fn ConstructionScript
  (|CallParentFunction))

(fn TextDisable
  (bind _as_new_hud (Variables|Default|GetAs%20New%20HUD)
    (:then
      (Default|AlpaccaJumpText (Variables|/Game/Jacob/NewHUD.NewHUD_C|GetUIRef _as_new_hud) false))
    (:else)))

(fn TextEnable
  (bind _asnew_hud (Utilities|Casting|CastToNewHUD (HUD|GetHUD (Game|GetPlayerController 0))))
  (bind _output_get (Variables|Default|SetAs%20New%20HUD _asnew_hud))
  (Default|AlpaccaJumpText (Variables|/Game/Jacob/NewHUD.NewHUD_C|GetUIRef _output_get) true))