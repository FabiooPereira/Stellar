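; BP_Killzone is a trigger volume that respawns the player by reloading their saved game.
; When a BP_ThirdPersonCharacter overlaps the Killzone component, it calls LoadGame on that character.
; It then shows respawn text through the NewHUD's UI reference, caching the HUD, and hides the text after a short delay.
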(event OnComponentBeginOverlap(Killzone)
  (params (OverlappedComponent :type Primitive%20Component%20Object%20Reference) (OtherActor :type Actor%20Object%20Reference) (OtherComp :type Primitive%20Component%20Object%20Reference) (OtherBodyIndex :type Integer) (bFromSweep :type Boolean) (SweepResult :type Hit%20Result%20Structure%20%28by%20ref%29))
  (bind _asbp_third_person_character (Utilities|Casting|CastToBP_ThirdPersonCharacter OtherActor))
  (Default|LoadGame _asbp_third_person_character)
  (CallFunction|TextEnable)
  (Utilities|FlowControl|Delay 2.0)
  (CallFunction|TextDisable))

(event EventBeginPlay)

(event Collision|EventActorBeginOverlap
  (params (OtherActor :type Actor%20Object%20Reference)))

(event EventTick
  (params (DeltaSeconds :type Float%20%28single-precision%29)))

(fn ConstructionScript)

(fn TextEnable
  (bind _asnew_hud (Utilities|Casting|CastToNewHUD (HUD|GetHUD (Game|GetPlayerController 0))))
  (bind _output_get (Variables|Default|SetAs%20New%20HUD _asnew_hud))
  (Default|RespawnText (Variables|/Game/Jacob/NewHUD.NewHUD_C|GetUIRef _output_get) true))

(fn TextDisable
  (bind _as_new_hud (Variables|Default|GetAs%20New%20HUD)
    (:then
      (Default|RespawnText (Variables|/Game/Jacob/NewHUD.NewHUD_C|GetUIRef _as_new_hud) false))
    (:else)))