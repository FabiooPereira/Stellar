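; BP_SaveZone is a trigger actor that saves the game when the BP_PlayerJacob player enters it.
; Overlapping its SpawnPosition component shows "GAME SAVED" through NewHUD and calls SaveGame on BP_MyInstance with slot name "SAVE 1".
; A DoOnce limits repeat saves and resets when any overlap ends.
; TextDisable can clear the message but is not called within this Blueprint.
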(event OnComponentBeginOverlap(SpawnPosition)
  (params (OverlappedComponent :type Primitive%20Component%20Object%20Reference) (OtherActor :type Actor%20Object%20Reference) (OtherComp :type Primitive%20Component%20Object%20Reference) (OtherBodyIndex :type Integer) (bFromSweep :type Boolean) (SweepResult :type Hit%20Result%20Structure%20%28by%20ref%29))
  ;[1 1 1] Overlap Begin/End
  (if (Utilities|ClassIsChildOf (Utilities|GetClass OtherActor) "/Game/ThirdPerson/Blueprints/BP_PlayerJacob.BP_PlayerJacob_C")
    (Utilities|FlowControl|DoOnce false
      (:Completed
        (CallFunction|TextEnable)
        (bind _asbp_my_instance (Utilities|Casting|CastToBP_MyInstance (Game|GetGameInstance)))
        (Default|SaveGame _asbp_my_instance "SAVE 1")))))

(event OnComponentEndOverlap(SpawnPosition)
  (params (OverlappedComponent :type Primitive%20Component%20Object%20Reference) (OtherActor :type Actor%20Object%20Reference) (OtherComp :type Primitive%20Component%20Object%20Reference) (OtherBodyIndex :type Integer))
  ;[1 1 1] Overlap Begin/End
  (Utilities|FlowControl|DoOnce false) ; enters at Reset
)

(event EventBeginPlay)

(event Collision|EventActorBeginOverlap
  (params (OtherActor :type Actor%20Object%20Reference)))

(event EventTick
  (params (DeltaSeconds :type Float%20%28single-precision%29)))

(fn ConstructionScript)

(fn TextDisable
  (bind _as_new_hud (Variables|Default|GetAs%20New%20HUD)
    (:then
      (Default|SetTextSaveLoad (Variables|/Game/Jacob/UI/NewHUD.NewHUD_C|GetUIRef _as_new_hud) "" "" false))
    (:else)))

(fn TextEnable
  (bind _asnew_hud (Utilities|Casting|CastToNewHUD (HUD|GetHUD (Game|GetPlayerController 0))))
  (bind _output_get (Variables|Default|SetAs%20New%20HUD _asnew_hud))
  (Default|SetTextSaveLoad (Variables|/Game/Jacob/UI/NewHUD.NewHUD_C|GetUIRef _output_get) "GAME SAVED" "GAME SAVED" true))