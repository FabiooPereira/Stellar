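; Game instance that saves and loads game progress by slot, plus restart (reload) and save-and-quit to main menu.
; Per-category helpers with an IsSaving flag copy transforms and state for player, alpaca, puzzle objects, lamps, NPCs and customization to or from BP_Save.
; Loading caches saved values, opens the level, then applies them next tick.
; Actor arrays match by index; only lamps are first sorted by distance from world origin.
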(event Custom|RestartGame
  ;[1 1 1] Restart Game
  (CallFunction|LoadGame (Variables|Default|GetSlot%20Name)))

(event Custom|LoadGame
  (params (SlotName :type String))
  ;[1 1 1] Load Game
  (bind _output_get (Variables|Default|SetSlot%20Name SlotName))
  (bind _returnvalue (SaveGame|DoesSaveGameExist _output_get))
  (if _returnvalue
    (bind _returnvalue_2 (SaveGame|LoadGamefromSlot (Variables|Default|GetSlot%20Name)))
    (bind _asbp_save (Utilities|Casting|CastToBP_Save _returnvalue_2))
    (Utilities|FlowControl|Sequence
      (:then_0
        (Game|OpenLevel(byName) (Utilities|String|StringToName (Variables|/Game/Jacob/SaveAndLoad/BP_Save.BP_Save_C|GetLevel _asbp_save)))
        (CallFunction|SetVariables _asbp_save))
      (:then_1
        (Utilities|FlowControl|DelayUntilNextTick)
        (CallFunction|PlayerPosition 0 false)
        (CallFunction|AlpacaPosition 0 false)
        (CallFunction|CrystalsPosition 0 false)
        (CallFunction|StonesPosition 0 false)
        (CallFunction|PillarsPosition 0 false)
        (CallFunction|FoxesPosition 0 false))
      (:then_2
        (Utilities|FlowControl|DelayUntilNextTick)
        (Game|Player|SetViewTargetwithBlend (Game|GetPlayerController 0) (Game|GetPlayerCharacter 0) 0.0 "VTBlend_Linear" 0.0 false))
      (:then_3
        (Utilities|FlowControl|DelayUntilNextTick)
        (CallFunction|ObjecttoTriggerVariables 0 false)
        (CallFunction|PlayerVariables 0 false)
        (CallFunction|LampVariables 0 false)
        (CallFunction|NPCVariables 0 false)
        (CallFunction|LeverVariables 0 false)
        (CallFunction|PlayerCustomizationVariables false))
      (:then_4
        (Utilities|FlowControl|DelayUntilNextTick)
        (CallFunction|TextEnableLoad)))
    (else
      (Game|OpenLevel(byName) "HubLevel"))))

(event Custom|SaveGame
  (params (SlotName :type String))
  ;[1 1 1] Save Game
  (bind _output_get (Variables|Default|SetSlot%20Name SlotName))
  (bind _returnvalue (SaveGame|DoesSaveGameExist _output_get))
  (if _returnvalue
    (bind _returnvalue_2 (SaveGame|LoadGamefromSlot (Variables|Default|GetSlot%20Name)))
    (bind _asbp_save (Utilities|Casting|CastToBP_Save _returnvalue_2))
    (Utilities|FlowControl|Sequence
      (:then_0
        (bind _returnvalue_3 (Game|GetCurrentLevelName true))
        (Variables|/Game/Jacob/SaveAndLoad/BP_Save.BP_Save_C|SetLevel _asbp_save _returnvalue_3))
      (:then_1
        (CallFunction|PlayerPosition _asbp_save true)
        (CallFunction|AlpacaPosition _asbp_save true)
        (CallFunction|CrystalsPosition _asbp_save true)
        (CallFunction|FoxesPosition _asbp_save true)
        (CallFunction|StonesPosition _asbp_save true)
        (CallFunction|PillarsPosition _asbp_save true)
        (CallFunction|ObjecttoTriggerVariables _asbp_save true)
        (CallFunction|PlayerVariables _asbp_save true)
        (CallFunction|LampVariables _asbp_save true)
        (CallFunction|NPCVariables _asbp_save true)
        (CallFunction|LeverVariables _asbp_save true)
        (CallFunction|PlayerCustomizationVariables true _asbp_save))
      (:then_2
        (SaveGame|SaveGametoSlot _asbp_save (Variables|Default|GetSlot%20Name))))
    (else
      (bind _returnvalue_4 (SaveGame|CreateSaveGameObject "/Game/Jacob/SaveAndLoad/BP_Save.BP_Save_C"))
      (Utilities|FlowControl|Sequence
        (:then_0
          (bind _returnvalue_5 (Game|GetCurrentLevelName true))
          (Variables|/Game/Jacob/SaveAndLoad/BP_Save.BP_Save_C|SetLevel _returnvalue_4 _returnvalue_5))
        (:then_1
          (CallFunction|PlayerPosition _returnvalue_4 true)
          (CallFunction|AlpacaPosition _returnvalue_4 true)
          (CallFunction|CrystalsPosition _returnvalue_4 true)
          (CallFunction|FoxesPosition _returnvalue_4 true)
          (CallFunction|StonesPosition _returnvalue_4 true)
          (CallFunction|PillarsPosition _returnvalue_4 true)
          (CallFunction|ObjecttoTriggerVariables _returnvalue_4 true)
          (CallFunction|PlayerVariables _returnvalue_4 true)
          (CallFunction|LampVariables _returnvalue_4 true)
          (CallFunction|NPCVariables _returnvalue_4 true)
          (CallFunction|LeverVariables _returnvalue_4 true)
          (CallFunction|PlayerCustomizationVariables true _returnvalue_4))
        (:then_2
          (SaveGame|SaveGametoSlot _returnvalue_4 (Variables|Default|GetSlot%20Name)))))))

(event Custom|QuitToMainMenu
  ;[1 1 1] Quit
  (CallFunction|SaveGame (Variables|Default|GetSlot%20Name))
  (Game|OpenLevel(byName) "MainMenu"))

(event Custom|IsValid
  (bind _returnvalue (Actor|GetActorOfClass "/Game/ThirdPerson/Blueprints/BP_PlayerJacob.BP_PlayerJacob_C"))
  (Utilities|IsValid _returnvalue
    (:Is%20Valid
      (Utilities|Time|ClearandInvalidateTimerbyHandle (Variables|Default|GetTimer))
      (Development|PrintString (Utilities|GetObjectName 0))
      (Development|PrintString "Is Valid" true true "(R=0.035727,G=1.000000,B=0.000000,A=1.000000)" 5.0))
    (:Is%20Not%20Valid
      (Development|PrintString "Is Not Valid" true true "(R=1.000000,G=0.113503,B=0.000000,A=1.000000)" 5.0))))

(fn GetAllActorsinOrder
  (params (Array :type Array%20of%20Actor%20Object%20References))
  (bind _output_get (LocalVariables|SetActorRefs Array))
  (LocalVariables|SetAscending false)
  (for (_array_element _array_index) _output_get
    (for _index (range _array_index (Utilities|Array|LastIndex (Utilities|Array|MakeArray (Utilities|GetDisplayName (Utilities|Array|Get(acopy) (LocalVariables|GetActorRefs))))))
      (bind _index_2 (Utilities|FlowControl|ForLoopwithBreak 0 (- (select (> (Utilities|String|Len (Utilities|Array|Get(acopy) (Utilities|Array|MakeArray (Utilities|GetDisplayName (Utilities|Array|Get(acopy) (LocalVariables|GetActorRefs)))) _index)) (Utilities|String|Len (Utilities|GetDisplayName _array_element))) (Utilities|String|Len (Utilities|GetDisplayName _array_element)) (Utilities|String|Len (Utilities|Array|Get(acopy) (Utilities|Array|MakeArray (Utilities|GetDisplayName (Utilities|Array|Get(acopy) (LocalVariables|GetActorRefs)))) _index))) 1) :!label _label)
        (:LoopBody
          (if (!= (Utilities|String|GetCharacterasNumber (Utilities|Array|Get(acopy) (Utilities|Array|MakeArray (Utilities|GetDisplayName (Utilities|Array|Get(acopy) (LocalVariables|GetActorRefs)))) _index) _index_2) (Utilities|String|GetCharacterasNumber (Utilities|GetDisplayName _array_element) _index_2))
            (goto _label Break)))
        (:Completed
          (if (LocalVariables|GetAscending)
            (if (> (Utilities|String|GetCharacterasNumber (Utilities|Array|Get(acopy) (Utilities|Array|MakeArray (Utilities|GetDisplayName (Utilities|Array|Get(acopy) (LocalVariables|GetActorRefs)))) _index) _index_2) (Utilities|String|GetCharacterasNumber (Utilities|GetDisplayName _array_element) _index_2))
              (Utilities|Array|Swap (Utilities|Array|MakeArray (Utilities|GetDisplayName (Utilities|Array|Get(acopy) (LocalVariables|GetActorRefs)))) _index _array_index :!label _label_2))
            (elif (< (Utilities|String|GetCharacterasNumber (Utilities|Array|Get(acopy) (Utilities|Array|MakeArray (Utilities|GetDisplayName (Utilities|Array|Get(acopy) (LocalVariables|GetActorRefs)))) _index) _index_2) (Utilities|String|GetCharacterasNumber (Utilities|GetDisplayName _array_element) _index_2))
              (goto _label_2)))))))
  (return (LocalVariables|GetActorRefs)))

(fn GetAllActorsinOrderWorking
  (params (Array :type Array%20of%20Actor%20Object%20References))
  (bind _distances (LocalVariables|GetDistances))
  (bind _indexofminvalue (Math|Float|MinOfFloatArray _distances))
  (bind _output_get (LocalVariables|SetActorRefs Array))
  (for _array_element _output_get
    (Utilities|Array|Add (LocalVariables|GetDistances) (Math|Vector|VectorLength (Transformation|GetActorLocation _array_element))))
  (if (> (Utilities|Array|Length (LocalVariables|GetDistances)) 0) :!label _label
    (Utilities|Array|Add (LocalVariables|GetOrderedActorRefs) (Utilities|Array|Get(acopy) (LocalVariables|GetActorRefs) _indexofminvalue))
    (Utilities|Array|RemoveIndex (LocalVariables|GetActorRefs) _indexofminvalue)
    (Utilities|Array|RemoveIndex (LocalVariables|GetDistances) _indexofminvalue)
    (goto _label)
    (else
      (return (LocalVariables|GetOrderedActorRefs)))))

(fn GetSortedActors
  (params (ArrayToSort :type Array%20of%20Actor%20Object%20References))
  (Variables|Default|SetArray%20to%20Sort ArrayToSort)
  (CallFunction|AlpacaPosition 0 false)
  (bind _outactors (Actor|GetAllActorsOfClass "/Game/Jacob/Grab/BP_AttachedObjectPickup_Crystal.BP_AttachedObjectPickup_Crystal_C"))
  (for _array_element _outactors
    (Utilities|Array|Add (Variables|Default|GetArray%20to%20Sort) _array_element))
  (bind _outactors_2 (Actor|GetAllActorsOfClass "/Game/Jacob/Push/BP_PushAndDragObject_Pillar.BP_PushAndDragObject_Pillar_C"))
  (for _array_element_2 _outactors_2
    (Utilities|Array|Add (Variables|Default|GetArray%20to%20Sort) _array_element_2))
  (bind _outactors_3 (Actor|GetAllActorsOfClass "/Game/Jacob/Push/BP_PushAndDragObject_Stone.BP_PushAndDragObject_Stone_C"))
  (for _array_element_3 _outactors_3
    (Utilities|Array|Add (Variables|Default|GetArray%20to%20Sort) _array_element_3))
  (bind _outactors_4 (Actor|GetAllActorsOfClass "/Game/Jacob/Objects/Other/BP_Cube.BP_Cube_C"))
  (for _array_element_4 _outactors_4
    (Utilities|Array|Add (Variables|Default|GetArray%20to%20Sort) 0))
  (return (Variables|Default|GetArray%20to%20Sort)))

(fn IsValidTimer
  (if (not (Utilities|Time|IsTimerActivebyHandle (Variables|Default|GetTimer)))
    (bind _returnvalue (Utilities|Time|SetTimerbyEvent (EventDispatchers|CreateEvent :!event Custom|IsValid) 0.3 true))
    (Variables|Default|SetTimer _returnvalue)))

(fn TextEnableSave
  (bind _asnew_hud (Utilities|Casting|CastToNewHUD (HUD|GetHUD (Game|GetPlayerController 0))))
  (bind _output_get (Variables|Default|SetAs%20New%20HUD _asnew_hud))
  (Default|SetTextSaveLoad (Variables|/Game/Jacob/UI/NewHUD.NewHUD_C|GetUIRef _output_get) "GAME SAVED" "GAME SAVED" true))

(fn TextEnableLoad
  (bind _asnew_hud (Utilities|Casting|CastToNewHUD (HUD|GetHUD (Game|GetPlayerController 0))))
  (bind _output_get (Variables|Default|SetAs%20New%20HUD _asnew_hud))
  (Default|SetTextSaveLoad (Variables|/Game/Jacob/UI/NewHUD.NewHUD_C|GetUIRef _output_get) "GAME LOADED" "GAME LOADED" true))

(fn AlpacaPosition
  (params (BP_Save :type BP%20Save%20Object%20Reference) (IsSaving :type Boolean))
  (bind _returnvalue (Actor|GetActorOfClass "/Game/AICompanion/AI_Alan.AI_Alan_C"))
  (if IsSaving
    (Variables|/Game/Jacob/SaveAndLoad/BP_Save.BP_Save_C|SetAlpacaPos BP_Save (Transformation|GetActorTransform _returnvalue))
    (else
      (Transformation|SetActorTransform _returnvalue (Variables|Default|GetAlpacaPos))))
  (return))

(fn PlayerPosition
  (params (BP_Save :type BP%20Save%20Object%20Reference) (IsSaving :type Boolean))
  (if IsSaving
    (Variables|/Game/Jacob/SaveAndLoad/BP_Save.BP_Save_C|SetPlayerPos BP_Save (Transformation|GetActorTransform (Game|GetPlayerCharacter 0)))
    (else
      (Transformation|SetActorTransform (Game|GetPlayerCharacter 0) (Variables|Default|GetPlayerPos))))
  (return))

(fn CrystalsPosition
  (params (BP_Save :type BP%20Save%20Object%20Reference) (IsSaving :type Boolean))
  (if IsSaving
    (Utilities|Array|Clear (Variables|/Game/Jacob/SaveAndLoad/BP_Save.BP_Save_C|GetCrystalsPos BP_Save))
    (bind _outactors (Actor|GetAllActorsOfClass "/Game/Jacob/Grab/BP_AttachedObjectPickup_Crystal.BP_AttachedObjectPickup_Crystal_C"))
    (for (_array_element _array_index) _outactors
      (Utilities|Array|SetArrayElem (Variables|/Game/Jacob/SaveAndLoad/BP_Save.BP_Save_C|GetCrystalsPos BP_Save) _array_index (Transformation|GetActorTransform _array_element) true))
    (else
      (bind _outactors_2 (Actor|GetAllActorsOfClass "/Game/Jacob/Grab/BP_AttachedObjectPickup_Crystal.BP_AttachedObjectPickup_Crystal_C"))
      (for (_array_element_2 _array_index_2) _outactors_2
        (Transformation|SetActorTransform _array_element_2 (Utilities|Array|Get(acopy) (Variables|Default|GetCrystalsPos) _array_index_2)))))
  (return))

(fn FoxesPosition
  (params (BP_Save :type BP%20Save%20Object%20Reference) (IsSaving :type Boolean))
  (if IsSaving
    (Utilities|Array|Clear (Variables|/Game/Jacob/SaveAndLoad/BP_Save.BP_Save_C|GetFoxesPos BP_Save))
    (bind _outactors (Actor|GetAllActorsOfClass "/Game/Jacob/Objects/Other/BP_Cube.BP_Cube_C"))
    (for (_array_element _array_index) _outactors
      (Utilities|Array|SetArrayElem (Variables|/Game/Jacob/SaveAndLoad/BP_Save.BP_Save_C|GetFoxesPos BP_Save) _array_index (Transformation|GetActorTransform _array_element) true))
    (else
      (bind _outactors_2 (Actor|GetAllActorsOfClass "/Game/Jacob/Objects/Other/BP_Cube.BP_Cube_C"))
      (for (_array_element_2 _array_index_2) _outactors_2
        (Transformation|SetActorTransform _array_element_2 (Utilities|Array|Get(acopy) (Variables|Default|GetFoxesPos) _array_index_2)))))
  (return))

(fn StonesPosition
  (params (BP_Save :type BP%20Save%20Object%20Reference) (IsSaving :type Boolean))
  (if IsSaving
    (Utilities|Array|Clear (Variables|/Game/Jacob/SaveAndLoad/BP_Save.BP_Save_C|GetStonesPos BP_Save))
    (bind _outactors (Actor|GetAllActorsOfClass "/Game/Jacob/Push/BP_PushAndDragObject_Stone.BP_PushAndDragObject_Stone_C"))
    (for (_array_element _array_index) _outactors
      (Utilities|Array|SetArrayElem (Variables|/Game/Jacob/SaveAndLoad/BP_Save.BP_Save_C|GetStonesPos BP_Save) _array_index (Transformation|GetActorTransform _array_element) true))
    (else
      (bind _outactors_2 (Actor|GetAllActorsOfClass "/Game/Jacob/Push/BP_PushAndDragObject_Stone.BP_PushAndDragObject_Stone_C"))
      (for (_array_element_2 _array_index_2) _outactors_2
        (Transformation|SetActorTransform _array_element_2 (Utilities|Array|Get(acopy) (Variables|Default|GetStonesPos) _array_index_2)))))
  (return))

(fn PillarsPosition
  (params (BP_Save :type BP%20Save%20Object%20Reference) (IsSaving :type Boolean))
  (if IsSaving
    (Utilities|Array|Clear (Variables|/Game/Jacob/SaveAndLoad/BP_Save.BP_Save_C|GetPillarsPos BP_Save))
    (bind _outactors (Actor|GetAllActorsOfClass "/Game/Jacob/Push/BP_PushAndDragObject_Pillar.BP_PushAndDragObject_Pillar_C"))
    (for (_array_element _array_index) _outactors
      (Utilities|Array|SetArrayElem (Variables|/Game/Jacob/SaveAndLoad/BP_Save.BP_Save_C|GetPillarsPos BP_Save) _array_index (Transformation|GetActorTransform _array_element) true))
    (return)
    (else
      (bind _outactors_2 (Actor|GetAllActorsOfClass "/Game/Jacob/Push/BP_PushAndDragObject_Pillar.BP_PushAndDragObject_Pillar_C"))
      (for (_array_element_2 _array_index_2) _outactors_2
        (Transformation|SetActorTransform _array_element_2 (Utilities|Array|Get(acopy) (Variables|Default|GetPillarsPos) _array_index_2))
        (return)))))

(fn PlayerVariables
  (params (BP_Save :type BP%20Save%20Object%20Reference) (IsSaving :type Boolean))
  (bind _asbp_player_jacob (Utilities|Casting|CastToBP_PlayerJacob (Game|GetPlayerCharacter 0)))
  (if IsSaving
    (Variables|/Game/Jacob/SaveAndLoad/BP_Save.BP_Save_C|SetHasLight BP_Save (Variables|/Game/ThirdPerson/Blueprints/BP_PlayerJacob.BP_PlayerJacob_C|GetHasLight _asbp_player_jacob))
    (Variables|/Game/Jacob/SaveAndLoad/BP_Save.BP_Save_C|SetSpringArmLength BP_Save (Variables|/Script/Engine.SpringArmComponent|GetTargetArmLength (Actor|GetComponentbyClass _asbp_player_jacob "/Script/Engine.SpringArmComponent")))
    (bind _asbp_third_person_character (Utilities|Casting|CastToBP_ThirdPersonCharacter (Game|GetPlayerCharacter 0)))
    (Variables|/Game/Jacob/SaveAndLoad/BP_Save.BP_Save_C|SetEnableCallStay BP_Save (Variables|/Game/ThirdPerson/Blueprints/BP_ThirdPersonCharacter.BP_ThirdPersonCharacter_C|GetEnableCallStay _asbp_third_person_character))
    (else
      (Variables|/Game/ThirdPerson/Blueprints/BP_PlayerJacob.BP_PlayerJacob_C|SetHasLight _asbp_player_jacob (Variables|Default|GetHasLight))
      (Variables|/Script/Engine.SpringArmComponent|SetTargetArmLength (Actor|GetComponentbyClass _asbp_player_jacob "/Script/Engine.SpringArmComponent") (Variables|Default|GetSpringArmLength))
      (bind _asbp_third_person_character_2 (Utilities|Casting|CastToBP_ThirdPersonCharacter (Game|GetPlayerCharacter 0)))
      (Variables|/Game/ThirdPerson/Blueprints/BP_ThirdPersonCharacter.BP_ThirdPersonCharacter_C|SetEnableCallStay _asbp_third_person_character_2 (Variables|Default|GetEnableCallStay))
      (Variables|/Script/Engine.SpringArmComponent|SetbEnableCameraLag (Actor|GetComponentbyClass _asbp_player_jacob "/Script/Engine.SpringArmComponent") false)))
  (return))

(fn ObjecttoTriggerVariables
  (params (BP_Save :type BP%20Save%20Object%20Reference) (IsSaving :type Boolean))
  (if IsSaving
    (Utilities|Array|Clear (Variables|/Game/Jacob/SaveAndLoad/BP_Save.BP_Save_C|GetDoorPlayed BP_Save))
    (bind _outactors (Actor|GetAllActorsOfClass "/Game/Jacob/Objects/Doors/BP_ObjectToTrigger_WallBig.BP_ObjectToTrigger_WallBig_C"))
    (for (_array_element _array_index) _outactors
      (Utilities|Array|SetArrayElem (Variables|/Game/Jacob/SaveAndLoad/BP_Save.BP_Save_C|GetDoorPlayed BP_Save) _array_index (Variables|/Game/Jacob/BP_ObjectToTrigger_Parent.BP_ObjectToTrigger_Parent_C|GetPlayed _array_element) true)
      (Utilities|Array|SetArrayElem (Variables|/Game/Jacob/SaveAndLoad/BP_Save.BP_Save_C|GetTriggersActive BP_Save) _array_index (Variables|/Game/Jacob/BP_ObjectToTrigger_Parent.BP_ObjectToTrigger_Parent_C|GetTriggersActive _array_element) true))
    (else
      (bind _outactors_2 (Actor|GetAllActorsOfClass "/Game/Jacob/Objects/Doors/BP_ObjectToTrigger_WallBig.BP_ObjectToTrigger_WallBig_C"))
      (for (_array_element_2 _array_index_2) _outactors_2
        (Variables|/Game/Jacob/BP_ObjectToTrigger_Parent.BP_ObjectToTrigger_Parent_C|SetPlayed _array_element_2 (Utilities|Array|Get(acopy) (Variables|Default|GetDoorPlayed) _array_index_2))
        (Variables|/Game/Jacob/BP_ObjectToTrigger_Parent.BP_ObjectToTrigger_Parent_C|SetTriggersActive _array_element_2 (Utilities|Array|Get(acopy) (Variables|Default|GetTriggersActive) _array_index_2))
        (Development|PrintString (Utilities|String|ToString(Boolean) (Utilities|Array|Get(acopy) (Variables|Default|GetDoorPlayed) _array_index_2))))))
  (return))

(fn SetVariables
  (params (BP_Save :type BP%20Save%20Object%20Reference))
  (Variables|Default|SetPlayerPos (Variables|/Game/Jacob/SaveAndLoad/BP_Save.BP_Save_C|GetPlayerPos BP_Save))
  (Variables|Default|SetHasLight (Variables|/Game/Jacob/SaveAndLoad/BP_Save.BP_Save_C|GetHasLight BP_Save))
  (Variables|Default|SetSpringArmLength (Variables|/Game/Jacob/SaveAndLoad/BP_Save.BP_Save_C|GetSpringArmLength BP_Save))
  (Variables|Default|SetAlpacaPos (Variables|/Game/Jacob/SaveAndLoad/BP_Save.BP_Save_C|GetAlpacaPos BP_Save))
  (Variables|Default|SetTriggersActive (Variables|/Game/Jacob/SaveAndLoad/BP_Save.BP_Save_C|GetTriggersActive BP_Save))
  (Variables|Default|SetPuzzleFinished (Variables|/Game/Jacob/SaveAndLoad/BP_Save.BP_Save_C|GetPuzzleFinished BP_Save))
  (Variables|Default|SetCrystalsPos (Variables|/Game/Jacob/SaveAndLoad/BP_Save.BP_Save_C|GetCrystalsPos BP_Save))
  (Variables|Default|SetFoxesPos (Variables|/Game/Jacob/SaveAndLoad/BP_Save.BP_Save_C|GetFoxesPos BP_Save))
  (Variables|Default|SetStonesPos (Variables|/Game/Jacob/SaveAndLoad/BP_Save.BP_Save_C|GetStonesPos BP_Save))
  (Variables|Default|SetPillarsPos (Variables|/Game/Jacob/SaveAndLoad/BP_Save.BP_Save_C|GetPillarsPos BP_Save))
  (Variables|Default|SetSwitchActivated (Variables|/Game/Jacob/SaveAndLoad/BP_Save.BP_Save_C|GetSwitchActivated BP_Save))
  (Variables|Default|SetThemeIndex (Variables|/Game/Jacob/SaveAndLoad/BP_Save.BP_Save_C|GetThemeIndex BP_Save))
  (Variables|Default|SetDoorPlayed (Variables|/Game/Jacob/SaveAndLoad/BP_Save.BP_Save_C|GetDoorPlayed BP_Save))
  (Variables|Default|SetLampisLit (Variables|/Game/Jacob/SaveAndLoad/BP_Save.BP_Save_C|GetLampisLit BP_Save))
  (bind _output_get (Variables|Default|SetNPCStatus (Variables|/Game/Jacob/SaveAndLoad/BP_Save.BP_Save_C|GetNPCStatus BP_Save)))
  (Variables|Default|SetEnableCallStay (Variables|/Game/Jacob/SaveAndLoad/BP_Save.BP_Save_C|GetEnableCallStay BP_Save))
  (return))

(fn NPCVariables
  (params (BP_Save :type BP%20Save%20Object%20Reference) (IsSaving :type Boolean))
  (bind _npcstatus (Variables|/Game/Jacob/SaveAndLoad/BP_Save.BP_Save_C|GetNPCStatus BP_Save))
  (bind _npcstatus_2 (Variables|Default|GetNPCStatus))
  (bind _asstellar_game_state (Utilities|Casting|CastToStellar_GameState (Game|GetGameState)))
  (if IsSaving
    (Utilities|Array|SetArrayElem _npcstatus 0 (Class|StellarGameState|GetInteractionStatus _asstellar_game_state "Gunter") true)
    (Utilities|Array|SetArrayElem _npcstatus 1 (Class|StellarGameState|GetTreeIndex _asstellar_game_state "Gunter") true)
    (Utilities|Array|SetArrayElem _npcstatus 2 (Class|StellarGameState|GetInteractionStatus _asstellar_game_state "Munter") true)
    (Utilities|Array|SetArrayElem _npcstatus 3 (Class|StellarGameState|GetTreeIndex _asstellar_game_state "Munter") true)
    (Utilities|Array|SetArrayElem _npcstatus 4 (Class|StellarGameState|GetInteractionStatus _asstellar_game_state "Bunter") true)
    (Utilities|Array|SetArrayElem _npcstatus 5 (Class|StellarGameState|GetTreeIndex _asstellar_game_state "Bunter") true)
    (else
      (Class|StellarGameState|UpdateNPCData _asstellar_game_state "Gunter" (Utilities|Array|Get(acopy) _npcstatus_2) (Utilities|Array|Get(acopy) _npcstatus_2 1))
      (Class|StellarGameState|UpdateNPCData _asstellar_game_state "Munter" (Utilities|Array|Get(acopy) _npcstatus_2 2) (Utilities|Array|Get(acopy) _npcstatus_2 3))
      (Class|StellarGameState|UpdateNPCData _asstellar_game_state "Bunter" (Utilities|Array|Get(acopy) _npcstatus_2 4) (Utilities|Array|Get(acopy) _npcstatus_2 5))
      (for _array_element _npcstatus_2
        (Development|PrintString (Utilities|String|ToString(Integer) _array_element) true true "(R=1.000000,G=0.085000,B=0.000000,A=1.000000)" 1e+02))))
  (return))

(fn LampVariables
  (params (BP_Save :type BP%20Save%20Object%20Reference) (IsSaving :type Boolean))
  (if IsSaving
    (bind _outactors (Actor|GetAllActorsOfClass "/Game/Marcus/Enemy/BP_Lamp_TEST.BP_Lamp_TEST_C"))
    (bind _orderedactorrefs1 (CallFunction|GetAllActorsinOrderWorking _outactors))
    (for (_array_element _array_index) _orderedactorrefs1
      (bind _asbp_lamp_test (Utilities|Casting|CastToBP_Lamp_TEST _array_element))
      (Utilities|Array|SetArrayElem (Variables|/Game/Jacob/SaveAndLoad/BP_Save.BP_Save_C|GetLampisLit BP_Save) _array_index (Variables|/Game/Marcus/Enemy/BP_Lamp_TEST.BP_Lamp_TEST_C|GetLampIsLIt _asbp_lamp_test) true))
    (else
      (bind _outactors_2 (Actor|GetAllActorsOfClass "/Game/Marcus/Enemy/BP_Lamp_TEST.BP_Lamp_TEST_C"))
      (bind _orderedactorrefs1_2 (CallFunction|GetAllActorsinOrderWorking _outactors_2))
      (for (_array_element_2 _array_index_2) _orderedactorrefs1_2
        (bind _asbp_lamp_test_2 (Utilities|Casting|CastToBP_Lamp_TEST _array_element_2))
        (Variables|/Game/Marcus/Enemy/BP_Lamp_TEST.BP_Lamp_TEST_C|SetLampIsLIt _asbp_lamp_test_2 (Utilities|Array|Get(acopy) (Variables|Default|GetLampisLit) _array_index_2)))))
  (return))

(fn LeverVariables
  (params (BP_Save :type BP%20Save%20Object%20Reference) (IsSaving :type Boolean))
  (if IsSaving
    (bind _outactors (Actor|GetAllActorsOfClass "/Game/Jacob/Objects/Levers/BP_Lever_DELETE.BP_Lever_DELETE_C"))
    (for _array_element _outactors
      (Variables|/Game/Jacob/SaveAndLoad/BP_Save.BP_Save_C|SetSwitchActivated BP_Save (Variables|/Game/Jacob/BP_Lever_Parent.BP_Lever_Parent_C|GetSwitchActivated _array_element)))
    (return)
    (else
      (bind _outactors_2 (Actor|GetAllActorsOfClass "/Game/Jacob/Objects/Levers/BP_Lever_DELETE.BP_Lever_DELETE_C"))
      (for _array_element_2 _outactors_2
        (Variables|/Game/Jacob/BP_Lever_Parent.BP_Lever_Parent_C|SetSwitchActivated _array_element_2 (Variables|Default|GetSwitchActivated)))
      (return))))

(fn PlayerCustomizationVariables
  (params (IsSaving :type Boolean) (BP_Save :type BP%20Save%20Object%20Reference))
  (bind _returnvalue (SaveGame|LoadGamefromSlot "SaveGame"))
  (bind _assave_game (Utilities|Casting|CastToSaveGame _returnvalue))
  (if IsSaving
    (Variables|/Game/Jacob/SaveAndLoad/BP_Save.BP_Save_C|SetThemeIndex BP_Save (Variables|/Game/Sound/SaveGame.SaveGame_C|GetThemeIndex _assave_game))
    (else
      (Variables|/Game/Sound/SaveGame.SaveGame_C|SetThemeIndex _assave_game (Variables|Default|GetThemeIndex))))
  (return))