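; Pushable and draggable stone whose cube starts simulating physics when the Jacob player character grabs it.
; The grab interaction toggles between grab and drop by flipping the player's IsPushingObject flag, which is set false on grab and true on drop.
; Grabbing requires CanInteract and shows text, while dropping requires the player's CanDropObject and hides it.
; Tick and construction only defer to the parent.
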(event EventBeginPlay)

(event Collision|EventActorBeginOverlap
  (params (OtherActor :type Actor%20Object%20Reference)))

(event EventTick
  (params (DeltaSeconds :type Float%20%28single-precision%29))
  (|CallParentFunction 0.0))

(event EventInteractGrab
  (params (Instigator :type Actor%20Object%20Reference))
  (bind _asbp_player_jacob (Utilities|Casting|CastToBP_PlayerJacob Instigator))
  (if (Variables|/Game/ThirdPerson/Blueprints/BP_PlayerJacob.BP_PlayerJacob_C|GetIsPushingObject _asbp_player_jacob)
    (if (Variables|Default|GetbCanInteract?)
      (Variables|/Game/ThirdPerson/Blueprints/BP_PlayerJacob.BP_PlayerJacob_C|SetIsPushingObject _asbp_player_jacob false)
      (Default|GrabandPushObject _asbp_player_jacob)
      (Physics|SetSimulatePhysics (Variables|Default|GetCube) true)
      (CallFunction|TextEnable))
    (elif (Variables|/Game/ThirdPerson/Blueprints/BP_PlayerJacob.BP_PlayerJacob_C|GetCanDropObject _asbp_player_jacob)
      (Variables|/Game/ThirdPerson/Blueprints/BP_PlayerJacob.BP_PlayerJacob_C|SetIsPushingObject _asbp_player_jacob true)
      (Default|DropandPushObject _asbp_player_jacob)
      (CallFunction|TextDisable))))

(fn ConstructionScript
  (|CallParentFunction))