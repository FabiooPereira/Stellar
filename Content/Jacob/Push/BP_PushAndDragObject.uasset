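; Interactable push-and-drag object that the Jacob player character can grab and release.
; When the player is not already holding or pushing something, SetInteractableState toggles the cube's custom depth rendering and the HUD drag prompt.
; InteractPush uses a FlipFlop to alternate between PushObject, if interactable, and ReleaseObject, if dropping is allowed, on the player.
; The FlipFlop advances even when those checks fail.
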(event EventInteractPush
  (params (Instigator :type Actor%20Object%20Reference))
  ;[1 1 1] Interact Push
  (bind _asbp_player_jacob (Utilities|Casting|CastToBP_PlayerJacob Instigator))
  (Utilities|FlowControl|FlipFlop
    (:A
      (if (Variables|Default|GetbCanInteract?)
        (Default|PushObject _asbp_player_jacob)
        (CallFunction|TextEnable)))
    (:B
      (if (Variables|/Game/ThirdPerson/Blueprints/BP_PlayerJacob.BP_PlayerJacob_C|GetCanDropObject _asbp_player_jacob)
        (Default|ReleaseObject _asbp_player_jacob)
        (CallFunction|TextDisable)))))

(event EventSetInteractableState
  (params (bCanShowInteract :type Boolean))
  (bind _cube (Variables|Default|GetCube))
  ;[1 1 1] Interactable State
  (bind _asbp_player_jacob (Utilities|Casting|CastToBP_PlayerJacob (Game|GetPlayerCharacter 0)))
  (if (not (or (Variables|/Game/ThirdPerson/Blueprints/BP_PlayerJacob.BP_PlayerJacob_C|GetIsHoldingObject _asbp_player_jacob) (Variables|/Game/ThirdPerson/Blueprints/BP_PlayerJacob.BP_PlayerJacob_C|GetIsPushingObject _asbp_player_jacob)))
    (bind _output_get (Variables|Default|SetbCanInteract? bCanShowInteract))
    (if _output_get
      (CallFunction|TextEnable)
      (Rendering|SetRenderCustomDepth _cube true)
      (else
        (CallFunction|TextDisable)
        (Rendering|SetRenderCustomDepth _cube false)))))

(event EventTick
  (params (DeltaSeconds :type Float%20%28single-precision%29)))

(fn ConstructionScript)

(fn TextDisable
  (bind _as_new_hud (Variables|Default|GetAs%20New%20HUD)
    (:then
      (Default|SetTextInputPlayer (Variables|/Game/Jacob/UI/NewHUD.NewHUD_C|GetUIRef _as_new_hud) "" "" false))
    (:else)))

(fn TextEnable
  (bind _asnew_hud (Utilities|Casting|CastToNewHUD (HUD|GetHUD (Game|GetPlayerController 0))))
  (bind _output_get (Variables|Default|SetAs%20New%20HUD _asnew_hud))
  (Default|SetTextInputPlayer (Variables|/Game/Jacob/UI/NewHUD.NewHUD_C|GetUIRef _output_get) "DRAG: B" "DRAG: E" true))