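; BP_PushAndDragObject_Bridge is a pushable bridge object that controls BP_PlayerJacob's movement speed during pushing.
; After parent Tick logic, it sphere-traces from the cube along the overlapping player's last input, halting the player when WorldStatic geometry blocks the way.
; Otherwise, max walk speed follows a WalkSpeed timeline, which a DoOnce gate replays continuously.
; A helper, not called here, finds the held key for an Enhanced Input action.
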(event EventBeginPlay)

(event Collision|EventActorBeginOverlap
  (params (OtherActor :type Actor%20Object%20Reference)))

(event EventTick
  (params (DeltaSeconds :type Float%20%28single-precision%29))
  ;[1 1 1] Tick
  (|CallParentFunction DeltaSeconds)
  (CallFunction|CheckforCollision)
  (CallFunction|SetCurveWalkSpeed))

(event EventSetCurveWalkSpeed
  ;[1 1 1] Curve Walk Speed
  (Utilities|FlowControl|DoOnce false :!label _label
    (:Completed
      (bind _walkspeed (Timeline|WalkSpeed PlayFromStart)
        (:Update
          (Variables|Default|SetCurveWalkSpeed _walkspeed))
        (:Finished
          (goto _label Reset))))))

(fn ConstructionScript
  (|CallParentFunction))

(fn GetActionPressedKey
  (params (Action :type Input%20Action%20Object%20Reference))
  (bind _asplayer_controller (Utilities|Casting|CastToPlayerController (Pawn|GetController (Game|GetPlayerCharacter 0))))
  (bind _returnvalue (Class|EnhancedInputSubsystemInterface|QueryKeysMappedtoAction(Message) (PlayerController|LocalPlayerSubsystems|GetEnhancedInputLocalPlayerSubsystem _asplayer_controller) Action))
  (for _array_element _returnvalue
    (if (Game|Player|IsInputKeyDown _asplayer_controller _array_element)
      (return _array_element))))

(fn CheckforCollision
  (bind _cube (Variables|Default|GetCube))
  (bind _returnvalue (Transformation|GetWorldLocation _cube))
  (bind _returnvalue_2 (+ _returnvalue "0.000000,0.000000,90.000000"))
  (bind _asbp_player_jacob (Utilities|Casting|CastToBP_PlayerJacob (Game|GetPlayerCharacter 0)))
  (Variables|Default|SetCharacter%20Movement (Variables|/Script/Engine.Character|GetCharacterMovement _asbp_player_jacob))
  (if (Collision|IsOverlappingActor _asbp_player_jacob :!class /Script/Engine.Actor)
    (if (Variables|/Game/ThirdPerson/Blueprints/BP_PlayerJacob.BP_PlayerJacob_C|GetIsPushingObject _asbp_player_jacob)
      (bind _returnvalue_3 (Collision|SphereTraceForObjects _returnvalue_2 (+ _returnvalue_2 (* (Math|Vector|Normalize (Pawn|Components|PawnMovement|GetLastInputVector (Variables|Default|GetCharacter%20Movement))) "90.000000,90.000000,0.000000")) 55.0 (Utilities|Array|MakeArray "ObjectTypeQuery1") true (Utilities|Array|MakeArray _asbp_player_jacob self) "ForOneFrame"))
      (if _returnvalue_3
        (Variables|/Script/Engine.CharacterMovementComponent|SetMinAnalogWalkSpeed (Variables|Default|GetCharacter%20Movement) 0.0)
        (Variables|/Script/Engine.CharacterMovementComponent|SetMaxWalkSpeed (Variables|Default|GetCharacter%20Movement) 0.0)
        (else
          (Variables|/Script/Engine.CharacterMovementComponent|SetMinAnalogWalkSpeed (Variables|Default|GetCharacter%20Movement) 2e+01)
          (Variables|/Script/Engine.CharacterMovementComponent|SetMaxWalkSpeed (Variables|Default|GetCharacter%20Movement) (Variables|Default|GetCurveWalkSpeed)))))))