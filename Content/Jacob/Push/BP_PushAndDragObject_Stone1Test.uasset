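; BP_PushAndDragObject_Stone1Test is a test push-and-drag stone that stops the player from moving it into static world geometry.
; Each tick, while an overlapping BP_PlayerJacob holds an object, it sphere-traces WorldStatic objects just ahead of the cube along the player's last input direction.
; A hit zeroes the player's walk speeds; otherwise it sets fixed walk speeds.
; Debug drawing and print strings remain active.
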(event EventBeginPlay)

(event Collision|EventActorBeginOverlap
  (params (OtherActor :type Actor%20Object%20Reference)))

(event EventTick
  (params (DeltaSeconds :type Float%20%28single-precision%29))
  ;[1 1 1] Tick
  (|CallParentFunction 0.0)
  (CallFunction|CheckforCollision))

(fn ConstructionScript
  (|CallParentFunction))

(fn CheckforCollision
  (bind _cube (Variables|Default|GetCube))
  (bind _returnvalue (Transformation|GetWorldLocation _cube))
  (bind _returnvalue_2 (+ _returnvalue "0.000000,0.000000,45.000000"))
  (bind _asbp_player_jacob (Utilities|Casting|CastToBP_PlayerJacob (Game|GetPlayerCharacter 0)))
  (Variables|Default|SetCharacter%20Movement (Variables|/Script/Engine.Character|GetCharacterMovement _asbp_player_jacob))
  (if (Collision|IsOverlappingActor _asbp_player_jacob :!class /Script/Engine.Actor)
    (if (Variables|/Game/ThirdPerson/Blueprints/BP_PlayerJacob.BP_PlayerJacob_C|GetIsHoldingObject _asbp_player_jacob)
      (bind (_outhit _returnvalue_3) (Collision|SphereTraceForObjects _returnvalue_2 (+ _returnvalue_2 (* (Math|Vector|Normalize (Pawn|Components|PawnMovement|GetLastInputVector (Variables|Default|GetCharacter%20Movement))) "20.000000,20.000000,0.000000")) 4e+01 (Utilities|Array|MakeArray "ObjectTypeQuery1") false (Utilities|Array|MakeArray _asbp_player_jacob self) "ForOneFrame"))
      (if _returnvalue_3
        (Variables|/Script/Engine.CharacterMovementComponent|SetMinAnalogWalkSpeed (Variables|Default|GetCharacter%20Movement) 0.0)
        (Variables|/Script/Engine.CharacterMovementComponent|SetMaxWalkSpeed (Variables|Default|GetCharacter%20Movement) 0.0)
        (Development|PrintString "Overlapping")
        (else
          (Variables|/Script/Engine.CharacterMovementComponent|SetMinAnalogWalkSpeed (Variables|Default|GetCharacter%20Movement) 2e+01)
          (Variables|/Script/Engine.CharacterMovementComponent|SetMaxWalkSpeed (Variables|Default|GetCharacter%20Movement) 1.5e+02)
          (Development|PrintString "NOT overlapping"))))))