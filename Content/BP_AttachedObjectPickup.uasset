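; BP_AttachedObjectPickup is a cube pickup that characters implementing BPI_CharacterAttachmentInteraction can interact with and hold.
; Box begin-overlap and Cube end-overlap notify that interface, with the end message suppressed while the object is held.
; Events set the held flag, swap the material for interactable state, and enable physics through ApplyForcewithDirection.
; ResetForce stops simulation, moves the actor to the cube's location and reattaches the cube to the root.
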(event OnComponentBeginOverlap(Box)
  (params (OverlappedComponent :type Primitive%20Component%20Object%20Reference) (OtherActor :type Actor%20Object%20Reference) (OtherComp :type Primitive%20Component%20Object%20Reference) (OtherBodyIndex :type Integer) (bFromSweep :type Boolean) (SweepResult :type Hit%20Result%20Structure%20%28by%20ref%29))
  ;[1 1 1] Begin Overlap
  (if (Utilities|DoesObjectImplementInterface OtherActor "/Game/BPI_CharacterAttachmentInteraction.BPI_CharacterAttachmentInteraction_C")
    (Class|BPICharacterAttachmentInteraction|OverlapStatusChange(Message) OtherActor "NewEnumerator0" self)))

(event OnComponentEndOverlap(Cube)
  (params (OverlappedComponent :type Primitive%20Component%20Object%20Reference) (OtherActor :type Actor%20Object%20Reference) (OtherComp :type Primitive%20Component%20Object%20Reference) (OtherBodyIndex :type Integer))
  ;[1 1 1] End Overlap
  (if (and (Utilities|DoesObjectImplementInterface OtherActor "/Game/BPI_CharacterAttachmentInteraction.BPI_CharacterAttachmentInteraction_C") (not (Variables|Default|GetObjectPickedUp)))
    (Class|BPICharacterAttachmentInteraction|OverlapStatusChange(Message) OtherActor "NewEnumerator1")))

(event EventBeginPlay
  (Physics|SetSimulatePhysics (Variables|Default|GetCube) false))

(event Collision|EventActorBeginOverlap
  (params (OtherActor :type Actor%20Object%20Reference)))

(event EventTick
  (params (DeltaSeconds :type Float%20%28single-precision%29)))

(event EventChangeHoldingStatusonObject
  (params (IsHolding :type Boolean))
  ;[1 1 1] Status Change
  (Variables|Default|SetObjectPickedUp IsHolding))

(event EventSetInteractableState
  (params (bCanShowInteract? :type Boolean))
  (bind _cube (Variables|Default|GetCube))
  ;[1 1 1] Interactable State
  (bind _output_get (Variables|Default|SetbCanInteract? bCanShowInteract?))
  (if _output_get
    (Rendering|Material|SetMaterial _cube 0 "/Engine/VREditor/BasicMeshes/MI_Cube_03.MI_Cube_03")
    (else
      (Rendering|Material|SetMaterial _cube 0 "/Engine/BasicShapes/BasicShapeMaterial.BasicShapeMaterial"))))

(event EventResetForce
  (bind _cube (Variables|Default|GetCube))
  ;[1 1 1] Reset Force
  (if (Physics|IsSimulatingPhysics _cube "None")
    (Physics|SetSimulatePhysics _cube false)
    (Transformation|SetActorLocation (Transformation|GetWorldLocation _cube) false false)
    (Transformation|AttachComponentToComponent (Variables|Default|GetCube) (Variables|Default|GetDefaultSceneRoot) "None" "KeepWorld" "KeepWorld" "KeepWorld" true)))

(event EventApplyForcewithDirection
  (params (DirectionVector :type Vector :default "0, 0, 0") (Power :type Float%20%28double-precision%29))
  ;[1 1 1] Apply Force With Direction
  (Physics|SetSimulatePhysics (Variables|Default|GetCube) true))

(fn ConstructionScript)