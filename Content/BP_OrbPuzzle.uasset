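; BP_OrbPuzzle is a quest puzzle actor that completes when enough of its own child actors, presumably orbs, overlap it.
; On BeginPlay it counts the box components under its root as the required Triggers.
; Begin and end overlaps from its child actors adjust a Triggered count, and reaching the total on a begin overlap calls EndQuest.
; BeginQuest only prints debug text, and disconnected nodes hold a player detach-and-teleport step.
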(event EventBeginPlay
  (for _array_element (Components|GetChildrenComponents (Variables|Default|GetDefaultSceneRoot) false)
    (Utilities|Casting|CastToBoxComponent _array_element
      (:then
        (Math|Integer|IncrementInt (Variables|Default|GetTriggers)
          (:%20%20
            (Development|PrintString (Utilities|GetDisplayName 0)))))
      (:CastFailed
        (Development|PrintString "cast failed"))))
  (Development|PrintString "total triggers is:")
  (Development|PrintString (Utilities|String|ToString(Integer) 0))
  (Development|PrintString "triggered is:")
  (Development|PrintString (Utilities|String|ToString(Integer) (Variables|Default|GetTriggered))))

(event Collision|EventActorBeginOverlap
  (params (OtherActor :type Actor%20Object%20Reference))
  (bind _triggers (Variables|Default|GetTriggers))
  (bind _triggered (Variables|Default|GetTriggered))
  (bind _returnvalue (Utilities|String|ToString(Integer) _triggered))
  (bind _returnvalue_2 (Utilities|String|ToString(Integer) _triggers))
  (if (== (Actor|GetParentActor OtherActor) self)
    (Development|PrintString "CHILD")
    (Math|Integer|IncrementInt _triggered
      (:%20%20
        (Development|PrintString "triggered is:")
        (if (== _triggered _triggers)
          (Development|PrintString _returnvalue)
          (Development|PrintString _returnvalue_2)
          (Class|Quest|EndQuest)
          (Development|PrintString "END")
          (else
            (Development|PrintString _returnvalue)
            (Development|PrintString _returnvalue_2)))))
    (else
      (Development|PrintString "NOT CHILD"))))

(event EventTick
  (params (DeltaSeconds :type Float%20%28single-precision%29)))

(event Collision|EventActorEndOverlap
  (params (OtherActor :type Actor%20Object%20Reference))
  (bind _triggered (Variables|Default|GetTriggered))
  (if (== (Actor|GetParentActor OtherActor) self)
    (Development|PrintString "CHILD")
    (Math|Integer|DecrementInt _triggered
      (:%20%20
        (Development|PrintString "triggered is:")
        (Development|PrintString (Utilities|String|ToString(Integer) _triggered))))
    (else
      (Development|PrintString "NOT CHILD"))))

(event EventBeginQuest
  (Development|PrintString "Begin orb puzzle"))

(fn ConstructionScript)