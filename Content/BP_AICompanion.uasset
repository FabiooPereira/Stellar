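; BP_AICompanion is an AI companion that adjusts its walk speed to its position relative to the player.
; A looping timer takes the dot product of the player's forward vector and the companion-to-player direction, raising a pace multiplier when the companion is behind the player.
; Tick smoothly interpolates max walk speed toward the base speed scaled by that pace and prints it for debugging.
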(event Custom|SetPace
  (bind _returnvalue (Game|GetPlayerCharacter 0))
  (Variables|Default|SetPace (Math|Float|SelectFloat 1.0 1.2 (<= (Math|Float|Sign(Float) (Math|Vector|DotProduct (Transformation|GetActorForwardVector _returnvalue) (Math|Vector|GetUnitDirection(Vector) (Transformation|GetActorLocation) (Transformation|GetActorLocation _returnvalue)))) 0.0))))

(event EventBeginPlay
  (Utilities|Time|SetTimerbyEvent (delegate Custom|SetPace) 0.2 true))

(event EventTick
  (params (DeltaSeconds :type Float%20%28single-precision%29))
  (bind _output_get (Variables|/Script/Engine.CharacterMovementComponent|SetMaxWalkSpeed (Variables|Character|GetCharacterMovement) (Math|Interpolation|FInterpTo (Variables|/Script/Engine.CharacterMovementComponent|GetMaxWalkSpeed (Variables|Character|GetCharacterMovement)) (* 5.5e+02 (Variables|Default|GetPace)) DeltaSeconds 2.0)))
  (Development|PrintString (Utilities|String|ToString(Float) _output_get)))

(fn ConstructionScript)