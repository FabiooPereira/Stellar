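; Game mode for Beyond The Fluff that sets up the pause menu and starts background audio.
; On BeginPlay it creates the pause menu widget, adds it to the viewport and spawns the starter background cue at the world origin.
; PauseGame, gated by CanPause, calls FreezeGame to toggle the game's paused state, then calls SetVisible on the menu.
; Debug prints trace startup and pausing.
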(event EventBeginPlay
  (Development|PrintString "GameModeBeginPlay")
  (bind _returnvalue (UserInterface|CreateWidget "/Game/Widgets/WBP_PauseMenu.WBP_PauseMenu_C"))
  (bind _output_get (Variables|Default|SetPause%20Menu _returnvalue))
  (UserInterface|Viewport|AddtoViewport _output_get 0)
  (Audio|SpawnSoundatLocation "/Game/StarterContent/Audio/Starter_Background_Cue.Starter_Background_Cue" "0, 0, 0" "0, 0, 0" 1.0 1.0 0.0 0 0))

(event EventTick
  (params (DeltaSeconds :type Float%20%28single-precision%29)))

(fn ConstructionScript)

(fn FreezeGame
  (bind _returnvalue (Game|IsGamePaused))
  (bind _returnvalue_2 (not _returnvalue))
  (Game|SetGamePaused _returnvalue_2)
  (Development|PrintString (Utilities|String|ToString(Boolean) _returnvalue_2))
  (Development|PrintString " Pause"))

(fn PauseGame
  (if (Variables|Default|GetCanPause)
    (CallFunction|FreezeGame)
    (Default|SetVisible (Variables|Default|GetPause%20Menu))))