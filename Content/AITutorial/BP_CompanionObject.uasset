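; Interactable world object that calls the AI companion over to act on it.
; On interaction it finds the BP_AICompanion and writes itself into the companion's TargetActor blackboard key.
; When that companion overlaps it, it plays a T-pose montage on the companion, waits for the returned montage length, then clears the key to release it.
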(event EventBeginPlay)

(event EventTick
  (params (DeltaSeconds :type Float%20%28single-precision%29)))

(event EventInteracwith
  (bind _returnvalue (Actor|GetActorOfClass "/Game/AITutorial/BP_AICompanion.BP_AICompanion_C"))
  (Variables|Default|SetCompanion _returnvalue)
  (AI|Components|Blackboard|SetValueasObject (AI|GetBlackboard (AI|GetAIController _returnvalue)) (Utilities|Name|MakeLiteralName "TargetActor") self))

(event Collision|EventActorBeginOverlap
  (params (OtherActor :type Actor%20Object%20Reference))
  (bind _companion (Variables|Default|GetCompanion)
    (:then
      (if (== _companion OtherActor)
        (bind _returnvalue (Animation|PlayAnimMontage (Variables|Default|GetCompanion) "/Game/AITutorial/MM_T_Pose_Montage.MM_T_Pose_Montage" 1.0 "None"))
        (Utilities|FlowControl|Delay _returnvalue)
        (AI|Components|Blackboard|ClearValue (AI|GetBlackboard (AI|GetAIController (Variables|Default|GetCompanion))) (Utilities|Name|MakeLiteralName "TargetActor"))))
    (:else)))

(fn ConstructionScript)