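; AI controller for a companion pawn that runs a behavior tree to follow the player using predicted movement.
; A looping timer requests an AI perception prediction of where the player will be a couple of seconds ahead.
; On perception updates, if the player is moving fast and is far from the companion, it writes a random reachable point near the stimulus to the TargetLocation blackboard key.
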(event OnTargetPerceptionUpdated(AIPerception)
  (params (Actor :type Actor%20Object%20Reference) (Stimulus :type AI%20Stimulus%20Structure))
  (if (CallFunction|ShouldGoAfterPlayer)
    (AI|Components|Blackboard|SetValueasVector (AI|GetBlackboard 0) (Utilities|Name|MakeLiteralName "TargetLocation") (.RandomLocation (AI|Navigation|GetRandomReachablePointinRadius (.StimulusLocation (Utilities|Struct|BreakAIStimulus Stimulus)) 1e+02 0 0)))))

(event Custom|GetLocation
  (Class|AISensePrediction|RequestPawnPredictionEvent (Pawn|GetControlledPawn) (Game|GetPlayerCharacter 0) 2.0))

(event EventBeginPlay
  (AI|RunBehaviorTree "/Game/AITutorial/BT_CompanionBehaviour.BT_CompanionBehaviour")
  (Utilities|Time|SetTimerbyEvent (delegate Custom|GetLocation) 1.0 true))

(event EventTick
  (params (DeltaSeconds :type Float%20%28single-precision%29)))

(fn ConstructionScript)

(fn ShouldGoAfterPlayer
  (bind _returnvalue (Game|GetPlayerCharacter 0))
  (return (and (> (Math|Vector|VectorLength (Transformation|GetVelocity _returnvalue)) 2e+02) (> (Math|Vector|Distance(Vector) (Transformation|GetActorLocation _returnvalue) (Transformation|GetActorLocation (Pawn|GetControlledPawn))) 5e+02))))