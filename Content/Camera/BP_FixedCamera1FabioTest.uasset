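; Test variant of a fixed camera zone that blends the view to itself when the player enters its box, optionally blending back on exit.
; Each tick the spring arm tracks the player's closest spline points, with interpolated X/Z from Spline and direct Y from SplineY.
; Tick also picks a front or back collision offset by player facing.
; Construction previews the camera along the spline; look-at rotation logic is disconnected.
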(event OnComponentBeginOverlap(Box)
  (params (OverlappedComponent :type Primitive%20Component%20Object%20Reference) (OtherActor :type Actor%20Object%20Reference) (OtherComp :type Primitive%20Component%20Object%20Reference) (OtherBodyIndex :type Integer) (bFromSweep :type Boolean) (SweepResult :type Hit%20Result%20Structure%20%28by%20ref%29))
  (Development|PrintString (Utilities|GetDisplayName OtherActor))
  (if (== OtherActor (Game|GetPlayerCharacter 0))
    (Variables|Default|SetIsPlayerInside true)
    (CallFunction|OnFixedCamOverlap)
    (bind _asbp_third_person_character (Utilities|Casting|CastToBP_ThirdPersonCharacter (Game|GetPlayerCharacter 0)))
    (Variables|/Game/ThirdPerson/Blueprints/BP_ThirdPersonCharacter.BP_ThirdPersonCharacter_C|SetLastCameraRef _asbp_third_person_character self)))

(event OnComponentEndOverlap(Box)
  (params (OverlappedComponent :type Primitive%20Component%20Object%20Reference) (OtherActor :type Actor%20Object%20Reference) (OtherComp :type Primitive%20Component%20Object%20Reference) (OtherBodyIndex :type Integer))
  (bind _returnvalue (Game|GetPlayerCharacter 0))
  (if (== OtherActor (Game|GetPlayerCharacter 0))
    (Variables|Default|SetIsPlayerInside false)
    (CallFunction|OnFIxedCamEndOverlap)
    (if (Variables|Default|GetChangeOnExit)
      (Game|Player|SetViewTargetwithBlend (Game|GetPlayerController 0) (Game|GetPlayerCharacter 0) 3.0 "VTBlend_EaseInOut" 2.0 true)
      (bind _asgrupp_onion_character (Utilities|Casting|CastToGruppOnionCharacter (Game|GetPlayerCharacter 0)))
      (Variables|/Script/GruppOnion.GruppOnionCharacter|SetCustomCamera _asgrupp_onion_character (Variables|/Script/GruppOnion.GruppOnionCharacter|GetFollowCamera _asgrupp_onion_character))
      (bind _asbp_third_person_character (Utilities|Casting|CastToBP_ThirdPersonCharacter _returnvalue))
      (Variables|/Game/ThirdPerson/Blueprints/BP_ThirdPersonCharacter.BP_ThirdPersonCharacter_C|SetLastCameraRef _asbp_third_person_character _returnvalue))))

(event EventTick
  (params (DeltaSeconds :type Float%20%28single-precision%29))
  (bind _returnvalue (Game|GetPlayerCharacter 0))
  (bind _returnvalue_2 (Transformation|GetActorLocation _returnvalue))
  (Variables|Default|SetDelta%20Seconds DeltaSeconds)
  (CallFunction|SetPlayerCollisionOffset)
  (Transformation|SetWorldLocation (Variables|Default|GetSpringArm) (Math|Vector|MakeVector (.x (Math|Interpolation|VInterpTo (Transformation|GetWorldLocation (Variables|Default|GetSpringArm)) (Spline|FindLocationClosesttoWorldLocation (Variables|Default|GetSpline) _returnvalue_2 "World") (Variables|Default|GetDelta%20Seconds) (Variables|Default|GetInterp%20Speed))) (.y (Spline|FindLocationClosesttoWorldLocation (Variables|Default|GetSplineY) _returnvalue_2 "World")) (.z (Math|Interpolation|VInterpTo (Transformation|GetWorldLocation (Variables|Default|GetSpringArm)) (Spline|FindLocationClosesttoWorldLocation (Variables|Default|GetSpline) _returnvalue_2 "World") (Variables|Default|GetDelta%20Seconds) (Variables|Default|GetInterp%20Speed)))) false false))

(fn ConstructionScript
  (CallFunction|SnaptoSpline)
  (Variables|/Script/Engine.SpringArmComponent|SetTargetArmLength (Variables|Default|GetSpringArm) (Variables|Default|GetSpringArmLenght)))

(fn OnFixedCamOverlap
  (Game|Player|SetViewTargetwithBlend (Game|GetPlayerController 0) self (Variables|Default|GetBlend%20Time) (Variables|Default|GetBlend%20Func) 2.0 true))

(fn SnaptoSpline
  (bind _spline (Variables|Default|GetSpline))
  (bind _camerapoint (Variables|Default|GetCameraPoint))
  (bind _returnvalue (Spline|GetSplineLength _spline))
  (bind _returnvalue_2 (Math|Float|Lerp 0.0 _returnvalue _camerapoint))
  (Transformation|SetWorldTransform (Variables|Default|GetCamera) (Math|Transform|MakeTransform (Spline|GetLocationatDistanceAlongSpline (Variables|Default|GetSpline) _returnvalue_2 "World") (Spline|GetRotationatDistanceAlongSpline (Variables|Default|GetSpline) _returnvalue_2 "World") "1.000000,1.000000,1.000000") false false))

(fn OnFIxedCamEndOverlap)

(fn SetPlayerCollisionOffset
  (Variables|Default|SetPlayerCollisionOffset (select (> (Math|Vector|DotProduct (Math|Vector|GetForwardVector (Variables|Default|GetCamera)) (Transformation|GetActorForwardVector (Game|GetPlayerCharacter 0))) 0.0) (Variables|Default|GetPlayerBackCollisionOffset) (Variables|Default|GetPlayerFrontCollisionOffset))))