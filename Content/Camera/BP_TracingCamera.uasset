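; BP_TracingCamera is a camera actor that turns to face player character 0 every tick.
; LookToPlayer snaps rotation to the look-at angle and prints it, ignoring its Delta and Power inputs; disconnected nodes hold unfinished rotation smoothing.
; MoveToTarget eases position toward TargetLocation with a delta-scaled lerp.
; TargetLocation starts at the actor's own location and is not changed in this Blueprint.
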(event Custom|LookToPlayer
  (params (Delta :type Float%20%28double-precision%29) (Power :type Float%20%28double-precision%29))
  (bind _returnvalue (Transformation|GetActorLocation))
  (bind _returnvalue_2 (Game|GetPlayerCharacter 0))
  (bind _returnvalue_3 (Transformation|GetActorLocation _returnvalue_2))
  (bind _returnvalue_4 (Math|Rotator|FindLookatRotation _returnvalue _returnvalue_3))
  (Transformation|SetActorRotation _returnvalue_4 true)
  (Development|PrintString (Utilities|String|ToString(Rotator) _returnvalue_4)))

(event Custom|MoveToTarget
  (params (Delta :type Float%20%28double-precision%29) (Power :type Float%20%28double-precision%29))
  (Transformation|SetActorLocation (Math|Vector|Lerp(Vector) (Transformation|GetActorLocation) (Variables|Default|GetTargetLocation) (* Delta Power)) false true))

(event EventBeginPlay
  (Variables|Default|SetTargetLocation (Transformation|GetActorLocation)))

(event EventTick
  (params (DeltaSeconds :type Float%20%28single-precision%29))
  (CallFunction|LooktoPlayer DeltaSeconds 3.0)
  (CallFunction|MovetoTarget DeltaSeconds 0.9))

(fn ConstructionScript)

(fn GetTargetLocation
  (return (Math|Rotator|FindLookatRotation (Transformation|GetActorLocation) (Transformation|GetActorLocation (Game|GetPlayerCharacter 0)))))