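; Camera actor that turns to face player character 0 and eases toward a stored target location.
; Each tick it snaps its rotation to the player and lerps its position by delta time, leaving the look power input unused.
; The target is set to the camera's own start location, not the player's, and is not updated here.
; GetTargetLocation returns a look-at rotation despite its name.
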(event Custom|LookToPlayer
  (params (Delta :type Float%20%28double-precision%29) (Power :type Float%20%28double-precision%29))
  ;[1 1 1] Rotates the camera to the player
  (Transformation|SetActorRotation (Math|Rotator|FindLookatRotation (Transformation|GetActorLocation) (Transformation|GetActorLocation (Game|GetPlayerCharacter 0))) true))

(event Custom|MoveToTarget
  (params (Delta :type Float%20%28double-precision%29) (Power :type Float%20%28double-precision%29))
  ;[1 1 1] Moves the camera to the new position
  (Transformation|SetActorLocation (Math|Vector|Lerp(Vector) (Transformation|GetActorLocation) (Variables|Default|GetTargetLocation) (* Delta Power)) false true))

(event EventBeginPlay
  ;[1 1 1] Gets player location and sets it as a target
  (Variables|Default|SetTargetLocation (Transformation|GetActorLocation)))

(event EventTick
  (params (DeltaSeconds :type Float%20%28single-precision%29))
  ;[1 1 1] Runs LookToPlayer and MoveToTarget every tick
  (CallFunction|LooktoPlayer DeltaSeconds 3.0)
  (CallFunction|MovetoTarget DeltaSeconds 0.9))

(fn ConstructionScript)

(fn GetTargetLocation
  (return (Math|Rotator|FindLookatRotation (Transformation|GetActorLocation) (Transformation|GetActorLocation (Game|GetPlayerCharacter 0)))))