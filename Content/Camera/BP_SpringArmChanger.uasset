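; BP_SpringArmChanger is a trigger volume that changes the player's camera boom while the player is inside its Box.
; Player overlap plays a timeline that drives the SpringArmComponent's TargetArmLength and TargetOffset Z, copying X and Y from SocketOffset.
; End overlap reverses the timeline for any actor, without a player check.
; InitialArmLength is saved on entry, but its restore logic is disconnected, so arm lengths come from the timeline curves.
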(event OnComponentBeginOverlap(Box)
  (params (OverlappedComponent :type Primitive%20Component%20Object%20Reference) (OtherActor :type Actor%20Object%20Reference) (OtherComp :type Primitive%20Component%20Object%20Reference) (OtherBodyIndex :type Integer) (bFromSweep :type Boolean) (SweepResult :type Hit%20Result%20Structure%20%28by%20ref%29))
  (bind _returnvalue (Game|GetPlayerCharacter 0))
  (bind _returnvalue_2 (Game|GetPlayerCharacter 0))
  (bind _returnvalue_3 (Actor|GetComponentbyClass _returnvalue_2 "/Script/Engine.SpringArmComponent"))
  (bind _returnvalue_4 (Actor|GetComponentbyClass _returnvalue "/Script/Engine.SpringArmComponent"))
  (bind _socketoffset (Variables|/Script/Engine.SpringArmComponent|GetSocketOffset _returnvalue_3))
  (if (== OtherActor (Game|GetPlayerCharacter 0))
    (Variables|Default|SetInitialArmLength (Variables|/Script/Engine.SpringArmComponent|GetTargetArmLength _returnvalue_3))
    (bind (_direction _springarm _zoffset) (Timeline|Timeline Play)
      (:Update
        (Variables|/Script/Engine.SpringArmComponent|SetTargetArmLength _returnvalue_4 _springarm)
        (Variables|/Script/Engine.SpringArmComponent|SetTargetOffset _returnvalue_4 (Math|Vector|MakeVector (.x _socketoffset) (.y _socketoffset) _zoffset))))))

(event OnComponentEndOverlap(Box)
  (params (OverlappedComponent :type Primitive%20Component%20Object%20Reference) (OtherActor :type Actor%20Object%20Reference) (OtherComp :type Primitive%20Component%20Object%20Reference) (OtherBodyIndex :type Integer))
  (bind _returnvalue (Game|GetPlayerCharacter 0))
  (bind _returnvalue_2 (Game|GetPlayerCharacter 0))
  (bind _returnvalue_3 (Actor|GetComponentbyClass _returnvalue_2 "/Script/Engine.SpringArmComponent"))
  (bind _returnvalue_4 (Actor|GetComponentbyClass _returnvalue "/Script/Engine.SpringArmComponent"))
  (bind _socketoffset (Variables|/Script/Engine.SpringArmComponent|GetSocketOffset _returnvalue_3))
  (bind (_direction _springarm _zoffset) (Timeline|Timeline Reverse)
    (:Update
      (Variables|/Script/Engine.SpringArmComponent|SetTargetArmLength _returnvalue_4 _springarm)
      (Variables|/Script/Engine.SpringArmComponent|SetTargetOffset _returnvalue_4 (Math|Vector|MakeVector (.x _socketoffset) (.y _socketoffset) _zoffset)))))

(event EventBeginPlay)

(event Collision|EventActorBeginOverlap
  (params (OtherActor :type Actor%20Object%20Reference)))

(event EventTick
  (params (DeltaSeconds :type Float%20%28single-precision%29)))

(fn ConstructionScript)