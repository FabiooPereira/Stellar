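; Trigger volume that changes the player's spring arm length and pitch while the player character is inside its Box.
; BeginPlay caches the initial arm length and pitch from the player's spring arm.
; Overlap begin writes the new targets to BP_PlayerJacob and overlap end writes back the cached ones, leaving their application to that Blueprint.
; Older Lerp and Timeline logic that moved the spring arm directly remains unconnected.
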(event OnComponentBeginOverlap(Box)
  (params (OverlappedComponent :type Primitive%20Component%20Object%20Reference) (OtherActor :type Actor%20Object%20Reference) (OtherComp :type Primitive%20Component%20Object%20Reference) (OtherBodyIndex :type Integer) (bFromSweep :type Boolean) (SweepResult :type Hit%20Result%20Structure%20%28by%20ref%29))
  (bind _returnvalue (Game|GetPlayerCharacter 0))
  (if (== OtherActor _returnvalue)
    (bind _asbp_player_jacob (Utilities|Casting|CastToBP_PlayerJacob _returnvalue))
    (Variables|/Game/ThirdPerson/Blueprints/BP_PlayerJacob.BP_PlayerJacob_C|SetNewTargetArmlenght _asbp_player_jacob (Variables|Default|GetNewArmLength))
    (Variables|/Game/ThirdPerson/Blueprints/BP_PlayerJacob.BP_PlayerJacob_C|SetNewTargetRotationY _asbp_player_jacob (Variables|Default|GetNewDegree))))

(event OnComponentEndOverlap(Box)
  (params (OverlappedComponent :type Primitive%20Component%20Object%20Reference) (OtherActor :type Actor%20Object%20Reference) (OtherComp :type Primitive%20Component%20Object%20Reference) (OtherBodyIndex :type Integer))
  (bind _returnvalue (Game|GetPlayerCharacter 0))
  (if (== OtherActor _returnvalue)
    (bind _asbp_player_jacob (Utilities|Casting|CastToBP_PlayerJacob _returnvalue))
    (Variables|/Game/ThirdPerson/Blueprints/BP_PlayerJacob.BP_PlayerJacob_C|SetNewTargetArmlenght _asbp_player_jacob (Variables|Default|GetInitialArmLength))
    (Variables|/Game/ThirdPerson/Blueprints/BP_PlayerJacob.BP_PlayerJacob_C|SetNewTargetRotationY _asbp_player_jacob (Variables|Default|GetInitialDegree))))

(event EventBeginPlay
  (bind _returnvalue (Game|GetPlayerCharacter 0))
  (bind _returnvalue_2 (Actor|GetComponentbyClass _returnvalue "/Script/Engine.SpringArmComponent"))
  (Variables|Default|SetInitialArmLength (Variables|/Script/Engine.SpringArmComponent|GetTargetArmLength _returnvalue_2))
  (Variables|Default|SetInitialDegree (.pitch (Class|SpringArmComponent|GetTargetRotation _returnvalue_2))))

(event Collision|EventActorBeginOverlap
  (params (OtherActor :type Actor%20Object%20Reference)))

(event EventTick
  (params (DeltaSeconds :type Float%20%28single-precision%29)))

(fn ConstructionScript)