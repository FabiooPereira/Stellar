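; Fixed-camera trigger volume that blends the view to its own camera when the player enters, optionally returning to the character on exit.
; Each tick, a spring arm eases along a spline toward the point nearest the player, matching spline rotation.
; The camera can track player yaw or pitch; when tracking, it becomes the character's CustomCamera only once WASD is released inside.
; Construction snaps the camera to a normalized spline position.
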(event OnComponentBeginOverlap(Box)
  (params (OverlappedComponent :type Primitive%20Component%20Object%20Reference) (OtherActor :type Actor%20Object%20Reference) (OtherComp :type Primitive%20Component%20Object%20Reference) (OtherBodyIndex :type Integer) (bFromSweep :type Boolean) (SweepResult :type Hit%20Result%20Structure%20%28by%20ref%29))
  (if (== OtherActor (Game|GetPlayerCharacter 0))
    (Variables|Default|SetIsPlayerInside true)
    (CallFunction|OnFixedCamOverlap)
    (bind _asbp_third_person_character (Utilities|Casting|CastToBP_ThirdPersonCharacter (Game|GetPlayerCharacter 0)))
    (Variables|/Game/ThirdPerson/Blueprints/BP_ThirdPersonCharacter.BP_ThirdPersonCharacter_C|SetLastCameraRef _asbp_third_person_character self)))

(event OnComponentEndOverlap(Box)
  (params (OverlappedComponent :type Primitive%20Component%20Object%20Reference) (OtherActor :type Actor%20Object%20Reference) (OtherComp :type Primitive%20Component%20Object%20Reference) (OtherBodyIndex :type Integer))
  (bind _returnvalue (Game|GetPlayerCharacter 0))
  (if (== OtherActor (Game|GetPlayerCharacter 0))
    (Variables|Default|SetIsPlayerInside false)
    (CallFunction|OnFIxedCamEndOverlap)
    (if (Variables|Default|GetChangeOnExit)
      (Game|Player|SetViewTargetwithBlend (Game|GetPlayerController 0) (Game|GetPlayerCharacter 0) 3.0 "VTBlend_EaseInOut" 2.0 true)
      (bind _asgrupp_onion_character (Utilities|Casting|CastToGruppOnionCharacter (Game|GetPlayerCharacter 0)))
      (Variables|/Script/GruppOnion.GruppOnionCharacter|SetCustomCamera _asgrupp_onion_character (Variables|/Script/GruppOnion.GruppOnionCharacter|GetFollowCamera _asgrupp_onion_character))
      (bind _asbp_third_person_character (Utilities|Casting|CastToBP_ThirdPersonCharacter _returnvalue))
      (Variables|/Game/ThirdPerson/Blueprints/BP_ThirdPersonCharacter.BP_ThirdPersonCharacter_C|SetLastCameraRef _asbp_third_person_character _returnvalue))))

(event EventTick
  (params (DeltaSeconds :type Float%20%28single-precision%29))
  (bind _returnvalue (Game|GetPlayerCharacter 0))
  (bind _returnvalue_2 (Game|GetPlayerCharacter 0))
  (bind _springarm (Variables|Default|GetSpringArm))
  (bind _camera (Variables|Default|GetCamera))
  (bind _camera_2 (Variables|Default|GetCamera))
  (bind _returnvalue_3 (Transformation|GetWorldLocation _camera))
  (bind _returnvalue_4 (Transformation|GetActorLocation _returnvalue))
  (bind _returnvalue_5 (Transformation|GetWorldRotation _camera_2))
  (bind _playerstate (Variables|/Script/Engine.Pawn|GetPlayerState _returnvalue_2))
  (bind _returnvalue_6 (Game|GetPlayerController _playerstate))
  (bind _returnvalue_7 (Math|Rotator|FindLookatRotation _returnvalue_3 _returnvalue_4))
  (Variables|Default|SetDelta%20Seconds DeltaSeconds)
  (CallFunction|SetPlayerCollisionOffset)
  (Transformation|SetWorldLocation (Variables|Default|GetSpringArm) (Math|Interpolation|VInterpTo (Transformation|GetWorldLocation (Variables|Default|GetSpringArm)) (Spline|FindLocationClosesttoWorldLocation (Variables|Default|GetSpline) (Transformation|GetActorLocation (Game|GetPlayerCharacter 0)) "World") (Variables|Default|GetDelta%20Seconds) (Variables|Default|GetInterp%20Speed)) false false)
  (Transformation|SetWorldRotation _springarm (Math|Interpolation|RInterpTo (Transformation|GetWorldRotation _springarm) (Class|SplineComponent|FindRotationClosesttoWorldLocation (Variables|Default|GetSpline) (Transformation|GetWorldLocation (Variables|Default|GetSpringArm)) "World") (Variables|Default|GetDelta%20Seconds) 1e+01) false false)
  (if (or (Variables|Default|GetHorizonatlPlayerFollow) (Variables|Default|GetVerticatlPlayerFollow))
    (Transformation|SetWorldRotation (Variables|Default|GetCamera) (Math|Interpolation|RInterpTo (Transformation|GetWorldRotation (Variables|Default|GetCamera)) (Math|Rotator|MakeRotator (.roll _returnvalue_5) (select (Variables|Default|GetVerticatlPlayerFollow) (.pitch _returnvalue_7) (.pitch _returnvalue_5)) (select (Variables|Default|GetHorizonatlPlayerFollow) (.yaw _returnvalue_7) (.yaw _returnvalue_5))) (Variables|Default|GetDelta%20Seconds) (Variables|Default|GetInterp%20Speed)) false false)
    (if (Variables|Default|GetIsPlayerInside)
      (if (not (Math|Boolean|ORBoolean (Game|Player|IsInputKeyDown _returnvalue_6 "W") (Game|Player|IsInputKeyDown _returnvalue_6 "S") (Game|Player|IsInputKeyDown _returnvalue_6 "A") (Game|Player|IsInputKeyDown _returnvalue_6 "D")))
        (bind _asgrupp_onion_character (Utilities|Casting|CastToGruppOnionCharacter (Game|GetPlayerCharacter 0)))
        (Variables|/Script/GruppOnion.GruppOnionCharacter|SetCustomCamera _asgrupp_onion_character (Variables|Default|GetCamera))))))

(fn ConstructionScript
  (CallFunction|SnaptoSpline)
  (Variables|/Script/Engine.SpringArmComponent|SetTargetArmLength (Variables|Default|GetSpringArm) (Variables|Default|GetSpringArmLenght)))

(fn OnFixedCamOverlap
  (Game|Player|SetViewTargetwithBlend (Game|GetPlayerController 0) self (Variables|Default|GetBlend%20Time) (Variables|Default|GetBlend%20Func) 2.0 true))

(fn SnaptoSpline
  (bind _spline (Variables|Default|GetSpline))
  (bind _camerapoint (Variables|Default|GetCameraPoint))
  (bind _returnvalue (Spline|GetSplineLength _spline))
  (bind _returnvalue_2 (Math|Float|Lerp 0.0 _returnvalue _camerapoint))
  (Transformation|SetWorldTransform (Variables|Default|GetCamera) (Math|Transform|MakeTransform (Spline|GetLocationatDistanceAlongSpline (Variables|Default|GetSpline) _returnvalue_2 "World") (Spline|GetRotationatDistanceAlongSpline (Variables|Default|GetSpline) _returnvalue_2 "World") "1.000000,1.000000,1.000000") false false))

(fn OnFIxedCamEndOverlap)

(fn SetPlayerCollisionOffset
  (Variables|Default|SetPlayerCollisionOffset (select (> (Math|Vector|DotProduct (Math|Vector|GetForwardVector (Variables|Default|GetCamera)) (Transformation|GetActorForwardVector (Game|GetPlayerCharacter 0))) 0.0) (Variables|Default|GetPlayerBackCollisionOffset) (Variables|Default|GetPlayerFrontCollisionOffset))))