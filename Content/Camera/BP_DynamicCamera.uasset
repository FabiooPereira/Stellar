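; BP_DynamicCamera is a placed trigger camera that takes over the player's view while the character overlaps it.
; Each tick its camera rotates to face the player.
; Overlap begin and end set a switch flag, rechecked after a short delay before blending the view to this camera or back to the character.
; Each blend also updates the GruppOnionCharacter's active camera, restoring its follow camera on exit.
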(event EventBeginPlay
  (Variables|Default|SetPlayer%20Character (Game|GetPlayerCharacter 0)))

(event Collision|EventActorBeginOverlap
  (params (OtherActor :type Actor%20Object%20Reference))
  ;[1 1 1] StartOfCollision
  (if (== OtherActor (Variables|Default|GetPlayer%20Character))
    (Variables|Default|SetCamera%20Switch true)
    (Utilities|FlowControl|Delay 1.0)
    (if (Variables|Default|GetCamera%20Switch)
      (Game|Player|SetViewTargetwithBlend (Game|GetPlayerController 0) self 1.0 "VTBlend_EaseIn" 2.0 false)
      (bind _asgrupp_onion_character (Utilities|Casting|CastToGruppOnionCharacter (Variables|Default|GetPlayer%20Character)))
      (Class|GruppOnionCharacter|SetActiveCamera _asgrupp_onion_character (Variables|CameraActor|GetCameraComponent)))))

(event EventTick
  (params (DeltaSeconds :type Float%20%28single-precision%29))
  (Transformation|SetWorldRotation (Variables|CameraActor|GetCameraComponent) (Math|Rotator|FindLookatRotation (Transformation|GetWorldLocation (Variables|CameraActor|GetCameraComponent)) (Transformation|GetActorLocation (Game|GetPlayerCharacter 0))) false false))

(event Collision|EventActorEndOverlap
  (params (OtherActor :type Actor%20Object%20Reference))
  ;[1 1 1] EndOfCollision
  (if (== OtherActor (Variables|Default|GetPlayer%20Character))
    (Variables|Default|SetCamera%20Switch false)
    (Utilities|FlowControl|Delay 1.0)
    (if (not (Variables|Default|GetCamera%20Switch))
      (Actor|GetActorOfClass "/Game/Camera/BP_TracingCamera.BP_TracingCamera_C")
      (Game|Player|SetViewTargetwithBlend (Game|GetPlayerController 0) (Game|GetPlayerCharacter 0) 0.5 "VTBlend_EaseOut" 2.0 false)
      (bind _asgrupp_onion_character (Utilities|Casting|CastToGruppOnionCharacter (Variables|Default|GetPlayer%20Character)))
      (Class|GruppOnionCharacter|SetActiveCamera _asgrupp_onion_character (Variables|/Script/GruppOnion.GruppOnionCharacter|GetFollowCamera _asgrupp_onion_character)))))

(fn ConstructionScript)