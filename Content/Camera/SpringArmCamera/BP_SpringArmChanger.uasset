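; Trigger volume that changes the player's camera spring arm length and height while the player is inside its box.
; BeginPlay caches the initial arm length and Z offset, then derives a new Z offset for the new length that preserves their angle.
; Box overlaps set inside/exit flags, and Tick lerps toward the new values or back to the initial ones until the offset is nearly restored.
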(event OnComponentBeginOverlap(Box)
  (params (OverlappedComponent :type Primitive%20Component%20Object%20Reference) (OtherActor :type Actor%20Object%20Reference) (OtherComp :type Primitive%20Component%20Object%20Reference) (OtherBodyIndex :type Integer) (bFromSweep :type Boolean) (SweepResult :type Hit%20Result%20Structure%20%28by%20ref%29))
  (if (== OtherActor (Game|GetPlayerCharacter 0))
    (Variables|Default|SetIsInside true)
    (Variables|Default|SetWentOut false)))

(event OnComponentEndOverlap(Box)
  (params (OverlappedComponent :type Primitive%20Component%20Object%20Reference) (OtherActor :type Actor%20Object%20Reference) (OtherComp :type Primitive%20Component%20Object%20Reference) (OtherBodyIndex :type Integer))
  (if (== OtherActor (Game|GetPlayerCharacter 0))
    (Variables|Default|SetIsInside false)
    (Variables|Default|SetWentOut true)))

(event EventBeginPlay
  (bind _returnvalue (Game|GetPlayerCharacter 0))
  (bind _returnvalue_2 (Actor|GetComponentbyClass _returnvalue "/Script/Engine.SpringArmComponent"))
  (bind _output_get (Variables|Default|SetInitialArmLength (Variables|/Script/Engine.SpringArmComponent|GetTargetArmLength _returnvalue_2)))
  (bind _output_get_2 (Variables|Default|SetInitialSpringArmOffsetZ (.z (Variables|/Script/Engine.SpringArmComponent|GetTargetOffset _returnvalue_2))))
  (Variables|Default|SetDegrees (Class|KismetMathLibrary|DegAtan (/ _output_get_2 _output_get)))
  (Variables|Default|SetNewSpringArmOffsetZ (* (Math|Trig|Tan(Degrees) (Variables|Default|GetDegrees)) (Variables|Default|GetNewArmLength))))

(event Collision|EventActorBeginOverlap
  (params (OtherActor :type Actor%20Object%20Reference)))

(event EventTick
  (params (DeltaSeconds :type Float%20%28single-precision%29))
  (bind _returnvalue (Game|GetPlayerCharacter 0))
  (bind _returnvalue_2 (Game|GetPlayerCharacter 0))
  (bind _power (Variables|Default|GetPower))
  (bind _returnvalue_3 (Actor|GetComponentbyClass _returnvalue "/Script/Engine.SpringArmComponent"))
  (bind _returnvalue_4 (Actor|GetComponentbyClass _returnvalue_2 "/Script/Engine.SpringArmComponent"))
  (bind _returnvalue_5 (* DeltaSeconds _power))
  (if (Variables|Default|GetIsInside)
    (Variables|/Script/Engine.SpringArmComponent|SetTargetOffset _returnvalue_3 (Math|Vector|MakeVector 0.0 0.0 (Math|Float|Lerp (.z (Variables|/Script/Engine.SpringArmComponent|GetTargetOffset (Actor|GetComponentbyClass (Game|GetPlayerCharacter 0) "/Script/Engine.SpringArmComponent"))) (Variables|Default|GetNewSpringArmOffsetZ) _returnvalue_5)))
    (Variables|/Script/Engine.SpringArmComponent|SetTargetArmLength _returnvalue_3 (Math|Float|Lerp (Variables|/Script/Engine.SpringArmComponent|GetTargetArmLength _returnvalue_3) (Variables|Default|GetNewArmLength) _returnvalue_5))
    (elif (Variables|Default|GetWentOut)
      (Variables|/Script/Engine.SpringArmComponent|SetTargetArmLength _returnvalue_4 (Math|Float|Lerp (Variables|/Script/Engine.SpringArmComponent|GetTargetArmLength _returnvalue_4) (Variables|Default|GetInitialArmLength) _returnvalue_5))
      (Variables|/Script/Engine.SpringArmComponent|SetTargetOffset _returnvalue_4 (Math|Vector|MakeVector 0.0 0.0 (Math|Float|Lerp (.z (Variables|/Script/Engine.SpringArmComponent|GetTargetOffset (Actor|GetComponentbyClass (Game|GetPlayerCharacter 0) "/Script/Engine.SpringArmComponent"))) (Variables|Default|GetInitialSpringArmOffsetZ) _returnvalue_5)))
      (if (Math|Float|NearlyEqual(Float) (Variables|Default|GetInitialSpringArmOffsetZ) (Math|Float|Lerp (.z (Variables|/Script/Engine.SpringArmComponent|GetTargetOffset (Actor|GetComponentbyClass (Game|GetPlayerCharacter 0) "/Script/Engine.SpringArmComponent"))) (Variables|Default|GetInitialSpringArmOffsetZ) _returnvalue_5) 1e+01)
        (Variables|Default|SetWentOut false)))))

(fn ConstructionScript)