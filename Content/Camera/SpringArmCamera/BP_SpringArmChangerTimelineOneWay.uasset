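; A one-way camera trigger box that changes the player's spring arm length and pitch on entry.
; On player overlap, a timeline eases the arm from its current values toward the new length and angle, with yaw fixed at -90.
; Exit updates the overlap list and checks for the on-foot and mounted players but restores nothing.
; The initial arm values saved at BeginPlay go unused.
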(event OnComponentBeginOverlap(Box)
  (params (OverlappedComponent :type Primitive%20Component%20Object%20Reference) (OtherActor :type Actor%20Object%20Reference) (OtherComp :type Primitive%20Component%20Object%20Reference) (OtherBodyIndex :type Integer) (bFromSweep :type Boolean) (SweepResult :type Hit%20Result%20Structure%20%28by%20ref%29))
  (bind _returnvalue (Game|GetPlayerCharacter 0))
  (bind _returnvalue_2 (Actor|GetComponentbyClass _returnvalue "/Script/Engine.SpringArmComponent"))
  ;[1 1 1] Adds actors into an Array
  (Utilities|Array|Add (Variables|Default|GetInsideActors) OtherActor)
  ;[1 1 1] Checks if player is overlaping
  (if (== OtherActor (Game|GetPlayerCharacter 0))
    ;[1 1 1] Changes players springarm values
    (bind _newtrack_0 (Timeline|Timeline PlayFromStart)
      (:Update
        (Variables|/Script/Engine.SpringArmComponent|SetTargetArmLength _returnvalue_2 (Math|Float|Lerp (Variables|/Script/Engine.SpringArmComponent|GetTargetArmLength _returnvalue_2) (Variables|Default|GetNewArmLength) _newtrack_0))
        (Transformation|SetRelativeRotation _returnvalue_2 (Math|Rotator|Lerp(Rotator) (Math|Rotator|MakeRotator 0.0 (.pitch (.rotation (Transformation|GetRelativeTransform _returnvalue_2))) -9e+01) (Math|Rotator|MakeRotator 0.0 (Variables|Default|GetNewDegree) -9e+01) _newtrack_0 true) false false)))))

(event OnComponentEndOverlap(Box)
  (params (OverlappedComponent :type Primitive%20Component%20Object%20Reference) (OtherActor :type Actor%20Object%20Reference) (OtherComp :type Primitive%20Component%20Object%20Reference) (OtherBodyIndex :type Integer))
  (bind _insideactors (Variables|Default|GetInsideActors))
  ;[1 1 1] Checks if both mountedplayer and unmountedplayer is outside the triggerbox
  (Utilities|FlowControl|DelayUntilNextTick)
  (Utilities|Array|RemoveItem (Variables|Default|GetInsideActors) OtherActor)
  (bind _returnvalue (Actor|GetActorOfClass "/Game/ThirdPerson/Blueprints/BP_PlayerJacob.BP_PlayerJacob_C"))
  (bind _returnvalue_2 (Actor|GetActorOfClass "/Game/ThirdPerson/Blueprints/BP_Player_Mounted.BP_Player_Mounted_C"))
  (if (or (Utilities|Array|ContainsItem _insideactors _returnvalue) (Utilities|Array|ContainsItem _insideactors _returnvalue_2))
    _))

(event EventBeginPlay
  (bind _returnvalue (Game|GetPlayerCharacter 0))
  (bind _returnvalue_2 (Actor|GetComponentbyClass _returnvalue "/Script/Engine.SpringArmComponent"))
  ;[1 1 1] Get InitialPlayerSpringArmValues
  (Variables|Default|SetInitialArmLength (Variables|/Script/Engine.SpringArmComponent|GetTargetArmLength _returnvalue_2))
  (Variables|Default|SetInitialDegree (.pitch (Class|SpringArmComponent|GetTargetRotation _returnvalue_2))))

(event Collision|EventActorBeginOverlap
  (params (OtherActor :type Actor%20Object%20Reference)))

(event EventTick
  (params (DeltaSeconds :type Float%20%28single-precision%29)))

(fn ConstructionScript)