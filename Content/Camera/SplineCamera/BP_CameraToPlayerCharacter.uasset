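; Trigger actor that returns the view from a custom camera to the player's own character camera when the player character overlaps it.
; On overlap it blends the player controller's view target to the character with an ease-in-out over a configurable blend time, locking the outgoing view.
; It then resets the GruppOnionCharacter's CustomCamera to its FollowCamera and records the character as BP_ThirdPersonCharacter's LastCameraRef.
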(event EventBeginPlay)

(event Collision|EventActorBeginOverlap
  (params (OtherActor :type Actor%20Object%20Reference))
  (bind _returnvalue (Game|GetPlayerCharacter 0))
  ;[1 1 1] Sets Camera view back to players lokal camera
  (if (== _returnvalue OtherActor)
    (Game|Player|SetViewTargetwithBlend (Game|GetPlayerController 0) _returnvalue (Variables|Default|GetBlendTIme) "VTBlend_EaseInOut" 2.0 true)
    (bind _asgrupp_onion_character (Utilities|Casting|CastToGruppOnionCharacter (Game|GetPlayerCharacter 0)))
    (Variables|/Script/GruppOnion.GruppOnionCharacter|SetCustomCamera _asgrupp_onion_character (Variables|/Script/GruppOnion.GruppOnionCharacter|GetFollowCamera _asgrupp_onion_character))
    (bind _asbp_third_person_character (Utilities|Casting|CastToBP_ThirdPersonCharacter OtherActor))
    (Variables|/Game/ThirdPerson/Blueprints/BP_ThirdPersonCharacter.BP_ThirdPersonCharacter_C|SetLastCameraRef _asbp_third_person_character OtherActor)))

(event EventTick
  (params (DeltaSeconds :type Float%20%28single-precision%29)))

(fn ConstructionScript)