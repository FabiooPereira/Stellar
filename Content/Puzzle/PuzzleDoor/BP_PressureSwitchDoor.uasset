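; Pressure switch for a puzzle that tells its linked DoorToActivate when it is activated or deactivated.
; Entering the overlap box activates the door and plays a timeline that moves the switch along Z; leaving deactivates it and reverses the timeline.
; An unconnected snap routine, marked buggy, would capsule-trace for a BP_ForceResponsiveObject, detach it and align it to the switch.
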(event OnComponentBeginOverlap(OverlapBox)
  (params (OverlappedComponent :type Primitive%20Component%20Object%20Reference) (OtherActor :type Actor%20Object%20Reference) (OtherComp :type Primitive%20Component%20Object%20Reference) (OtherBodyIndex :type Integer) (bFromSweep :type Boolean) (SweepResult :type Hit%20Result%20Structure%20%28by%20ref%29))
  ;[1 1 1] Switch Trigger
  (Default|SwitchActivatedDoor (Variables|Default|GetDoorToActivate))
  (bind _switchposition (Timeline|Timeline Play)
    (:Update
      (Transformation|SetRelativeLocation (Variables|Default|GetSwitch) (Math|Vector|MakeVector 0.0 0.0 _switchposition) false false))))

(event OnComponentEndOverlap(OverlapBox)
  (params (OverlappedComponent :type Primitive%20Component%20Object%20Reference) (OtherActor :type Actor%20Object%20Reference) (OtherComp :type Primitive%20Component%20Object%20Reference) (OtherBodyIndex :type Integer))
  ;[1 1 1] Switch Trigger
  (Default|SwitchDeactivatedDoor (Variables|Default|GetDoorToActivate))
  (bind _switchposition (Timeline|Timeline Reverse)
    (:Update
      (Transformation|SetRelativeLocation (Variables|Default|GetSwitch) (Math|Vector|MakeVector 0.0 0.0 _switchposition) false false))))

(event EventBeginPlay)

(event EventTick
  (params (DeltaSeconds :type Float%20%28single-precision%29)))

(fn ConstructionScript)

(fn ComponentIsChild
  (params (Component :type Actor%20Object%20Reference%20%28by%20ref%29))
  (return (== (Actor|GetParentActor Component) self)))