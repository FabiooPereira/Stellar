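; Puzzle lever that, when interacted with, activates a referenced stone wall and rotates its handle on the X axis through a timeline.
; SetInteractableState swaps the lever material to show whether it can be used, while Tick keeps the non-interactable material applied once the switch is activated.
; An unused snap routine, marked buggy, would capsule-trace for a BP_ForceResponsiveObject, detach it and move it onto the lever.
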(event EventBeginPlay)

(event EventInteract
  (params (Instigator :type Actor%20Object%20Reference))
  ;[1 1 1] Switch Trigger
  (Variables|Default|SetSwitchActivated true)
  (Default|LeverActivatedStoneWall (Variables|Default|GetStoneWallToActivate))
  (bind _switchposition (Timeline|Timeline Play)
    (:Update
      (Transformation|SetRelativeRotation (Variables|Default|GetLever) (Math|Rotator|MakeRotator _switchposition 0.0 0.0) false false))))

(event EventTick
  (params (DeltaSeconds :type Float%20%28single-precision%29))
  (if (Variables|Default|GetSwitchActivated)
    (Rendering|Material|SetMaterial (Variables|Default|GetLever) 0 "/Engine/EngineMaterials/WorldGridMaterial_Low.WorldGridMaterial_Low")))

(event EventSetInteractableState
  (params (bCanShowInteract? :type Boolean))
  (bind _lever (Variables|Default|GetLever))
  (bind _output_get (Variables|Default|SetbCanInteract? bCanShowInteract?))
  (if _output_get
    (Rendering|Material|SetMaterial _lever 0 "/Engine/MapTemplates/Materials/BasicAsset01.BasicAsset01")
    (else
      (Rendering|Material|SetMaterial _lever 0 "/Engine/EngineMaterials/WorldGridMaterial_Low.WorldGridMaterial_Low"))))

(fn ConstructionScript)

(fn ComponentIsChild
  (params (Component :type Actor%20Object%20Reference%20%28by%20ref%29))
  (return (== (Actor|GetParentActor Component) self)))