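; BP_LampStart is an interactable lamp that trades light with BP_PlayerJacob, taking it when the player has light and giving it back otherwise.
; One timeline, played forward or reversed, moves a Niagara transfer effect between player and lamp.
; On finish it updates player light and lamp state, then broadcasts ChangesState; material swaps mark the change.
; Interactable focus toggles a custom-depth highlight and a "Collect Light" HUD prompt.
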(event EventTick
  (params (DeltaSeconds :type Float%20%28single-precision%29)))

(event EventSetInteractableState
  (params (bCanShowInteract :type Boolean))
  (bind _lampa (Variables|Default|GetLampa))
  (if bCanShowInteract
    (Rendering|SetRenderCustomDepth _lampa true)
    (CallFunction|TextEnable)
    (else
      (Rendering|SetRenderCustomDepth _lampa false)
      (CallFunction|TextDisable))))

(event EventInteract
  (params (Instigator :type Actor%20Object%20Reference))
  (bind _asbp_player_jacob (Utilities|Casting|CastToBP_PlayerJacob Instigator))
  (Variables|Default|SetPlayer _asbp_player_jacob)
  (if (Variables|/Game/ThirdPerson/Blueprints/BP_PlayerJacob.BP_PlayerJacob_C|GetHasLight _asbp_player_jacob)
    (if (not (Variables|Default|GetLampIsLIt))
      (Variables|Default|SetIsLit true)
      (bind _returnvalue (Niagara|SpawnSystematLocation "/Game/Kio/Particles/FXS_LightTransfer.FXS_LightTransfer" (Math|Vector|MakeVector (+ (.x (Transformation|GetWorldLocation (Variables|/Script/Engine.Actor|GetRootComponent (Variables|Default|GetPlayer)))) 1e+01) (+ (.y (Transformation|GetWorldLocation (Variables|/Script/Engine.Actor|GetRootComponent (Variables|Default|GetPlayer)))) 1e+01) (+ (.z (Transformation|GetWorldLocation (Variables|/Script/Engine.Actor|GetRootComponent (Variables|Default|GetPlayer)))) 4e+01)) "0, 0, 0" "1.000000,1.000000,1.000000" false))
      (Variables|Default|SetParticle _returnvalue)
      (bind _time (Timeline|LIghtTransfer Play)
        (:Update
          (Transformation|SetWorldLocation (Variables|Default|GetParticle) (Math|Vector|Lerp(Vector) (Math|Vector|MakeVector (.x (Transformation|GetWorldLocation (Variables|/Script/Engine.Actor|GetRootComponent (Variables|Default|GetPlayer)))) (.y (Transformation|GetWorldLocation (Variables|/Script/Engine.Actor|GetRootComponent (Variables|Default|GetPlayer)))) (+ (.z (Transformation|GetWorldLocation (Variables|/Script/Engine.Actor|GetRootComponent (Variables|Default|GetPlayer)))) 4e+01)) (Transformation|GetWorldLocation (Variables|Default|GetLampa)) _time) false false))
        (:Finished
          (Components|DestroyComponent (Variables|Default|GetParticle))
          (if (Variables|Default|GetIsLit)
            (Rendering|Material|SetMaterial (Variables|Default|GetStaticMesh) 0 "/Engine/EngineMaterials/DefaultLightFunctionMaterial.DefaultLightFunctionMaterial")
            (Default|LightDown (Variables|Default|GetPlayer))
            (Variables|Default|SetLampIsLIt true)
            (else
              (Default|LightUp (Variables|Default|GetPlayer))
              (Variables|Default|SetLampIsLIt false)))
          (Default|CallChangesState (Variables|Default|GetLampIsLIt)))))
    (elif (Variables|Default|GetLampIsLIt)
      (Variables|Default|SetIsLit false)
      (Rendering|Material|SetMaterial (Variables|Default|GetStaticMesh) 0 "/Game/Materials/Characters/Stella_Emissive.Stella_Emissive")
      (bind _returnvalue_2 (Niagara|SpawnSystematLocation "/Game/Kio/Particles/FXS_LightTransfer.FXS_LightTransfer" (Transformation|GetWorldLocation (Variables|Default|GetLampa)) "0, 0, 0" "1.000000,1.000000,1.000000" false))
      (Variables|Default|SetParticle _returnvalue_2)
      (Timeline|LIghtTransfer Reverse))))

(fn ConstructionScript)

(fn LitLamp)

(fn TextEnable
  (bind _asnew_hud (Utilities|Casting|CastToNewHUD (HUD|GetHUD (Game|GetPlayerController 0))))
  (bind _output_get (Variables|Default|SetAs%20New%20HUD _asnew_hud))
  (Default|SetTextInput (Variables|/Game/Jacob/UI/NewHUD.NewHUD_C|GetUIRef _output_get) "COLLECT LIGHT: B" "COLLECT LIGHT: E" true))

(fn TextDisable
  (bind _as_new_hud (Variables|Default|GetAs%20New%20HUD)
    (:then
      (Default|SetTextInput (Variables|/Game/Jacob/UI/NewHUD.NewHUD_C|GetUIRef _as_new_hud) "" "" false))
    (:else)))