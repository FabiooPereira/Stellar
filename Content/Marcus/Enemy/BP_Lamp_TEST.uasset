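; Test version of an interactable lamp that BP_PlayerJacob can pass light to or take it back from.
; Interact plays a timeline forward or reversed to move a particle between player and lamp, updating material, player light and lit state.
; DestroyLight starts a second timeline whose frequency track times FlipFlopLight's flickering until the lamp turns off.
; Focus toggles a custom-depth outline and HUD prompt, while Tick yaws the text toward the camera.
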(event Custom|DestroyLight
  (bind _player (Variables|Default|GetPlayer))
  (bind _player_2 (Variables|Default|GetPlayer))
  (bind _rootcomponent (Variables|/Script/Engine.Actor|GetRootComponent _player))
  (bind _rootcomponent_2 (Variables|/Script/Engine.Actor|GetRootComponent _player_2))
  (bind _returnvalue (Transformation|GetWorldLocation _rootcomponent))
  (bind _returnvalue_2 (Transformation|GetWorldLocation _rootcomponent_2))
  (bind _frequency (Timeline|DestructionTimer PlayFromStart)
    (:Update
      (if (not (Class|KismetSystemLibrary|IsTimerActive 0 "FlipFlopLight"))
        (Utilities|Time|SetTimerbyFunctionName 0 "FlipFlopLight" _frequency)))
    (:Finished
      (Utilities|Time|ClearTimerbyFunctionName 0 "FlipFlopLight")
      (Rendering|Material|SetMaterial (Variables|Default|GetStaticMesh) 0 "/Game/Materials/Characters/Stella_Emissive.Stella_Emissive")
      (Development|PrintString "off 2")
      (if (Variables|/Game/ThirdPerson/Blueprints/BP_PlayerJacob.BP_PlayerJacob_C|GetHasLight (Variables|Default|GetPlayer))
        (if (not (Variables|Default|GetLampIsLIt))
          (Variables|Default|SetIsLit true)
          (bind _returnvalue_3 (Niagara|SpawnSystematLocation "/Game/Kio/Particles/FXS_LightTransfer.FXS_LightTransfer" (Math|Vector|MakeVector (+ (.x _returnvalue) 1e+01) (+ (.y _returnvalue) 1e+01) (+ (.z _returnvalue) 4e+01)) "0, 0, 0" "1.000000,1.000000,1.000000" false))
          (Variables|Default|SetParticle _returnvalue_3)
          (bind _time (Timeline|LIghtTransfer Play)
            (:Update
              (Transformation|SetWorldLocation (Variables|Default|GetParticle) (Math|Vector|Lerp(Vector) (Math|Vector|MakeVector (.x _returnvalue_2) (.y _returnvalue_2) (+ (.z _returnvalue_2) 4e+01)) (Transformation|GetWorldLocation (Variables|Default|GetLampa)) _time) false false))
            (:Finished
              (Components|DestroyComponent (Variables|Default|GetParticle))
              (if (Variables|Default|GetIsLit)
                (Rendering|Material|SetMaterial (Variables|Default|GetStaticMesh) 0 "/Engine/EngineMaterials/DefaultLightFunctionMaterial.DefaultLightFunctionMaterial")
                (Default|LightDown (Variables|Default|GetPlayer))
                (Variables|Default|SetLampIsLIt true)
                (else
                  (Default|LightUp (Variables|Default|GetPlayer))
                  (Variables|Default|SetLampIsLIt false)))
              (Default|CallChangesState (Variables|Default|GetLampIsLIt)))))
        (elif (Variables|Default|GetLampIsLIt)
          (Variables|Default|SetIsLit false)
          (bind _returnvalue_4 (Niagara|SpawnSystematLocation "/Game/Kio/Particles/FXS_LightTransfer.FXS_LightTransfer" (Transformation|GetWorldLocation (Variables|Default|GetLampa)) "0, 0, 0" "1.000000,1.000000,1.000000" false))
          (Variables|Default|SetParticle _returnvalue_4)
          (Utilities|FlowControl|Sequence
            (:then_0
              (Timeline|DestructionTimer Stop))
            (:then_1
              (Rendering|Material|SetMaterial (Variables|Default|GetStaticMesh) 0 "/Game/Materials/Characters/Stella_Emissive.Stella_Emissive"))
            (:then_2
              (Timeline|LIghtTransfer Reverse))))))))

(event EventTick
  (params (DeltaSeconds :type Float%20%28single-precision%29))
  (Transformation|SetWorldRotation (Variables|Default|GetTextRender) (Math|Rotator|MakeRotator 0.0 0.0 (.yaw (Math|Rotator|FindLookatRotation (Transformation|GetSocketLocation (Variables|Default|GetTextRender) "None") (Transformation|GetActorLocation (Game|GetPlayerCameraManager 0))))) false false))

(event EventSetInteractableState
  (params (bCanShowInteract :type Boolean))
  (bind _staticmesh (Variables|Default|GetStaticMesh))
  (if bCanShowInteract
    (Rendering|SetRenderCustomDepth _staticmesh true)
    (CallFunction|TextEnable)
    (else
      (Rendering|SetRenderCustomDepth _staticmesh false)
      (CallFunction|TextDisable))))

(event EventInteract
  (params (Instigator :type Actor%20Object%20Reference))
  (bind _asbp_player_jacob (Utilities|Casting|CastToBP_PlayerJacob Instigator))
  (Variables|Default|SetPlayer _asbp_player_jacob)
  (Utilities|Time|ClearTimerbyFunctionName 0 "FlipFlopLight")
  (if (Variables|/Game/ThirdPerson/Blueprints/BP_PlayerJacob.BP_PlayerJacob_C|GetHasLight (Variables|Default|GetPlayer)) :!label _label
    (if (not (Variables|Default|GetLampIsLIt))
      (Variables|Default|SetIsLit true)
      (bind _returnvalue (Niagara|SpawnSystematLocation "/Game/Kio/Particles/FXS_LightTransfer.FXS_LightTransfer" (Math|Vector|MakeVector (+ (.x (Transformation|GetWorldLocation (Variables|/Script/Engine.Actor|GetRootComponent (Variables|Default|GetPlayer)))) 1e+01) (+ (.y (Transformation|GetWorldLocation (Variables|/Script/Engine.Actor|GetRootComponent (Variables|Default|GetPlayer)))) 1e+01) (+ (.z (Transformation|GetWorldLocation (Variables|/Script/Engine.Actor|GetRootComponent (Variables|Default|GetPlayer)))) 4e+01)) "0, 0, 0" "1.000000,1.000000,1.000000" false))
      (Variables|Default|SetParticle _returnvalue)
      (bind _time (Timeline|LIghtTransfer Play)
        (:Update
          (Transformation|SetWorldLocation (Variables|Default|GetParticle) (Math|Vector|Lerp(Vector) (Math|Vector|MakeVector (.x (Transformation|GetWorldLocation (Variables|/Script/Engine.Actor|GetRootComponent (Variables|Default|GetPlayer)))) (.y (Transformation|GetWorldLocation (Variables|/Script/Engine.Actor|GetRootComponent (Variables|Default|GetPlayer)))) (+ (.z (Transformation|GetWorldLocation (Variables|/Script/Engine.Actor|GetRootComponent (Variables|Default|GetPlayer)))) 4e+01)) (Transformation|GetWorldLocation (Variables|Default|GetLampa)) _time) false false))
        (:Finished
          (Components|DestroyComponent (Variables|Default|GetParticle))
          (if (Variables|Default|GetIsLit)
            (Rendering|Material|SetMaterial (Variables|Default|GetStaticMesh) 0 "/Engine/EngineMaterials/DefaultLightFunctionMaterial.DefaultLightFunctionMaterial")
            (Default|LightDown (Variables|Default|GetPlayer))
            (Variables|Default|SetLampIsLIt true)
            (else
              (Default|LightUp (Variables|Default|GetPlayer))
              (Variables|Default|SetLampIsLIt false)))
          (Default|CallChangesState (Variables|Default|GetLampIsLIt)))))
    (elif (Variables|Default|GetLampIsLIt)
      (Variables|Default|SetIsLit false)
      (bind _returnvalue_2 (Niagara|SpawnSystematLocation "/Game/Kio/Particles/FXS_LightTransfer.FXS_LightTransfer" (Transformation|GetWorldLocation (Variables|Default|GetLampa)) "0, 0, 0" "1.000000,1.000000,1.000000" false))
      (Variables|Default|SetParticle _returnvalue_2)
      (Utilities|FlowControl|Sequence
        (:then_0
          (bind _frequency (Timeline|DestructionTimer Stop)
            (:Update
              (if (not (Class|KismetSystemLibrary|IsTimerActive 0 "FlipFlopLight"))
                (Utilities|Time|SetTimerbyFunctionName 0 "FlipFlopLight" _frequency)))
            (:Finished
              (Utilities|Time|ClearTimerbyFunctionName 0 "FlipFlopLight")
              (Rendering|Material|SetMaterial (Variables|Default|GetStaticMesh) 0 "/Game/Materials/Characters/Stella_Emissive.Stella_Emissive")
              (Development|PrintString "off 2")
              (goto _label))))
        (:then_1
          (Rendering|Material|SetMaterial (Variables|Default|GetStaticMesh) 0 "/Game/Materials/Characters/Stella_Emissive.Stella_Emissive"))
        (:then_2
          (Timeline|LIghtTransfer Reverse))))))

(fn ConstructionScript)

(fn LitLamp)

(fn TextEnable
  (bind _asnew_hud (Utilities|Casting|CastToNewHUD (HUD|GetHUD (Game|GetPlayerController 0))))
  (bind _output_get (Variables|Default|SetAs%20New%20HUD _asnew_hud))
  (Default|SetTextInput (Variables|/Game/Jacob/UI/NewHUD.NewHUD_C|GetUIRef _output_get) "TRANSFER LIGHT: B" "TRANSFER LIGHT: E" true))

(fn TextDisable
  (bind _as_new_hud (Variables|Default|GetAs%20New%20HUD)
    (:then
      (Default|SetTextInput (Variables|/Game/Jacob/UI/NewHUD.NewHUD_C|GetUIRef _as_new_hud) "" "" false))
    (:else)))

(fn FlipFlopLight
  (if (Variables|Default|GetPrevStatus)
    (Variables|Default|SetPrevStatus false)
    (Rendering|Material|SetMaterial (Variables|Default|GetStaticMesh) 0 "/Game/Materials/Characters/Stella_Emissive.Stella_Emissive")
    (Development|PrintString "off")
    (else
      (Variables|Default|SetPrevStatus true)
      (Rendering|Material|SetMaterial (Variables|Default|GetStaticMesh) 0 "/Engine/EngineMaterials/DefaultLightFunctionMaterial.DefaultLightFunctionMaterial")
      (Development|PrintString "on"))))