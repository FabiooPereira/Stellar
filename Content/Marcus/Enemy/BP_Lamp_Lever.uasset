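; Interactable lamp that swaps a single light back and forth with the player, acting as a lever that broadcasts its lit state.
; Interacting plays or reverses one timeline that moves a Niagara effect between player and lamp.
; The lamp's material darkens as light leaves or brightens on arrival, when the player's light and dispatched state also update.
; A prompt text, toggled by interactable state, yaws toward the camera every tick.
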(event EventTick
  (params (DeltaSeconds :type Float%20%28single-precision%29))
  (Transformation|SetWorldRotation (Variables|Default|GetTextRender) (Math|Rotator|MakeRotator 0.0 0.0 (.yaw (Math|Rotator|FindLookatRotation (Transformation|GetSocketLocation (Variables|Default|GetTextRender) "None") (Transformation|GetActorLocation (Game|GetPlayerCameraManager 0))))) false false))

(event EventSetInteractableState
  (params (bCanShowInteract :type Boolean))
  (bind _textrender (Variables|Default|GetTextRender))
  (if bCanShowInteract
    (Rendering|SetVisibility _textrender true false)
    (else
      (Rendering|SetVisibility _textrender false false))))

(event EventInteract
  (params (Instigator :type Actor%20Object%20Reference))
  (bind _asbp_player_jacob (Utilities|Casting|CastToBP_PlayerJacob Instigator))
  (Variables|Default|SetPlayer _asbp_player_jacob)
  (if (Variables|/Game/ThirdPerson/Blueprints/BP_PlayerJacob.BP_PlayerJacob_C|GetHasLight _asbp_player_jacob)
    (if (not (Variables|Default|GetLampIsLIt))
      (Variables|Default|SetIsLit true)
      (bind _returnvalue (Niagara|SpawnSystematLocation "/Game/Kio/Particles/FXS_LightTransfer.FXS_LightTransfer" (Math|Vector|MakeVector (+ (.x (Transformation|GetWorldLocation (Variables|/Script/Engine.Actor|GetRootComponent (Variables|Default|GetPlayer)))) 1e+01) (+ (.y (Transformation|GetWorldLocation (Variables|/Script/Engine.Actor|GetRootComponent (Variables|Default|GetPlayer)))) 1e+01) (+ (.z (Transformation|GetWorldLocation (Variables|/Script/Engine.Actor|GetRootComponent (Variables|Default|GetPlayer)))) 4e+01)) "0, 0, 0" "1.000000,1.000000,1.000000" false))
      (Variables|Default|SetParticle _returnvalue)
      (bind _time (Timeline|LIghtTransfer Play)
        (:Update
          (Transformation|SetWorldLocation (Variables|Default|GetParticle) (Math|Vector|Lerp(Vector) (Math|Vector|MakeVector (.x (Transformation|GetWorldLocation (Variables|/Script/Engine.Actor|GetRootComponent (Variables|Default|GetPlayer)))) (.y (Transformation|GetWorldLocation (Variables|/Script/Engine.Actor|GetRootComponent (Variables|Default|GetPlayer)))) (+ (.z (Transformation|GetWorldLocation (Variables|/Script/Engine.Actor|GetRootComponent (Variables|Default|GetPlayer)))) 4e+01)) (Transformation|GetWorldLocation (Variables|Default|GetLampa)) _time) false false))
        (:Finished
          (Components|DestroyComponent (Variables|Default|GetParticle))
          (if (Variables|Default|GetIsLit)
            (Rendering|Material|SetMaterial (Variables|Default|GetLampa) 0 "/DatasmithContent/Materials/Arealight.Arealight")
            (Default|LightDown (Variables|Default|GetPlayer))
            (Variables|Default|SetLampIsLIt true)
            (else
              (Default|LightUp (Variables|Default|GetPlayer))
              (Variables|Default|SetLampIsLIt false)))
          (Default|CallChangesState (Variables|Default|GetLampIsLIt)))))
    (elif (Variables|Default|GetLampIsLIt)
      (Variables|Default|SetIsLit false)
      (Rendering|Material|SetMaterial (Variables|Default|GetLampa) 0 "/Engine/EngineMeshes/BackgroundMaterial.BackgroundMaterial")
      (bind _returnvalue_2 (Niagara|SpawnSystematLocation "/Game/Kio/Particles/FXS_LightTransfer.FXS_LightTransfer" (Transformation|GetWorldLocation (Variables|Default|GetLampa)) "0, 0, 0" "1.000000,1.000000,1.000000" false))
      (Variables|Default|SetParticle _returnvalue_2)
      (Timeline|LIghtTransfer Reverse))))

(fn ConstructionScript)

(fn LitLamp)