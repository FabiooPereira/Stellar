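; BP_Rock is a rock actor in the Enemy folder that detects hits on lamps.
; When it hits a BP_Lamp_TEST, it calls the HitTarget dispatcher, stops the rock's physics, restarts a Niagara effect, hides the mesh and destroys itself after a short delay.
; Hits on anything else only print a debug miss message and leave the rock in play.
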(event Collision|EventHit
  (params (MyComp :type Primitive%20Component%20Object%20Reference) (Other :type Actor%20Object%20Reference) (OtherComp :type Primitive%20Component%20Object%20Reference) (bSelfMoved :type Boolean) (HitLocation :type Vector :default "0, 0, 0") (HitNormal :type Vector :default "0, 0, 0") (NormalImpulse :type Vector :default "0, 0, 0") (Hit :type Hit%20Result%20Structure%20%28by%20ref%29))
  (if (Class|GameplayStatics|ObjectIsA Other "/Game/Marcus/Enemy/BP_Lamp_TEST.BP_Lamp_TEST_C")
    (Default|CallHitTarget)
    (Development|PrintString "Hit Lamp!!")
    (Physics|SetSimulatePhysics (Variables|Default|GetRock) false)
    (Niagara|ReinitializeSystem (Variables|Default|GetNiagara))
    (Rendering|SetVisibility (Variables|Default|GetRock) false false)
    (Utilities|FlowControl|Delay 2.0)
    (Actor|DestroyActor)
    (else
      (Development|PrintString "Missed Lamp!"))))

(fn ConstructionScript)