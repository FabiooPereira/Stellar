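; Enemy controller Blueprint that passes rock and lamp locations to the enemy's AI Blackboard.
; SetLocations writes the two given vectors to the LampLocation and RockLocation keys, then prints the stored rock location back from the Blackboard.
; The construction script is empty, and the file shows no behavior tree startup or other logic.
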(fn ConstructionScript)

(fn SetLocations
  (params (Rock :type Vector) (Lamp :type Vector))
  (bind _returnvalue (AI|GetBlackboard 0))
  (bind _returnvalue_2 (Utilities|Name|MakeLiteralName "RockLocation"))
  (AI|Components|Blackboard|SetValueasVector (AI|GetBlackboard 0) (Utilities|Name|MakeLiteralName "LampLocation") Lamp)
  (AI|Components|Blackboard|SetValueasVector _returnvalue _returnvalue_2 Rock)
  (Development|PrintString (Utilities|String|ToString(Vector) (AI|Components|Blackboard|GetValueasVector _returnvalue _returnvalue_2))))