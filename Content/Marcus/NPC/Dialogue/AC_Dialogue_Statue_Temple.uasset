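; Dialogue component for a strange temple statue whose inscription hints that an offering at the threshold opens the temple door.
; It overrides the parent Dialogue function and branches on the dialogue tree index.
; The first branch offers a choice to read or leave; leaving clears progress and closes the conversation.
; Reading advances the index before closing, so later conversations at that index jump straight to the inscription.
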(fn Dialogue
  (|CallParentFunction)
  (switch int (Variables|Default|GetDialogueTreeIndex)
    (:0
      (bind (_state _optionindex) (CallFunction|AddDialogue "Stella" "Something is written on the statue..." (Utilities|Array|MakeArray "Read it" "Leave")))
      (switch Utilities|FlowControl|Switch|SwitchonEnum_DialogueState _state
        (:NewEnumerator0
          (switch int _optionindex
            (:0
              (bind _state_2 (CallFunction|AddDialogue "Strange Statue" "Where shadows lengthen and the silent stars watch, lay the sacred offering at the threshold. Only then shall the temple’s ancient door yield its secrets.\"" (Utilities|Array|MakeArray "Continue") :!label _label))
              (switch Utilities|FlowControl|Switch|SwitchonEnum_DialogueState _state_2
                (:NewEnumerator0
                  (CallFunction|SetDialogueTreeIndex 1)
                  (CallFunction|CloseConversation))))
            (:1
              (CallFunction|ClearDialogueProgress)
              (CallFunction|CloseConversation))))))
    (:1
      (goto _label))))