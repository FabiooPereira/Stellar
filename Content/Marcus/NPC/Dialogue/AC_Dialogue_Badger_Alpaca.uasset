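; Dialogue component for Gunter the badger, an NPC who points the player toward a nearby alpaca companion.
; Overrides Dialogue, branching on DialogueTreeIndex through AddDialogue nodes with voice audio and reply options.
; The introduction sets the index to an annoyed or friendly state, each giving random one-liners on later talks.
; The first reply's switch is fixed at 0, so both greetings follow the same branch.
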(fn Dialogue
  (|CallParentFunction)
  (switch int (Variables|Default|GetDialogueTreeIndex)
    (:0
      (bind _state (CallFunction|AddDialogue "Gunter" "Why hello, I dont think we've met! I'm Gunter it's nice to meet you!" (Utilities|Array|MakeArray "Don't you recognize me Gunter?" "Hello there!") "/Game/Marcus/NPC/Dialogue/Sounds/NPC_Talk_1.NPC_Talk_1"))
      (switch Utilities|FlowControl|Switch|SwitchonEnum_DialogueState _state
        (:NewEnumerator0
          (switch int 0
            (:0
              (bind (_state_2 _optionindex) (CallFunction|AddDialogue "Gunter" "I'm quite sure I'd remember a twinkling visitor like you!  You must be mistaking me for another woodland critter!" (Utilities|Array|MakeArray "I'm quite certain Gunter" "Yes, my mistake") "/Game/Marcus/NPC/Dialogue/Sounds/NPC_Talk_4.NPC_Talk_4"))
              (switch Utilities|FlowControl|Switch|SwitchonEnum_DialogueState _state_2
                (:NewEnumerator0
                  (switch int _optionindex
                    (:0
                      (bind (_state_3 _optionindex_2) (CallFunction|AddDialogue "Gunter" "Why, are you on woodland patrol? Got a badge hidden somewhere?" (Utilities|Array|MakeArray "You're taking it too far Gunter" "No matter") "/Game/Marcus/NPC/Dialogue/Sounds/NPC_Talk_2.NPC_Talk_2"))
                      (switch Utilities|FlowControl|Switch|SwitchonEnum_DialogueState _state_3
                        (:NewEnumerator0
                          (switch int _optionindex_2
                            (:0
                              (bind _state_4 (CallFunction|AddDialogue "Gunter" "I'm not to fond of your tone. Perhaps the alpaca over there will appreciate your company more—it seems quite taken with you!" (Utilities|Array|MakeArray "Continue") "/Game/Marcus/NPC/Dialogue/Sounds/NPC_Talk_1.NPC_Talk_1"))
                              (switch Utilities|FlowControl|Switch|SwitchonEnum_DialogueState _state_4
                                (:NewEnumerator0
                                  (switch int 0
                                    (:0
                                      (CallFunction|SetDialogueTreeIndex 1)
                                      (CallFunction|CloseConversation))))))
                            (:1
                              (bind _state_5 (CallFunction|AddDialogue "Gunter" "Notice that alpaca over there? Seems you've caught its eye. I'd wager it'll be good company on your road ahead." (Utilities|Array|MakeArray "Continue") "/Game/Marcus/NPC/Dialogue/Sounds/NPC_Talk_3.NPC_Talk_3" :!label _label))
                              (switch Utilities|FlowControl|Switch|SwitchonEnum_DialogueState _state_5
                                (:NewEnumerator0
                                  (switch int 0
                                    (:0
                                      (CallFunction|SetDialogueTreeIndex 2)
                                      (CallFunction|CloseConversation))))))))))
                    (:1
                      (goto _label))))))
            (:1
              (goto _label))))))
    (:1
      (bind (_state_6 _optionindex_3) (CallFunction|AddDialogue "Badger" (Utilities|Select :Index (Math|Random|RandomIntegerinRange 0 1) :Option%200 "I'm having a good time, please let me be" :Option%201 "Go talk to that alpaca over there and leave me alone") (Utilities|Array|MakeArray "Continue") "/Game/Marcus/NPC/Dialogue/Sounds/NPC_Talk_2.NPC_Talk_2"))
      (switch Utilities|FlowControl|Switch|SwitchonEnum_DialogueState _state_6
        (:NewEnumerator0
          (switch int _optionindex_3
            (:0
              (CallFunction|ClearDialogueProgress)
              (CallFunction|CloseConversation))))))
    (:2
      (bind _state_7 (CallFunction|AddDialogue "Gunter" (Utilities|Select :Index (Math|Random|RandomIntegerinRange 0 1) :Option%200 "Don't be shy, get to know each other" :Option%201 "Isn't this a nice place to relax after long day") (Utilities|Array|MakeArray "Continue") "/Game/Marcus/NPC/Dialogue/Sounds/NPC_Talk_3.NPC_Talk_3"))
      (switch Utilities|FlowControl|Switch|SwitchonEnum_DialogueState _state_7
        (:NewEnumerator0
          (switch int 0
            (:0
              (CallFunction|ClearDialogueProgress)
              (CallFunction|CloseConversation))))))))