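; Dialogue component for the Strange Statue intro, where Stella can read an inscribed riddle pointing toward a hidden temple.
; Overrides Dialogue, calling the parent and then branching on DialogueTreeIndex, with each line and choice driven by AddDialogue.
; Leaving clears dialogue progress, while finishing the riddle advances the tree index so later conversations jump straight to the inscription.
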(fn Dialogue
  (|CallParentFunction)
  (switch int (Variables|Default|GetDialogueTreeIndex)
    (:0
      (bind (_state _optionindex) (CallFunction|AddDialogue "Stella" "Something is written on the statue..." (Utilities|Array|MakeArray "Read it" "Leave")))
      (switch Utilities|FlowControl|Switch|SwitchonEnum_DialogueState _state
        (:NewEnumerator0
          (switch int _optionindex
            (:0
              (bind _state_2 (CallFunction|AddDialogue "Strange Statue" "Traveler of the celestial trails, you wander the earthly veils. Where sky meets stone, a sacred dome awaits those who roam. Seek the haven where stars embrace, within the temple's hidden grace." (Utilities|Array|MakeArray "Continue") :!label _label))
              (switch Utilities|FlowControl|Switch|SwitchonEnum_DialogueState _state_2
                (:NewEnumerator0
                  (CallFunction|SetDialogueTreeIndex 1)
                  (CallFunction|CloseConversation))))
            (:1
              (CallFunction|ClearDialogueProgress)
              (CallFunction|CloseConversation))))))
    (:1
      (goto _label))))