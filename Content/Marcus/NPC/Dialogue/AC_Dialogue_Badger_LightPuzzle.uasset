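; Dialogue component for Munter, the badger NPC who warns Stella to watch her light before the dark cave.
; Overrides Dialogue, switching on the tree index between introduction, Bunter follow-up and random idle hints.
; GameState records of Bunter and Gunter choose the greeting, including an apology nudge, and later unlock a reconciliation remark.
; Each AddDialogue carries text, options, voice and talk animation, with greeting branches converging on shared cave advice.
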(fn Dialogue
  (bind _returnvalue (Math|Random|RandomIntegerinRange 0 1))
  (bind _gamestate (Variables|Default|GetGameState))
  (|CallParentFunction)
  (switch int (Variables|Default|GetDialogueTreeIndex)
    (:0
      (if (and (Class|StellarGameState|GetHasTalkedto _gamestate "Bunter") (Class|StellarGameState|GetHasTalkedto _gamestate "Gunter"))
        (if (== (Class|StellarGameState|GetInteractionStatus (Variables|Default|GetGameState) "Bunter") 1)
          (bind _state (CallFunction|AddDialogue "Bunter?" "Why hello, I'm Munter! I heard your argument with that guy Bunter just now. I wouldn't want to upset him, I think you should go back and say sorry" (Utilities|Array|MakeArray "Yes seems fair, it was my fault") "/Game/Marcus/NPC/Dialogue/Sounds/Munter/Munter-004.Munter-004" "/Game/Marcus/Animation/Badger/AM_Badger_Talk.AM_Badger_Talk"))
          (switch Utilities|FlowControl|Switch|SwitchonEnum_DialogueState _state
            (:NewEnumerator0
              (bind (_state_2 _optionindex) (CallFunction|AddDialogue "Munter" "Don't forget it! Are you heading for that dark cave over there by the way?" (Utilities|Array|MakeArray "Yes, I was on my way" "No I need to head for Bunter") "/Game/Marcus/NPC/Dialogue/Sounds/Munter/Munter-005.Munter-005" "/Game/Marcus/Animation/Badger/AM_Badger_Talk.AM_Badger_Talk"))
              (switch Utilities|FlowControl|Switch|SwitchonEnum_DialogueState _state_2
                (:NewEnumerator0
                  (Class|StellarGameState|UpdateNPCData (Variables|Default|GetGameState) "Munter" 0 (Variables|Default|GetDialogueTreeIndex))
                  (switch int _optionindex
                    (:0
                      (bind _state_3 (CallFunction|AddDialogue "Munter" "How scary! Make sure to keep a close eye on your light in there; you wouldn't want it to slip away in case you need it" (Utilities|Array|MakeArray "Thank you, I'll see you around Munter") "/Game/Marcus/NPC/Dialogue/Sounds/Munter/Munter-006.Munter-006" "/Game/Marcus/Animation/Badger/AM_Badger_Talk.AM_Badger_Talk" :!label _label))
                      (switch Utilities|FlowControl|Switch|SwitchonEnum_DialogueState _state_3
                        (:NewEnumerator0
                          (CallFunction|SetDialogueTreeIndex 1)
                          (CallFunction|CloseConversation))))
                    (:1
                      (bind _state_4 (CallFunction|AddDialogue "Munter" "Oh I understand, I wouldn't venture there myself. If you decide to enter, I recommend keeping a close watch on your light and make good use of it." (Utilities|Array|MakeArray "Thank you, I'll see you around Munter") "/Game/Marcus/NPC/Dialogue/Sounds/Munter/Munter-007.Munter-007" "/Game/Marcus/Animation/Badger/AM_Badger_Talk.AM_Badger_Talk" :!label _label_2))
                      (switch Utilities|FlowControl|Switch|SwitchonEnum_DialogueState _state_4
                        (:NewEnumerator0
                          (CallFunction|SetDialogueTreeIndex 1)
                          (CallFunction|CloseConversation)))))))))
          (else
            (bind _state_5 (CallFunction|AddDialogue "Bunter?" "Why hello, I dont think we've met! I'm Munter it's nice to meet you!" (Utilities|Array|MakeArray "Oh hello Munter") "/Game/Marcus/NPC/Dialogue/Sounds/Munter/Munter-001.Munter-001" "/Game/Marcus/Animation/Badger/AM_Badger_Talk.AM_Badger_Talk"))
            (switch Utilities|FlowControl|Switch|SwitchonEnum_DialogueState _state_5
              (:NewEnumerator0
                (Class|StellarGameState|UpdateNPCData (Variables|Default|GetGameState) "Munter" 0 (Variables|Default|GetDialogueTreeIndex))
                (bind (_state_6 _optionindex_2) (CallFunction|AddDialogue "Munter" "Stella, what a nice name? Are you perhaps heading for that dark cave over there?" (Utilities|Array|MakeArray "Yes, there's only one way forward..." "No") "/Game/Marcus/NPC/Dialogue/Sounds/Munter/Munter-003.Munter-003" "/Game/Marcus/Animation/Badger/AM_Badger_Talk.AM_Badger_Talk"))
                (switch Utilities|FlowControl|Switch|SwitchonEnum_DialogueState _state_6
                  (:NewEnumerator0
                    (switch int _optionindex_2
                      (:0
                        (goto _label))
                      (:1
                        (goto _label_2)))))))))
        (else
          (bind _state_7 (CallFunction|AddDialogue "Bunter?" "Why hello, I dont think we've met! I'm Munter it's nice to meet you!" (Utilities|Array|MakeArray "Hi there, I'm Stella!") "/Game/Marcus/NPC/Dialogue/Sounds/Munter/Munter-001.Munter-001" "/Game/Marcus/Animation/Badger/AM_Badger_Talk.AM_Badger_Talk"))
          (switch Utilities|FlowControl|Switch|SwitchonEnum_DialogueState _state_7
            (:NewEnumerator0
              (Class|StellarGameState|UpdateNPCData (Variables|Default|GetGameState) "Munter" 0 (Variables|Default|GetDialogueTreeIndex))
              (bind (_state_8 _optionindex_3) (CallFunction|AddDialogue "Munter" "Stella, what a nice name? Are you perhaps heading for that dark cave over there?" (Utilities|Array|MakeArray "Yes!" "Not at this time") "/Game/Marcus/NPC/Dialogue/Sounds/Munter/Munter-003.Munter-003" "/Game/Marcus/Animation/Badger/AM_Badger_Talk.AM_Badger_Talk"))
              (switch Utilities|FlowControl|Switch|SwitchonEnum_DialogueState _state_8
                (:NewEnumerator0
                  (switch int _optionindex_3
                    (:0
                      (goto _label))
                    (:1
                      (goto _label_2))))))))))
    (:1
      (if (== (Class|StellarGameState|GetInteractionStatus (Variables|Default|GetGameState) "Bunter") 2)
        (bind _state_9 (CallFunction|AddDialogue "Bunter?" "I'm glad you made peace with Bunter, he's actually quite cool!" (Utilities|Array|MakeArray "Sure Munter") "/Game/Marcus/NPC/Dialogue/Sounds/Munter/Munter-008.Munter-008" "/Game/Marcus/Animation/Badger/AM_Badger_Talk.AM_Badger_Talk"))
        (switch Utilities|FlowControl|Switch|SwitchonEnum_DialogueState _state_9
          (:NewEnumerator0
            (CallFunction|SetDialogueTreeIndex 2)
            (CallFunction|ClearDialogueProgress)
            (CallFunction|CloseConversation)))
        (else
          (bind _state_10 (CallFunction|AddDialogue "Munter" (Utilities|Select :Index _returnvalue :Option%200 "I would never dare to go near that cave myself, I'll stay out here thank you very much. And that'll be the end of it" :Option%201 "Remember to keep track of your light, you'll need it") (Utilities|Array|MakeArray "Continue") (Utilities|Select :Index _returnvalue :Option%200 "/Game/Marcus/NPC/Dialogue/Sounds/Munter/Munter-009.Munter-009" :Option%201 "/Game/Marcus/NPC/Dialogue/Sounds/Munter/Munter-010.Munter-010") "/Game/Marcus/Animation/Badger/AM_Badger_Talk.AM_Badger_Talk" :!label _label_3))
          (switch Utilities|FlowControl|Switch|SwitchonEnum_DialogueState _state_10
            (:NewEnumerator0
              (CallFunction|ClearDialogueProgress)
              (CallFunction|CloseConversation))))))
    (:2
      (goto _label_3))))