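; Dialogue component for Gunter, the badger NPC who greets the player in the woods and hints at a coming companion.
; On top of the parent dialogue, it resets Gunter's GameState NPC data and branches on DialogueTreeIndex.
; The first conversation chains voiced lines with one optional follow-up, then advances the index.
; Later talks show a repeat line; its random range is pinned, so only the locked-door hint appears.
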(fn Dialogue
  (|CallParentFunction)
  (Class|StellarGameState|UpdateNPCData (Variables|Default|GetGameState) "Gunter")
  (switch int (Variables|Default|GetDialogueTreeIndex)
    (:0
      (Variables|Default|SetbTalkedToStartGunter true)
      (bind _state (CallFunction|AddDialogue "Gunter" "Hello there! I'm one of the keepers of these woods. What adventure brings you this way?" (Utilities|Array|MakeArray "I'm searching for a way back home") "/Game/Marcus/NPC/Dialogue/Sounds/NPC_Hello.NPC_Hello" "/Game/Marcus/Animation/Badger/AM_Badger_Talking.AM_Badger_Talking"))
      (switch Utilities|FlowControl|Switch|SwitchonEnum_DialogueState _state
        (:NewEnumerator0
          (bind (_state_2 _optionindex) (CallFunction|AddDialogue "Gunter" "Ah, home! Keep your spirits high and your eyes open, you might soon find a fluffy friend to join you on your journey." (Utilities|Array|MakeArray "A fluffy friend?" "Thanks for the heads up.") "/Game/Marcus/NPC/Dialogue/Sounds/NPC_Badger_Start_2.NPC_Badger_Start_2"))
          (switch Utilities|FlowControl|Switch|SwitchonEnum_DialogueState _state_2
            (:NewEnumerator0
              (switch int _optionindex
                (:0
                  (bind _state_3 (CallFunction|AddDialogue "Gunter" "Yes, one who's soft on the hooves and big on heart. They'll stroll beside you when you least expect it." (Utilities|Array|MakeArray "You sure know a lot, I can't wait to meet them.") "/Game/Marcus/NPC/Dialogue/Sounds/NPC_Hooves.NPC_Hooves"))
                  (switch Utilities|FlowControl|Switch|SwitchonEnum_DialogueState _state_3
                    (:NewEnumerator0
                      _)))
                (:1
                  _))
              (bind _state_4 (CallFunction|AddDialogue "Gunter" "Just a bit of woodland wisdom for you! Safe travels, and remember to relish those quiet moments!" (Utilities|Array|MakeArray "Continue") "/Game/Marcus/NPC/Dialogue/Sounds/NPC_Badger_Start_4.NPC_Badger_Start_4"))
              (switch Utilities|FlowControl|Switch|SwitchonEnum_DialogueState _state_4
                (:NewEnumerator0
                  (CallFunction|SetDialogueTreeIndex 1)
                  (CallFunction|CloseConversation))))))))
    (:1
      (bind _state_5 (CallFunction|AddDialogue "Badger" (Utilities|Select :Index (Math|Random|RandomIntegerinRange 1 1) :Option%200 "Best of luck on your journey friend!" :Option%201 "If only that pesky door you walked by weren't locked... ") (Utilities|Array|MakeArray "Continue") "/Game/Marcus/NPC/Dialogue/Sounds/NPC_Badger_Start_5.NPC_Badger_Start_5"))
      (switch Utilities|FlowControl|Switch|SwitchonEnum_DialogueState _state_5
        (:NewEnumerator0
          (CallFunction|ClearDialogueProgress)
          (CallFunction|CloseConversation))))))